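; Arena game mode that runs timed gladiator matches between player and AI teams.
; Spawns each player's chosen gladiator at a random team spawner, then once spawns AI gladiators from the "custommatch" save.
; AI controllers get random skill within difficulty bands, and initial gladiators are tallied per team.
; Timer expiry makes pawns immortal and declares a draw; player deaths can trigger defeat, while older "match" save logic is disconnected.
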(event Custom|StartTheMatchSpawnAIAndOthers
  (if (not (Variables|Default|GetbSpawnedAI))
    (bind _gladiators (CallFunction|SpawntheCustomGladiators (CallFunction|FetchSpawners)))
    (CallFunction|CountandAssignGladiatorPerTeam _gladiators)
    (Variables|Default|SetbSpawnedAI true)))

(event Custom|SpawnThePlayerPawnWithParams
  (params (NewPlayer :type BP%20GOTAPC%20Max%20Par%20Class%20Object%20Reference))
  (bind _spawners (CallFunction|FetchSpawners))
  (bind _playerteam (Variables|/Game/GOTA2/Blueprints/Controllers/BP_GOTAPCMaxParClass.BP_GOTAPCMaxParClass_C|GetPlayerTeam NewPlayer))
  (bind _returnvalue (Math|Conversions|ToByte(Integer) _playerteam))
  (bind _teamspawners (CallFunction|ReturnRandomSpawnerOfTeambyArray _spawners _returnvalue))
  (bind _gladiator (Default|SpawnGladiatorCustomandReturnIt (Utilities|Array|Get(acopy) _teamspawners (Math|Random|RandomIntegerinRange 0 (- (Utilities|Array|Length _teamspawners) 1))) "NewEnumerator0" (Variables|/Game/GOTA2/Blueprints/Controllers/BP_GOTAPCMaxParClass.BP_GOTAPCMaxParClass_C|GetPlayerChosenGladiator NewPlayer) _playerteam))
  (Pawn|Possess NewPlayer _gladiator)
  (Input|SetInputModeGameOnly NewPlayer)
  (CallFunction|StarttheMatchSpawnAIandOthers)
  (switch int _playerteam
    (:0
      (Math|Integer|IncrementInt (Variables|Default|GetInitialTeam0GladiatorsFreeForAll)))
    (:1
      (Math|Integer|IncrementInt (Variables|Default|GetInitialTeam1Gladiators)))
    (:2
      (Math|Integer|IncrementInt (Variables|Default|GetInitialTeam2Gladiators)))
    (:3
      (Math|Integer|IncrementInt (Variables|Default|GetInitialTeam3Gladiators)))
    (:4
      (Math|Integer|IncrementInt (Variables|Default|GetInitialTeam4Gladiators)))))

(event Custom|CustomEvent
  (CallFunction|HandleCommonDraw "Time is over!"))

(event Custom|HandleEndMatchByTimer_1
  (CallFunction|HandleCommonDraw "Time is over!"))

(event EventBeginPlay
  (Utilities|FlowControl|Sequence
    (:then_0
      (|CallParentFunction))
    (:then_1
      (Utilities|FlowControl|Delay 2.0))
    (:then_2
      (bind _returnvalue (Utilities|Time|SetTimerbyEvent (delegate Custom|CustomEvent) (Variables|Default|GetTimeToEndMatch)))
      (bind _output_get (Variables|Default|SetMatchEndTHandle _returnvalue)))))

(event EventTick
  (params (DeltaSeconds :type Float%20%28single-precision%29))
  (|CallParentFunction DeltaSeconds) ; This node is disabled and will not be called.\nDrag off pins to build functionality.
)

(event EventHandlePawnDied
  (params (DiedPawn :type BP%20GOTA%20Char%20Max%20Par%20Class%20Object%20Reference))
  (if (Variables|Default|GetbShouldHaveGoalWinAndSuch)
    (Utilities|FlowControl|Sequence
      (:then_0
        (|CallParentFunction DiedPawn))
      (:then_1
        (bind _asbp_gotapcmax_par_class (Utilities|Casting|CastToBP_GOTAPCMaxParClass (Pawn|GetController DiedPawn)))
        (if (Utilities|Enum|Equal(Enum) (Variables|/Game/GOTA2/Blueprints/Characters/BP_GOTACharMaxParClass.BP_GOTACharMaxParClass_C|GetPawnState DiedPawn) "NewEnumerator2")
          (Default|ClientPlayDefeat _asbp_gotapcmax_par_class)
          (Utilities|FlowControl|Delay 3.0)
          (if (Variables|Default|GetShouldGoToMenuWhenDefeat)
            _))))))

(event EventOnLogout
  (params (ExitingController :type Controller%20Object%20Reference))
  ;[1 1 1] Not working so well
)

(event EventHandleCommonDraw
  (params (reason :type String))
  (CallFunction|TurnAllPawnsInmortal)
  (|CallParentFunction reason))

(event EventPostLogin
  (params (NewPlayer :type Player%20Controller%20Object%20Reference))
  (bind _asbp_gotapcmax_par_class (Utilities|Casting|CastToBP_GOTAPCMaxParClass NewPlayer))
  ;[1 1 1] Left here just in case
  (if (Variables|Default|GetbSpawnedAI)
    _
    (else
      _))
  (Utilities|FlowControl|Delay 2.0)
  (bind _asbp_gotapcmax_par_class_2 (Utilities|Casting|CastToBP_GOTAPCMaxParClass NewPlayer))
  (Default|ClientSetCountDownVisiblity _asbp_gotapcmax_par_class_2 true))

(event EventHandleStartingNewPlayer
  (params (NewPlayer :type Player%20Controller%20Object%20Reference)))

(fn ConstructionScript
  (|CallParentFunction))

(fn FetchSpawners
  (bind _outactors (Actor|GetAllActorsOfClass "/Game/GOTA2/Blueprints/Spawners/BP_GOTASpawnerMaxPar.BP_GOTASpawnerMaxPar_C"))
  (return _outactors))

(fn SpawntheGladiators
  (params (Spawners :type Array%20of%20BP%20GOTA%20Spawner%20Max%20Par%20Object%20References))
  ;[1 1 1] DEPRA?
)

(fn GetMinBotDifffromMatch)

(fn GetMaxBotDifffromMatch)

(fn ReturnRandomWeaponClassandQLWIP
  (return (Utilities|Select :Index (Math|Random|RandomInteger 4) :Option%200 "/Game/GOTA2/Blueprints/InventoryAndItems/BP_GOTAGladius_A.BP_GOTAGladius_A_C" :Option%201 "/Game/GOTA2/Blueprints/InventoryAndItems/BP_GOTASpearItem.BP_GOTASpearItem_C" :Option%202 "/Game/GOTA2/Blueprints/InventoryAndItems/BP_GOTAGladius_A.BP_GOTAGladius_A_C" :Option%203 "/Game/GOTA2/Blueprints/InventoryAndItems/BP_GOTAFalx.BP_GOTAFalx_C" :Option%204 "/Game/GOTA2/Blueprints/InventoryAndItems/BP_GOTAGladius_A.BP_GOTAGladius_A_C" :Option%205 "/Game/GOTA2/Blueprints/InventoryAndItems/BP_GOTAGladius_A.BP_GOTAGladius_A_C" :Option%206 "/Game/GOTA2/Blueprints/InventoryAndItems/BP_GOTAGladius_A.BP_GOTAGladius_A_C") 0))

(fn SpawntheCustomGladiators
  (params (Spawners :type Array%20of%20BP%20GOTA%20Spawner%20Max%20Par%20Object%20References))
  (bind _returnvalue (SaveGame|DoesSaveGameExist "custommatch"))
  (if _returnvalue
    (bind _returnvalue_2 (SaveGame|LoadGamefromSlot "custommatch"))
    (bind _asbp_gotasave_custom_match_max_par (Utilities|Casting|CastToBP_GOTASaveCustomMatchMaxPar _returnvalue_2))
    (for _array_element (Variables|/Game/GOTA2/Blueprints/SaveSystem/BP_GOTASaveCustomMatchMaxPar.BP_GOTASaveCustomMatchMaxPar_C|GetGladiatorsArrayToFight _asbp_gotasave_custom_match_max_par)
      ;[1 1 1] Should add name later
      (bind (_gladiator _gladiatordifficulty) (Default|SpawnGladiatorCustomandReturnIt (Utilities|Array|Get(acopy) (CallFunction|ReturnRandomSpawnerOfTeambyArray Spawners (Math|Conversions|ToByte(Integer) (.teamnum _array_element))) (Math|Random|RandomIntegerinRange 0 (- (Utilities|Array|Length (CallFunction|ReturnRandomSpawnerOfTeambyArray Spawners (Math|Conversions|ToByte(Integer) (.teamnum _array_element)))) 1))) (.gladiatordifficulty _array_element) (.gladiatortypeuniversal _array_element) (.teamnum _array_element)))
      ;[1 1 1] This is doing nothing here
      (Utilities|Array|Add (LocalVariables|GetGladiatorsSpawned) _gladiator)
      (bind _returnvalue_3 (Game|SpawnActorfromClass "/Game/GOTA2/Blueprints/Controllers/BP_GOTAAICMaxParClass.BP_GOTAAICMaxParClass_C" (Math|Transform|MakeTransform (Transformation|GetActorLocation) (Transformation|GetActorRotation)) "AlwaysSpawn" 0 "NewEnumerator1" (Math|Random|RandomFloatinRange (CallFunction|GetMinBotDifffromCustom _gladiatordifficulty) (CallFunction|GetMaxBotDifffromCustom _gladiatordifficulty)) "NewEnumerator18" 0))
      (Pawn|Possess _returnvalue_3 _gladiator))
    (return (LocalVariables|GetGladiatorsSpawned))))

(fn GetMinBotDifffromCustom
  (params (BotDiff :type EN_MatchDifficulty%20Enum :default "NewEnumerator0"))
  (return (Utilities|Select :Index BotDiff :NewEnumerator0 0.1 :NewEnumerator1 0.5 :NewEnumerator2 0.75)))

(fn GetMaxBotDifffromCustom
  (params (BotDiff :type EN_MatchDifficulty%20Enum :default "NewEnumerator0"))
  (return (Utilities|Select :Index BotDiff :NewEnumerator0 0.3 :NewEnumerator1 0.7 :NewEnumerator2 1.0)))

(fn CountandAssignGladiatorPerTeam
  (params (GladiatorsInTeam :type Array%20of%20BP%20GOTA%20Char%20Max%20Par%20Class%20Object%20References))
  (for _array_element GladiatorsInTeam
    (switch int (Variables|/Game/GOTA2/Blueprints/Characters/BP_GOTACharMaxParClass.BP_GOTACharMaxParClass_C|GetTeamNumInt _array_element)
      (:0
        (Math|Integer|IncrementInt (Variables|Default|GetInitialTeam0GladiatorsFreeForAll)))
      (:1
        (Math|Integer|IncrementInt (Variables|Default|GetInitialTeam1Gladiators)))
      (:2
        (Math|Integer|IncrementInt (Variables|Default|GetInitialTeam2Gladiators)))
      (:3
        (Math|Integer|IncrementInt (Variables|Default|GetInitialTeam3Gladiators)))
      (:4
        (Math|Integer|IncrementInt (Variables|Default|GetInitialTeam4Gladiators))))))

(fn ReturnRandomSpawnerOfTeambyArray
  (params (Spawners :type Array%20of%20BP%20GOTA%20Spawner%20Max%20Par%20Object%20References) (TeamNum :type Byte))
  (bind _spawnersofteam (LocalVariables|GetSpawnersOfTeam))
  (bind _array_element (Utilities|Array|ForEachLoopwithBreak Spawners)
    (:LoopBody
      (if (== (Variables|/Game/GOTA2/Blueprints/Spawners/BP_GOTASpawnerMaxPar.BP_GOTASpawnerMaxPar_C|GetSPWNRTeam _array_element) TeamNum)
        (Utilities|Array|Add _spawnersofteam _array_element)))
    (:Completed
      (return _spawnersofteam))))