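; Base spectator character for GOTA2 that rewards or penalizes the gladiator who kills it.
; On death it resolves the killer from the damaging actor and checks that gladiator's individual entertainment score against a threshold.
; A high score earns entertainment points and a low one loses the same amount, applied as a bonification through the game mode after calling the parent handler.
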(event EventBeginPlay
  (|CallParentFunction) ; This node is disabled and will not be called.\nDrag off pins to build functionality.
)

(event Collision|EventActorBeginOverlap
  (params (OtherActor :type Actor%20Object%20Reference))
  (|CallParentFunction OtherActor) ; This node is disabled and will not be called.\nDrag off pins to build functionality.
)

(event EventTick
  (params (DeltaSeconds :type Float%20%28single-precision%29))
  (|CallParentFunction DeltaSeconds) ; This node is disabled and will not be called.\nDrag off pins to build functionality.
)

(event EventTakeDamageHandleSpecialEvents
  (params (ActorDamaging :type Actor%20Object%20Reference))
  (|CallParentFunction ActorDamaging))

(event EventHandleBonificationKIllerAfterDying
  (params (ActorKiller :type Actor%20Object%20Reference))
  (bind _charkilling (CallFunction|ReturnKillerbyActorItem ActorKiller))
  (|CallParentFunction ActorKiller)
  (bind _asbp_gotagame_info_max_par_class (Utilities|Casting|CastToBP_GOTAGameInfoMaxParClass (Game|GetGameMode)))
  (if (>= (Variables|/Game/GOTA2/Blueprints/Characters/BP_GOTACharMaxParClass.BP_GOTACharMaxParClass_C|GetEntertainmentIndividual _charkilling) 50)
    (Default|HandleNewBonification _asbp_gotagame_info_max_par_class (Utilities|Struct|MakeST_Bonification "NewEnumerator12" 50) _charkilling)
    (else
      (Default|HandleNewBonification _asbp_gotagame_info_max_par_class (Utilities|Struct|MakeST_Bonification "NewEnumerator12" -50) _charkilling))))

(fn ConstructionScript
  (|CallParentFunction))