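; Campaign save game object for GOTA that stores campaign progress and the Corrupt Legionaries side.
; Saving writes itself to the "campaign" slot only if that slot exists, reporting success or error through game-info messages.
; Loading checks "campaign" but loads "match", cast to the general save class, or creates that class if "campaign" is absent.
; The loader's Slot input is unused.
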(fn LoadandReturntheSlot
  (params (slot :type String))
  (bind _returnvalue (SaveGame|DoesSaveGameExist "campaign"))
  (if _returnvalue
    (bind _returnvalue_2 (SaveGame|LoadGamefromSlot "match"))
    (bind _asbp_gotasave_system_general (Utilities|Casting|CastToBP_GOTASaveSystemGeneral _returnvalue_2))
    (return _asbp_gotasave_system_general)
    (else
      ;[1 1 1] Unnecesary but you never know
      (bind _returnvalue_3 (SaveGame|CreateSaveGameObject "/Game/GOTA2/Blueprints/SaveSystem/BP_GOTASaveSystemGeneral.BP_GOTASaveSystemGeneral_C"))
      (bind _asbp_gotasave_system_general_2 (Utilities|Casting|CastToBP_GOTASaveSystemGeneral _returnvalue_3))
      (return _asbp_gotasave_system_general_2))))

(fn SaveGameandReturnResultCampaignsandAll
  (params (gameinfo :type Game%20Mode%20Base%20Object%20Reference) (CampaignProcess :type Integer) (CorruptLegionariesSide :type Boolean))
  (bind _returnvalue (SaveGame|DoesSaveGameExist "campaign"))
  (if _returnvalue
    (Variables|Default|SetCamp1Progress CampaignProcess)
    (Variables|Default|SetCorruptLegionariesSide CorruptLegionariesSide)
    (bind _returnvalue_2 (SaveGame|SaveGametoSlot self "campaign"))
    (Development|PrintString 0 (Utilities|String|Append "FROM GOTASaveGame saving game  " (Utilities|GetDisplayName self)) true true "(R=1.000000,G=0.795438,B=0.000000,A=1.000000)" 1e+01)
    (bind _asbp_gotagame_info_max_par_class (Utilities|Casting|CastToBP_GOTAGameInfoMaxParClass gameinfo))
    (Default|AddMessageforAll _asbp_gotagame_info_max_par_class (Utilities|String|Append "Saving Progress Campaing Progress " (Utilities|String|ToString(Integer) (Variables|Default|GetCamp1Progress))) 1e+01 (Math|Color|MakeColor 0 255 255 255))
    (return _returnvalue_2)
    (else
      (bind _asbp_gotagame_info_max_par_class_2 (Utilities|Casting|CastToBP_GOTAGameInfoMaxParClass gameinfo))
      (Default|AddMessageforAll _asbp_gotagame_info_max_par_class_2 (Utilities|String|Append "ERROR did not exist Saving Progress Campaing  " (Utilities|String|ToString(Integer) (Variables|Default|GetCamp1Progress))) 1e+01 (Math|Color|MakeColor 0 0 255 255))
      (return false))))