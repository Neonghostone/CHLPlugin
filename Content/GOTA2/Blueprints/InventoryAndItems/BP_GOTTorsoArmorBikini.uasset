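; Torso bikini armor item Blueprint for GOTA2 that tints the armor in the wearer's team color.
; Its PaintTeamColorIcon function casts the owner to BP_GOTACharMaxParClass and creates a dynamic material from BikiniMainMat on element 1 of that character's TorsoProtection.
; It sets the TeamColor parameter from ArrayTeamColors by team number and returns the material instance.
; The event graph holds only disabled default events.
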(event EventBeginPlay
  (|CallParentFunction) ; This node is disabled and will not be called.\nDrag off pins to build functionality.
)

(event Collision|EventActorBeginOverlap
  (params (OtherActor :type Actor%20Object%20Reference))
  (|CallParentFunction OtherActor) ; This node is disabled and will not be called.\nDrag off pins to build functionality.
)

(event EventTick
  (params (DeltaSeconds :type Float%20%28single-precision%29))
  (|CallParentFunction DeltaSeconds) ; This node is disabled and will not be called.\nDrag off pins to build functionality.
)

(fn ConstructionScript
  (|CallParentFunction))

(fn PaintTeamColorIcon
  (bind _asbp_gotachar_max_par_class (Utilities|Casting|CastToBP_GOTACharMaxParClass (Components|GetOwner)))
  (bind _returnvalue (Rendering|Material|CreateDynamicMaterialInstance (Variables|/Game/GOTA2/Blueprints/Characters/BP_GOTACharMaxParClass.BP_GOTACharMaxParClass_C|GetTorsoProtection _asbp_gotachar_max_par_class) 1 "/Game/GOTA2/3d/Items/Armours/Female/BikiniMainMat.BikiniMainMat" "None" :!class /Script/Engine.PrimitiveComponent))
  (Rendering|Material|SetVectorParameterValue _returnvalue "TeamColor" (Utilities|Array|Get(acopy) (Variables|Default|GetArrayTeamColors) (Variables|/Game/GOTA2/Blueprints/Characters/BP_GOTACharMaxParClass.BP_GOTACharMaxParClass_C|GetTeamNumInt _asbp_gotachar_max_par_class)) :!class /Script/Engine.MaterialInstanceDynamic)
  (return _returnvalue))