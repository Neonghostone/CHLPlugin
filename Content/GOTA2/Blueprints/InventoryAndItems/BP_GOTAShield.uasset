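; BP_GOTAShield is an equippable shield item that occupies the secondary slot and can block or be thrown.
; Equipping removes any two-handed weapon and sets the left-arm mesh through the owning character's Repno variables.
; Blocking and throw charging drive the owner's replicated anim state.
; Hits adjust vigour and attacker special power, can stun a low-vigour holder, and cost extra durability; destruction clears inventory and notifies the player.
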(event EventBeginPlay
  (|CallParentFunction) ; This node is disabled and will not be called.\nDrag off pins to build functionality.
)

(event Collision|EventActorBeginOverlap
  (params (OtherActor :type Actor%20Object%20Reference))
  (|CallParentFunction OtherActor) ; This node is disabled and will not be called.\nDrag off pins to build functionality.
)

(event EventTick
  (params (DeltaSeconds :type Float%20%28single-precision%29))
  (|CallParentFunction DeltaSeconds) ; This node is disabled and will not be called.\nDrag off pins to build functionality.
)

(event EventEquip
  (bind _skelemeshtoequip (Variables|Default|GetSkeleMeshToEquip))
  (bind _asbp_gotachar_max_par_class (Utilities|Casting|CastToBP_GOTACharMaxParClass (Components|GetOwner)))
  ;[1 1 1] Unnequip the two handed weapon
  (bind _asbp_gotathitem (Utilities|Casting|CastToBP_GOTATHItem (Variables|/Game/GOTA2/Blueprints/InventoryAndItems/BP_GOTAInvMaxParClassInclBag.BP_GOTAInvMaxParClassInclBag_C|GetPrimaryItem (Variables|/Game/GOTA2/Blueprints/Characters/BP_GOTACharMaxParClass.BP_GOTACharMaxParClass_C|GetInvReference _asbp_gotachar_max_par_class)))
    (:then
      (Default|Unequip (Variables|/Game/GOTA2/Blueprints/InventoryAndItems/BP_GOTAInvMaxParClassInclBag.BP_GOTAInvMaxParClassInclBag_C|GetPrimaryItem (Variables|/Game/GOTA2/Blueprints/Characters/BP_GOTACharMaxParClass.BP_GOTACharMaxParClass_C|GetInvReference _asbp_gotachar_max_par_class))))
    (:CastFailed
      _))
  (Class|SkinnedMeshComponent|SetSkeletalMesh (Variables|/Game/GOTA2/Blueprints/Characters/BP_GOTACharMaxParClass.BP_GOTACharMaxParClass_C|GetLeftArmWeapon _asbp_gotachar_max_par_class) _skelemeshtoequip true)
  (Default|SetSecondaryItem (Variables|/Game/GOTA2/Blueprints/Characters/BP_GOTACharMaxParClass.BP_GOTACharMaxParClass_C|GetInvReference _asbp_gotachar_max_par_class) self)
  (Variables|Default|SetbPicked true)
  (Variables|/Game/GOTA2/Blueprints/Characters/BP_GOTACharMaxParClass.BP_GOTACharMaxParClass_C|SetRepnoSkeletalMeshLeft _asbp_gotachar_max_par_class _skelemeshtoequip)
  (CallFunction|ResetforEquip)
  (Variables|/Game/GOTA2/Blueprints/Characters/BP_GOTACharMaxParClass.BP_GOTACharMaxParClass_C|SetRepnoLeftScale _asbp_gotachar_max_par_class (Variables|Default|GetEquippingScale))
  (Variables|/Game/GOTA2/Blueprints/Characters/BP_GOTACharMaxParClass.BP_GOTACharMaxParClass_C|SetRepnoShieldScutum _asbp_gotachar_max_par_class (Variables|Default|GetbScutumShieldKind)))

(event EventStartProtecting
  (Variables|Default|SetbProtecting true)
  (bind _asbp_gotachar_max_par_class (Utilities|Casting|CastToBP_GOTACharMaxParClass (Components|GetOwner)))
  (Variables|/Game/GOTA2/Blueprints/Characters/BP_GOTACharMaxParClass.BP_GOTACharMaxParClass_C|SetReplicatedAnimState _asbp_gotachar_max_par_class "NewEnumerator4")
  (Variables|/Game/GOTA2/Blueprints/Characters/BP_GOTACharMaxParClass.BP_GOTACharMaxParClass_C|SetAccumulatedMouseX _asbp_gotachar_max_par_class 0)
  (Variables|/Game/GOTA2/Blueprints/Characters/BP_GOTACharMaxParClass.BP_GOTACharMaxParClass_C|SetAccumulatedMouseY _asbp_gotachar_max_par_class 0)
  (bind _asbp_gotachar_max_par_class_2 (Utilities|Casting|CastToBP_GOTACharMaxParClass (Components|GetOwner)))
  (Default|CallEventDispatcherProtectwithShield _asbp_gotachar_max_par_class_2))

(event EventStopProtecting
  (Variables|Default|SetbProtecting false)
  (bind _asbp_gotachar_max_par_class (Utilities|Casting|CastToBP_GOTACharMaxParClass (Components|GetOwner)))
  (Variables|/Game/GOTA2/Blueprints/Characters/BP_GOTACharMaxParClass.BP_GOTACharMaxParClass_C|SetReplicatedAnimState _asbp_gotachar_max_par_class "NewEnumerator0"))

(event EventUnequip
  (bind _asbp_gotachar_max_par_class (Utilities|Casting|CastToBP_GOTACharMaxParClass (Components|GetOwner)))
  (Class|SkinnedMeshComponent|SetSkeletalMesh (Variables|/Game/GOTA2/Blueprints/Characters/BP_GOTACharMaxParClass.BP_GOTACharMaxParClass_C|GetLeftArmWeapon _asbp_gotachar_max_par_class) 0 true)
  (Default|SetSecondaryItem (Variables|/Game/GOTA2/Blueprints/Characters/BP_GOTACharMaxParClass.BP_GOTACharMaxParClass_C|GetInvReference _asbp_gotachar_max_par_class))
  (Variables|Default|SetbPicked false)
  (Variables|/Game/GOTA2/Blueprints/Characters/BP_GOTACharMaxParClass.BP_GOTACharMaxParClass_C|SetRepnoSkeletalMeshLeft _asbp_gotachar_max_par_class 0))

(event EventStartThrowingWeapon
  (bind _returnvalue (Components|GetOwner))
  (Variables|Default|SetWheelHold true)
  (bind _asbp_gotachar_max_par_class (Utilities|Casting|CastToBP_GOTACharMaxParClass _returnvalue))
  (switch Utilities|FlowControl|Switch|SwitchonEN_AnimState (Variables|/Game/GOTA2/Blueprints/Characters/BP_GOTACharMaxParClass.BP_GOTACharMaxParClass_C|GetReplicatedAnimState _asbp_gotachar_max_par_class)
    (:NewEnumerator0
      (Variables|Default|SetbMinLoadTime false)
      (Utilities|FlowControl|Sequence
        (:then_0
          (Variables|Default|SetThrowPowerLatent 0.0)
          (bind _asbp_gotachar_max_par_class_2 (Utilities|Casting|CastToBP_GOTACharMaxParClass (Components|GetOwner)))
          (Variables|/Game/GOTA2/Blueprints/Characters/BP_GOTACharMaxParClass.BP_GOTACharMaxParClass_C|SetRepnoSkeletalMeshLeft _asbp_gotachar_max_par_class_2 0)
          (Variables|/Game/GOTA2/Blueprints/Characters/BP_GOTACharMaxParClass.BP_GOTACharMaxParClass_C|SetRepnoSkeletalMeshRight _asbp_gotachar_max_par_class_2 (Variables|Default|GetSkeleMeshToEquip))
          (Variables|/Game/GOTA2/Blueprints/Characters/BP_GOTACharMaxParClass.BP_GOTACharMaxParClass_C|SetReplicatedAnimState _asbp_gotachar_max_par_class_2 "NewEnumerator6")
          (CallFunction|BeginAddingPowerOfThrow)
          (Utilities|FlowControl|Delay (Variables|Default|GetMinWhenToThrowWeapon))
          (Variables|Default|SetbMinLoadTime true)
          (if (not (Variables|Default|GetWheelHold))
            (CallFunction|ClientGetAimVector)))
        (:then_1
          (bind _aspawn (Utilities|Casting|CastToPawn _returnvalue))
          (if (Pawn|IsPlayerControlled _aspawn)
            (CallFunction|ClientShowThrowingStuffandProgress false 0.01 self)))))))

(event EventActorTakeDamage
  (params (Damage :type Integer) (HitLoc :type Vector :default "0, 0, 0") (Normal :type Vector :default "0, 0, 0") (SocketIfAnyName :type String) (WeaponType :type EN_WeaponItemTypeEnum%20Enum :default "NewEnumerator0") (bShouldHaveImpulse :type Boolean) (ImpulseAmount :type Float%20%28single-precision%29) (bShouldStun :type Boolean) (TimeStunned :type Float%20%28single-precision%29) (SpeedOfHit :type Float%20%28single-precision%29) (HitRes :type Hit%20Result%20Structure) (Damager :type Actor%20Object%20Reference) (ParticleHitRot :type Rotator :default "0, 0, 0") (PROVISIONALDamageKind :type EN_AttackDamageKind%20Enum :default "NewEnumerator0"))
  (bind _asbp_gotachar_max_par_class (Utilities|Casting|CastToBP_GOTACharMaxParClass (Components|GetOwner)))
  (bind _asbp_gotaitem_max_par_class_i (Utilities|Casting|CastToBP_GOTAItemMaxParClassI Damager)
    (:then
      (bind _asbp_gotachar_max_par_class_2 (Utilities|Casting|CastToBP_GOTACharMaxParClass (Components|GetOwner _asbp_gotaitem_max_par_class_i)))
      (Default|AddSpecialAttackPower _asbp_gotachar_max_par_class_2 0 25)
      (Default|ServerSpendVigour _asbp_gotachar_max_par_class 20)
      (if (Default|BHasEnoughVig _asbp_gotachar_max_par_class 40)
        _
        (else
          (Default|DoShieldStun _asbp_gotachar_max_par_class)
          (Default|ServerSpendVigour _asbp_gotachar_max_par_class_2 20))))
    (:CastFailed
      (bind _asbp_gotachar_max_par_class_3 (Utilities|Casting|CastToBP_GOTACharMaxParClass Damager))
      (Default|AddSpecialAttackPower _asbp_gotachar_max_par_class_3 0 25)
      (Default|ServerSpendVigour _asbp_gotachar_max_par_class_3 20)
      (if (Default|BHasEnoughVig _asbp_gotachar_max_par_class 40)
        _
        (else
          (Default|DoShieldStun _asbp_gotachar_max_par_class)
          (Default|ServerSpendVigour _asbp_gotachar_max_par_class_3 20)))))
  (|CallParentFunction Damage HitLoc Normal SocketIfAnyName WeaponType bShouldHaveImpulse ImpulseAmount bShouldStun TimeStunned SpeedOfHit HitRes Damager ParticleHitRot "NewEnumerator0")
  ;[1 1 1] Extra durability loose
  (Utilities|Casting|CastToBP_GOTATHItem Damager
    (:then
      ;;[1 1 1] Loose extra durability for shield TH Does a lot more
      (CallFunction|LooseDurability 30))
    (:CastFailed
      (CallFunction|LooseDurability 15))))

(event EventDestroyed
  (CallFunction|ForAllPcsSpawnParticle "/Game/GOTA2/Particles/PSN_SparksParry.PSN_SparksParry" (Transformation|GetActorLocation) "0, 0, 0" (Math|Vector|MakeVector (Math|Random|RandomFloatinRange 0.5 2.0) (Math|Random|RandomFloatinRange 0.5 2.0) (Math|Random|RandomFloatinRange 0.5 2.0)))
  (bind _asbp_gotachar_max_par_class (Utilities|Casting|CastToBP_GOTACharMaxParClass (Variables|Default|GetLastOwner))
    (:then
      (Variables|/Game/GOTA2/Blueprints/Characters/BP_GOTACharMaxParClass.BP_GOTACharMaxParClass_C|SetReplicatedAnimState _asbp_gotachar_max_par_class "NewEnumerator0"))
    (:CastFailed
      _))
  (if (== (Variables|/Game/GOTA2/Blueprints/InventoryAndItems/BP_GOTAInvMaxParClassInclBag.BP_GOTAInvMaxParClassInclBag_C|GetPrimaryItem (Variables|/Game/GOTA2/Blueprints/Characters/BP_GOTACharMaxParClass.BP_GOTACharMaxParClass_C|GetInvReference _asbp_gotachar_max_par_class)) self)
    (Default|SetPrimaryItem (Variables|/Game/GOTA2/Blueprints/Characters/BP_GOTACharMaxParClass.BP_GOTACharMaxParClass_C|GetInvReference _asbp_gotachar_max_par_class)))
  (Default|RemoveItemfromInv (Variables|/Game/GOTA2/Blueprints/Characters/BP_GOTACharMaxParClass.BP_GOTACharMaxParClass_C|GetInvReference _asbp_gotachar_max_par_class) self)
  (if (Pawn|IsPlayerControlled _asbp_gotachar_max_par_class)
    (bind _asbp_gotapcmax_par_class (Utilities|Casting|CastToBP_GOTAPCMaxParClass (Pawn|GetController _asbp_gotachar_max_par_class)))
    (Default|ClientAddMessage _asbp_gotapcmax_par_class (Utilities|Array|Get(acopy) (Variables|Default|GetMultiNameItemBreak) (Math|Conversions|ToInteger(Byte) (Variables|/Game/GOTA2/Blueprints/Controllers/BP_GOTAPCMaxParClass.BP_GOTAPCMaxParClass_C|GetPlayerLanguage _asbp_gotapcmax_par_class))) 2.0 (Math|Color|MakeColor 0 0 255 255))))

(fn ConstructionScript
  (|CallParentFunction))