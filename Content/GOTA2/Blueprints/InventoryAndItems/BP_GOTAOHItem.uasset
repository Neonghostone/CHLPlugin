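; BP_GOTAOHItem is an inventory item Blueprint for an "OH" weapon type that defines its available special attacks.
; Its construction script adds three unique special attack structs with weapon-component tracing, a shared unleash time and power cost, icons, and damage set on two.
; It then calls the parent construction script, with the attacks already in place.
; The event graph holds only disabled default events.
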(event EventBeginPlay
  (|CallParentFunction) ; This node is disabled and will not be called.\nDrag off pins to build functionality.
)

(event Collision|EventActorBeginOverlap
  (params (OtherActor :type Actor%20Object%20Reference))
  (|CallParentFunction OtherActor) ; This node is disabled and will not be called.\nDrag off pins to build functionality.
)

(event EventTick
  (params (DeltaSeconds :type Float%20%28single-precision%29))
  (|CallParentFunction DeltaSeconds) ; This node is disabled and will not be called.\nDrag off pins to build functionality.
)

(fn ConstructionScript
  (bind _specialattacks (Variables|Default|GetSpecialAttacks))
  (Utilities|Array|AddUnique _specialattacks (Utilities|Struct|MakeST_SpecialAttack "NewEnumerator1" true 0 0 0.5 "/Game/GOTA2/Anims/AnimsUE4Skele/SpecialAttacks/SpecialAttackSpinningTwoHanded.SpecialAttackSpinningTwoHanded" 40 30 25 (Utilities|Struct|MakeSlateBrush "(X=32.000000,Y=32.000000)" "(Left=0.000000,Top=0.000000,Right=0.000000,Bottom=0.000000)" "(SpecifiedColor=(R=1.000000,G=1.000000,B=1.000000,A=1.000000),ColorUseRule=UseColor_Specified)" "/Game/GOTA2/2d/SpecialAttackIcons/SpecialSpearLongThrust.SpecialSpearLongThrust" "Image" "NoTile" "NoMirror")))
  (Utilities|Array|AddUnique _specialattacks (Utilities|Struct|MakeST_SpecialAttack "NewEnumerator2" true 0 0 0.5 "/Game/GOTA2/Anims/AnimsUE4Skele/SpecialAttacks/SpecialAttackSpinningTwoHanded.SpecialAttackSpinningTwoHanded" 40 30 50 (Utilities|Struct|MakeSlateBrush "(X=32.000000,Y=32.000000)" "(Left=0.000000,Top=0.000000,Right=0.000000,Bottom=0.000000)" "(SpecifiedColor=(R=1.000000,G=1.000000,B=1.000000,A=1.000000),ColorUseRule=UseColor_Specified)" "/Game/GOTA2/2d/SpecialAttackIcons/SpecialSpearLongThrust.SpecialSpearLongThrust" "Image" "NoTile" "NoMirror")))
  (Utilities|Array|AddUnique _specialattacks (Utilities|Struct|MakeST_SpecialAttack "NewEnumerator9" true 0 0 0.5 "/Game/GOTA2/Anims/AnimsUE4Skele/SpecialAttacks/SpecialAttackSpinningTwoHanded.SpecialAttackSpinningTwoHanded" 40 30 75 (Utilities|Struct|MakeSlateBrush "(X=32.000000,Y=32.000000)" "(Left=0.000000,Top=0.000000,Right=0.000000,Bottom=0.000000)" "(SpecifiedColor=(R=1.000000,G=1.000000,B=1.000000,A=1.000000),ColorUseRule=UseColor_Specified)" "/Game/GOTA2/2d/SpecialAttackIcons/1HRoll3FromBPack.1HRoll3FromBPack" "Image" "NoTile" "NoMirror")))
  (|CallParentFunction))