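; Tutorial arrow actor that pulses in size and can be shown or hidden through a replicated flag.
; On BeginPlay the Oscilate timeline drives the ArrowToDescribe component's relative Y and Z scale around the actor's scale, alongside the parent BeginPlay.
; ServerSetActorVisibleAndOtherAttris stores visibility and scale, and the visibility OnRep toggles hidden-in-game.
; The stored scale is not applied in these graphs.
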(event Custom|ServerSetActorVisibleAndOtherAttris
  (params (NewVisible :type Boolean) (Scale :type Vector :default "1.000000,1.000000,1.000000") (NewParam2 :type Boolean))
  (Variables|Default|SetrepnoNewVisible NewVisible)
  (Variables|Default|SetrepnoScaleVector Scale))

(event EventBeginPlay
  (Utilities|FlowControl|Sequence
    (:then_0
      (bind _floattofloataround (Timeline|Oscilate Play)
        (:Update
          (Transformation|SetRelativeScale3D (Variables|Default|GetArrowToDescribe) (+ (Transformation|GetActorScale3D) (* (Math|Vector|MakeVector 0.0 _floattofloataround _floattofloataround) 0.25))))))
    (:then_1
      (|CallParentFunction))))

(event Collision|EventActorBeginOverlap
  (params (OtherActor :type Actor%20Object%20Reference)))

(event EventTick
  (params (DeltaSeconds :type Float%20%28single-precision%29)))

(fn ConstructionScript)

(fn OnRepRepnoNewVisible
  (Rendering|SetActorHiddenInGame (not (Variables|Default|GetrepnoNewVisible))))