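; Game mode for the GOTA menu that clears any leftover online session and picks menu music.
; BeginPlay starts DestroySession on the first player controller, calls parent BeginPlay without waiting for the result, and prints a debug string on success.
; PostLogin, labeled "Commented out" yet still wired, hands a random PeacefulMusic track to the joining BP_GOTAPCMaxParClass controller.
; The parent PostLogin call is disconnected.
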(event EventBeginPlay
  (|DestroySession (Game|GetPlayerController 0)
    (:then
      (|CallParentFunction))
    (:OnSuccess
      (Development|PrintString "FROM GOTAGameInfo destyrotijg seuccesfully trhe session "))))

(event EventTick
  (params (DeltaSeconds :type Float%20%28single-precision%29))
  (|CallParentFunction DeltaSeconds) ; This node is disabled and will not be called.\nDrag off pins to build functionality.
)

(event EventPostLogin
  (params (NewPlayer :type Player%20Controller%20Object%20Reference))
  (bind _peacefulmusic (Variables|Default|GetPeacefulMusic))
  ;[1 1 1] Commented out
  (bind _asbp_gotapcmax_par_class (Utilities|Casting|CastToBP_GOTAPCMaxParClass NewPlayer))
  (Default|SetSongPlayingTrack1 _asbp_gotapcmax_par_class (Utilities|Array|Get(acopy) _peacefulmusic (Math|Random|RandomIntegerinRange 0 (- (Utilities|Array|Length _peacefulmusic) 1)))))

(fn ConstructionScript
  (|CallParentFunction))