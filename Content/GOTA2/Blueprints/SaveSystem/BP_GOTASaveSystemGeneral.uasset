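; BP_GOTASaveSystemGeneral is a save game object that stores general GOTA data: the match kind and whether the tutorial is done.
; Its save function sets both fields and writes itself to the "general" slot, identically whether or not that save exists.
; Its load function ignores the Slot input and reads the "match" slot, not "general", casting the result to this class or creating a fresh object when none exists.
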(fn LoadandReturntheSlot
  (params (slot :type String))
  (bind _returnvalue (SaveGame|DoesSaveGameExist "match"))
  (if _returnvalue
    (bind _returnvalue_2 (SaveGame|LoadGamefromSlot "match"))
    (bind _asbp_gotasave_system_general (Utilities|Casting|CastToBP_GOTASaveSystemGeneral _returnvalue_2))
    (return _asbp_gotasave_system_general)
    (else
      ;[1 1 1] Unnecesary but you never know
      (bind _returnvalue_3 (SaveGame|CreateSaveGameObject "BP_GOTASaveSystemGeneral_C"))
      (bind _asbp_gotasave_system_general_2 (Utilities|Casting|CastToBP_GOTASaveSystemGeneral _returnvalue_3))
      (return _asbp_gotasave_system_general_2))))

(fn SaveGameandAndgeneral
  (params (gameinfo :type Game%20Mode%20Base%20Object%20Reference) (bMatchKind :type Boolean) (bhasDoneTutorial :type Boolean))
  (bind _returnvalue (SaveGame|DoesSaveGameExist "general"))
  (if _returnvalue
    (Variables|Default|SetbCustomOrDebugMatch bMatchKind)
    (Variables|Default|SetbhasDoneTutorial bhasDoneTutorial)
    (bind _returnvalue_2 (SaveGame|SaveGametoSlot self "general"))
    (return _returnvalue_2)
    (else
      (Variables|Default|SetbCustomOrDebugMatch bMatchKind)
      (Variables|Default|SetbhasDoneTutorial bhasDoneTutorial)
      (bind _returnvalue_3 (SaveGame|SaveGametoSlot self "general"))
      (return _returnvalue_3))))