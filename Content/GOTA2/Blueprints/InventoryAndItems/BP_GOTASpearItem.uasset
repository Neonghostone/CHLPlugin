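; Spear weapon item that handles melee hit tracing, thrown-projectile tracing and three special attacks.
; The construction script registers the specials; unleashing one spends the owner's special power, opens delayed, timer-gated trace windows and resets the character's replicated animation state.
; Tick runs capped combo traces on authority during those windows, traces projectile flight in one item state, and updates the trail and trajectory rendering.
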(event EventBeginPlay
  (|CallParentFunction))

(event Collision|EventActorBeginOverlap
  (params (OtherActor :type Actor%20Object%20Reference))
  (|CallParentFunction OtherActor) ; This node is disabled and will not be called.\nDrag off pins to build functionality.
)

(event EventTick
  (params (DeltaSeconds :type Float%20%28single-precision%29))
  (Utilities|FlowControl|Sequence
    (:then_0
      (Networking|SwitchHasAuthority
        (:Authority
          (if (Variables|Default|GetbTracing)
            (if (< (Variables|Default|GetTracesNum) (Variables|Default|GetMaxTraces))
              (if (Class|KismetSystemLibrary|IsTimerActive 0 "TimerBasedCooldownUnleashAttack")
                (CallFunction|DefinitiveComboTrace)
                (Variables|Default|SetTracesNum (+ (Variables|Default|GetTracesNum) 1))))))))
    (:then_1
      (if (Utilities|Enum|Equal(Enum) (Variables|Default|GetEnumItemState) "NewEnumerator8")
        (if (> (Math|Vector|VectorLength (Variables|Default|GetLastLocVector)) 0.0)
          (CallFunction|PerformProjectileTrace)
          (else
            (Variables|Default|SetLastLocVector (Transformation|GetActorLocation))))))
    (:then_2
      (CallFunction|DrawTrailCloud))
    (:then_3
      (CallFunction|FORBOTHRenderTrajectory))))

(event EventSpawnAppearProjectileforThrow
  (params (ProjVelo :type Vector :default "0, 0, 0") (LocToSpawn :type Vector :default "0, 0, 0") (FinalPower :type Float%20%28single-precision%29) (ShouldActivateParticles :type Boolean))
  (|CallParentFunction ProjVelo LocToSpawn FinalPower ShouldActivateParticles))

(event EventUnleashSpecialAttack
  (CallFunction|SHServerSetDamageType "NewEnumerator1")
  (bind _asbp_gotachar_max_par_class (Utilities|Casting|CastToBP_GOTACharMaxParClass (Components|GetOwner)))
  (Default|SubtractSpecialPower _asbp_gotachar_max_par_class (Math|Random|RandomIntegerinRange (Math|Conversions|ToInteger(Byte) (Variables|Default|GetSpecialAttackPowerThatLoosesMin)) (Math|Conversions|ToInteger(Byte) (Variables|Default|GetSpecialAttackPowerThatLoosesMax))))
  (switch Utilities|FlowControl|Switch|SwitchonEN_SpecialAttack (.nameofatttackandstate (Utilities|Array|Get(acopy) (Variables|Default|GetSpecialAttacks) (Math|Conversions|ToInteger(Byte) (Variables|/Game/GOTA2/Blueprints/Characters/BP_GOTACharMaxParClass.BP_GOTACharMaxParClass_C|GetSpecialAttackNum _asbp_gotachar_max_par_class))))
    (:NewEnumerator0
      (Utilities|FlowControl|Delay 0.285714)
      (Variables|Default|SetTracesNum 0)
      (Utilities|FlowControl|Sequence
        (:then_0
          (Variables|Default|SetbTracing true)
          (Utilities|Time|SetTimerbyFunctionName 0 "TimerBasedCooldownUnleashAttack" 0.1)
          (Variables|Default|SetMaxTraces 200)
          (Utilities|FlowControl|Delay 0.2)
          (Variables|Default|SetbTracing true)
          (Variables|Default|SetTracesNum 0)
          (Utilities|Time|SetTimerbyFunctionName 0 "TimerBasedCooldownUnleashAttack" 0.1)
          (Utilities|FlowControl|Delay 0.2)
          (Variables|Default|SetTracesNum 0)
          (Variables|Default|SetbTracing true)
          (Utilities|Time|SetTimerbyFunctionName 0 "TimerBasedCooldownUnleashAttack" 0.1)
          (Utilities|FlowControl|Delay 0.4)
          (Variables|Default|SetTracesNum 0)
          (Variables|Default|SetbTracing true)
          (Utilities|Time|SetTimerbyFunctionName 0 "TimerBasedCooldownUnleashAttack" 0.3)
          (Utilities|FlowControl|Delay 0.25)
          (bind _asbp_gotachar_max_par_class_2 (Utilities|Casting|CastToBP_GOTACharMaxParClass (Components|GetOwner)))
          (Variables|/Game/GOTA2/Blueprints/Characters/BP_GOTACharMaxParClass.BP_GOTACharMaxParClass_C|SetReplicatedAnimState _asbp_gotachar_max_par_class_2 "NewEnumerator0")
          (Variables|Default|SetbTracing false)
          (Variables|Default|SetMaxTraces 60))))
    (:NewEnumerator1
      (Utilities|FlowControl|Delay 0.285714)
      (Variables|Default|SetTracesNum 0)
      (Utilities|FlowControl|Sequence
        (:then_0
          (Variables|Default|SetbTracing true)
          (Utilities|Time|SetTimerbyFunctionName 0 "TimerBasedCooldownUnleashAttack" 0.1)
          (Utilities|FlowControl|Delay (Math|Random|RandomFloatinRange 0.1 0.2))
          (bind _asbp_gotachar_max_par_class_3 (Utilities|Casting|CastToBP_GOTACharMaxParClass (Components|GetOwner)))
          (Variables|/Game/GOTA2/Blueprints/Characters/BP_GOTACharMaxParClass.BP_GOTACharMaxParClass_C|SetReplicatedAnimState _asbp_gotachar_max_par_class_3 "NewEnumerator0"))))
    (:NewEnumerator10
      (Utilities|FlowControl|Delay 0.285714)
      (Variables|Default|SetTracesNum 0)
      (Utilities|FlowControl|Sequence
        (:then_0
          (Variables|Default|SetbTracing true)
          (Utilities|Time|SetTimerbyFunctionName 0 "TimerBasedCooldownUnleashAttack" 0.1)
          (Utilities|FlowControl|Delay (Math|Random|RandomFloatinRange 0.1 0.2))
          (bind _asbp_gotachar_max_par_class_4 (Utilities|Casting|CastToBP_GOTACharMaxParClass (Components|GetOwner)))
          (Variables|/Game/GOTA2/Blueprints/Characters/BP_GOTACharMaxParClass.BP_GOTACharMaxParClass_C|SetReplicatedAnimState _asbp_gotachar_max_par_class_4 "NewEnumerator0"))))))

(fn ConstructionScript
  (Utilities|Array|AddUnique (Variables|Default|GetSpecialAttacks) (Utilities|Struct|MakeST_SpecialAttack "NewEnumerator0" true 0 0 2.0 "/Game/GOTA2/Anims/AnimsUE4Skele/SpecialAttacks/SpecialAttackSpinningTwoHanded.SpecialAttackSpinningTwoHanded" 40 60 25 (Utilities|Struct|MakeSlateBrush "(X=32.000000,Y=32.000000)" "(Left=0.000000,Top=0.000000,Right=0.000000,Bottom=0.000000)" "(SpecifiedColor=(R=1.000000,G=1.000000,B=1.000000,A=1.000000),ColorUseRule=UseColor_Specified)" "/Game/GOTA2/2d/SpecialAttackIcons/SpecialSpearLongThrust.SpecialSpearLongThrust" "Image" "NoTile" "NoMirror")))
  (Utilities|Array|AddUnique (Variables|Default|GetSpecialAttacks) (Utilities|Struct|MakeST_SpecialAttack "NewEnumerator0" true 0 0 2.0 "/Game/GOTA2/Anims/AnimsUE4Skele/SpecialAttacks/SpecialAttackSpinningTwoHanded.SpecialAttackSpinningTwoHanded" 40 60 25 (Utilities|Struct|MakeSlateBrush "(X=32.000000,Y=32.000000)" "(Left=0.000000,Top=0.000000,Right=0.000000,Bottom=0.000000)" "(SpecifiedColor=(R=1.000000,G=1.000000,B=1.000000,A=1.000000),ColorUseRule=UseColor_Specified)" "/Game/GOTA2/2d/SpecialAttackIcons/SpecialSpearDoubleAttack.SpecialSpearDoubleAttack" "Image" "NoTile" "NoMirror")))
  (Utilities|Array|AddUnique (Variables|Default|GetSpecialAttacks) (Utilities|Struct|MakeST_SpecialAttack "NewEnumerator10" true 0 0 2.0 "/Game/GOTA2/Anims/BougthPack1SwordManne/AttackA4.AttackA4" 40 60 25 (Utilities|Struct|MakeSlateBrush "(X=32.000000,Y=32.000000)" "(Left=0.000000,Top=0.000000,Right=0.000000,Bottom=0.000000)" "(SpecifiedColor=(R=1.000000,G=1.000000,B=1.000000,A=1.000000),ColorUseRule=UseColor_Specified)" "/Game/GOTA2/2d/SpecialAttackIcons/SpecialSpearDoubleAttack.SpecialSpearDoubleAttack" "Image" "NoTile" "NoMirror")))
  (|CallParentFunction))