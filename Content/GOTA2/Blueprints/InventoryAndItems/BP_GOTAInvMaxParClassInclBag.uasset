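; Base inventory class for GOTA characters that holds items, primary/secondary weapons and a quiver or bag.
; On BeginPlay the server spawns and equips the owner's default items; added arrows go into the quiver when one exists.
; Setters and OnRep functions push weapon changes to the HUD and reattach some left-hand gear.
; Helpers cycle equipable items, skipping shields and armour, and spawn random items from per-category archetype arrays.
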(event Custom|HandleItemGetThrownOrDropped
  (params (Item :type BP%20GOTA%20Item%20Max%20Par%20Class%20I%20Object%20Reference))
  (bind _secondaryitem (Variables|Default|GetSecondaryItem))
  (bind _primaryitem (Variables|Default|GetPrimaryItem))
  (Variables|/Game/GOTA2/Blueprints/InventoryAndItems/BP_GOTAItemMaxParClassI.BP_GOTAItemMaxParClassI_C|SetLastOwner Item (.AsBP%20GOTAChar%20Max%20Par%20Class (Utilities|Casting|CastToBP_GOTACharMaxParClass (Components|GetOwner))))
  (Utilities|FlowControl|Sequence
    (:then_0
      (Utilities|IsValid _primaryitem
        (:Is%20Valid
          (if (== Item _primaryitem)
            (CallFunction|SetPrimaryItem)))))
    (:then_1
      (Utilities|IsValid _secondaryitem
        (:Is%20Valid
          (if (== Item _secondaryitem)
            (CallFunction|SetSecondaryItem)))))
    (:then_2
      (bind _returnvalue (Utilities|Array|RemoveItem (Variables|Default|GetItemsInInv) Item))
      (if _returnvalue
        _))))

(event Custom|ServerDropTheseItems
  (params (ItemReferences :type Array%20of%20BP%20GOTA%20Item%20Max%20Par%20Class%20I%20Object%20References))
  ;[1 1 1] Kind off redundant but you never know, BUT works for specific items
  (for _array_element ItemReferences
    (Default|Drop _array_element)))

(event Custom|ClientDoLDisplayWeap
  (params (ItemToDisplay :type BP%20GOTA%20Item%20Max%20Par%20Class%20I%20Object%20Reference) (NewDura :type Integer))
  (bind _returnvalue (Components|GetOwner))
  (Utilities|IsValid _returnvalue
    (:Is%20Valid
      (bind _asbp_gotachar_max_par_class (Utilities|Casting|CastToBP_GOTACharMaxParClass _returnvalue))
      (bind _asbp_gotapcmax_par_class (Utilities|Casting|CastToBP_GOTAPCMaxParClass (Pawn|GetController _asbp_gotachar_max_par_class)))
      (bind _asbp_gotahudmax_par_class (Utilities|Casting|CastToBP_GOTAHUDMaxParClass (HUD|GetHUD _asbp_gotapcmax_par_class)))
      (Default|HandleNewSecondaryWeapon _asbp_gotahudmax_par_class ItemToDisplay NewDura))))

(event Custom|ClientDoRDisplayWeap
  (params (ItemToDisplay :type BP%20GOTA%20Item%20Max%20Par%20Class%20I%20Object%20Reference) (NewDura :type Integer))
  (bind _returnvalue (Components|GetOwner))
  (Utilities|IsValid _returnvalue
    (:Is%20Valid
      (bind _asbp_gotachar_max_par_class (Utilities|Casting|CastToBP_GOTACharMaxParClass _returnvalue))
      (bind _asbp_gotapcmax_par_class (Utilities|Casting|CastToBP_GOTAPCMaxParClass (Pawn|GetController _asbp_gotachar_max_par_class)))
      (bind _asbp_gotahudmax_par_class (Utilities|Casting|CastToBP_GOTAHUDMaxParClass (HUD|GetHUD _asbp_gotapcmax_par_class)))
      (Default|HandleNewPrimaryWeapon _asbp_gotahudmax_par_class ItemToDisplay NewDura))))

(event EventBeginPlay
  (Utilities|FlowControl|Delay 0.2)
  (Networking|SwitchHasAuthority
    (:Authority
      (CallFunction|AddDefaultItems))))

(event Collision|EventActorBeginOverlap
  (params (OtherActor :type Actor%20Object%20Reference)))

(event EventTick
  (params (DeltaSeconds :type Float%20%28single-precision%29)))

(fn ConstructionScript)

(fn SetPrimaryItem
  (params (NewPItem :type BP%20GOTA%20Item%20Max%20Par%20Class%20I%20Object%20Reference))
  (bind _returnvalue (Components|GetOwner))
  (bind _output_get (Variables|Default|SetPrimaryItem NewPItem))
  (Utilities|IsValid _output_get
    (:Is%20Valid
      (CallFunction|ClientDoRDisplayWeap NewPItem (Variables|/Game/GOTA2/Blueprints/InventoryAndItems/BP_GOTAItemMaxParClassI.BP_GOTAItemMaxParClassI_C|GetDurability _output_get))
      (bind _asbp_gotachar_max_par_class (Utilities|Casting|CastToBP_GOTACharMaxParClass _returnvalue))
      (Default|CallEventDispatcherCharSwitchWeapon _asbp_gotachar_max_par_class _output_get)
      (bind _asbp_gotapcmax_par_class (Utilities|Casting|CastToBP_GOTAPCMaxParClass (Pawn|GetController _asbp_gotachar_max_par_class)))
      (bind _asbp_gotahudmax_par_class (Utilities|Casting|CastToBP_GOTAHUDMaxParClass (HUD|GetHUD _asbp_gotapcmax_par_class)))
      (Default|UpdateSpecialAttacksLowerLeft (Variables|/Game/GOTA2/Blueprints/HUD/BP_GOTAHUDMaxParClass.BP_GOTAHUDMaxParClass_C|GetMainHUDMovie _asbp_gotahudmax_par_class) (Variables|/Game/GOTA2/Blueprints/InventoryAndItems/BP_GOTAItemMaxParClassI.BP_GOTAItemMaxParClassI_C|GetSpecialAttacks _output_get)))
    (:Is%20Not%20Valid
      (CallFunction|ClientDoRDisplayWeap)
      (bind _asbp_gotachar_max_par_class_2 (Utilities|Casting|CastToBP_GOTACharMaxParClass _returnvalue))
      (bind _asbp_gotapcmax_par_class_2 (Utilities|Casting|CastToBP_GOTAPCMaxParClass (Pawn|GetController _asbp_gotachar_max_par_class_2)))
      (bind _asbp_gotahudmax_par_class_2 (Utilities|Casting|CastToBP_GOTAHUDMaxParClass (HUD|GetHUD _asbp_gotapcmax_par_class_2)))
      (Default|UpdateSpecialAttacksLowerLeft (Variables|/Game/GOTA2/Blueprints/HUD/BP_GOTAHUDMaxParClass.BP_GOTAHUDMaxParClass_C|GetMainHUDMovie _asbp_gotahudmax_par_class_2) (Variables|/Game/GOTA2/Blueprints/Characters/BP_GOTACharMaxParClass.BP_GOTACharMaxParClass_C|GetMeleeSpecialAttacks _asbp_gotachar_max_par_class_2)))))

(fn AddItemtoInventory
  (params (NewItem :type BP%20GOTA%20Item%20Max%20Par%20Class%20I%20Object%20Reference))
  (bind _returnvalue (Components|GetOwner))
  (bind _quiver (CallFunction|HasQuiver))
  (if (not (CallFunction|IsInventoryFull))
    (Utilities|IsValid NewItem
      (:Is%20Valid
        ;[1 1 1] Neongho: Arrows here
        (bind _asbp_gotaarrow_item (Utilities|Casting|CastToBP_GOTAArrowItem NewItem)
          (:then
            (Utilities|IsValid _quiver
              (:Is%20Valid
                (Actor|SetOwner _asbp_gotaarrow_item _returnvalue)
                (Default|AddIteminQuiverorBag _quiver _asbp_gotaarrow_item)
                (return true))
              (:Is%20Not%20Valid
                _)))
          (:CastFailed
            _))
        (Actor|SetOwner NewItem _returnvalue)
        (Utilities|Array|Add (Variables|Default|GetItemsInInv) NewItem)
        (return true)))
    (else
      (return false))))

(fn SetSecondaryItem
  (params (NewSItem :type BP%20GOTA%20Item%20Max%20Par%20Class%20I%20Object%20Reference))
  (bind _output_get (Variables|Default|SetSecondaryItem NewSItem))
  (Utilities|IsValid _output_get
    (:Is%20Valid
      (CallFunction|ClientDoLDisplayWeap NewSItem (Variables|/Game/GOTA2/Blueprints/InventoryAndItems/BP_GOTAItemMaxParClassI.BP_GOTAItemMaxParClassI_C|GetDurability _output_get)))
    (:Is%20Not%20Valid
      (CallFunction|ClientDoLDisplayWeap))))

(fn AddDefaultItems
  (bind _returnvalue (Components|GetOwner))
  (bind _returnvalue_2 (Transformation|GetActorTransform _returnvalue))
  (bind _asbp_gotachar_max_par_class (Utilities|Casting|CastToBP_GOTACharMaxParClass _returnvalue))
  (for _array_element (Variables|/Game/GOTA2/Blueprints/Characters/BP_GOTACharMaxParClass.BP_GOTACharMaxParClass_C|GetDefaultItems _asbp_gotachar_max_par_class)
    (bind _returnvalue_3 (Game|SpawnActorfromClass _array_element (Math|Transform|MakeTransform (.location _returnvalue_2) (.rotation _returnvalue_2)) "Undefined" _returnvalue 90 "1.000000,1.000000,1.000000" false 0))
    (Utilities|IsValid _returnvalue_3
      (:Is%20Valid
        (Default|Equip _returnvalue_3)
        (CallFunction|AddItemtoInventory _returnvalue_3)))))

(fn RemoveItemfromInv
  (params (NewItem :type BP%20GOTA%20Item%20Max%20Par%20Class%20I%20Object%20Reference))
  (bind _quiverorbag (Variables|Default|GetQuiverOrBag))
  (Actor|SetOwner NewItem 0)
  (bind _returnvalue (Utilities|Array|RemoveItem (Variables|Default|GetItemsInInv) NewItem))
  ;[1 1 1] If is inside quiver or bag remove it
  (Utilities|IsValid _quiverorbag
    (:Is%20Valid
      (Default|RemoveItemfromBagorQuiver _quiverorbag NewItem)
      (return _returnvalue))))

(fn GetItemIndexonArray
  (params (ItemToCheckIndex :type BP%20GOTA%20Item%20Max%20Par%20Class%20I%20Object%20Reference))
  (return (Utilities|Array|FindItem (Variables|Default|GetItemsInInv) ItemToCheckIndex)))

(fn GetNextEquipableItem
  (params (StartingInvPoint :type Integer))
  (bind _itemsininv (Variables|Default|GetItemsInInv))
  (Variables|Default|SetCachedLastItemIndexIterated StartingInvPoint)
  (for (_ _array_index) _itemsininv
    (if (Math|Boolean|ANDBoolean (not (.bSuccess (Utilities|Casting|CastToBP_GOTAShield (Utilities|Array|Get(acopy) _itemsininv (+ (Variables|Default|GetCachedLastItemIndexIterated) 1))))) (not (.bSuccess (Utilities|Casting|CastToBP_GOTAArmour (Utilities|Array|Get(acopy) _itemsininv (+ (Variables|Default|GetCachedLastItemIndexIterated) 1))))) (Utilities|IsValid (Utilities|Array|Get(acopy) _itemsininv (+ (Variables|Default|GetCachedLastItemIndexIterated) 1))) (!= (Utilities|Array|Get(acopy) _itemsininv (+ (Variables|Default|GetCachedLastItemIndexIterated) 1)) (Variables|Default|GetPrimaryItem)))
      (return (Utilities|Array|Get(acopy) _itemsininv (+ (Variables|Default|GetCachedLastItemIndexIterated) 1)))
      (else
        (Math|Integer|IncrementInt (Variables|Default|GetCachedLastItemIndexIterated)))))
  (Variables|Default|SetCachedLastItemIndexIterated 0)
  (for _array_element _itemsininv
    (if (Math|Boolean|ANDBoolean (not (.bSuccess (Utilities|Casting|CastToBP_GOTAArmour (Utilities|Array|Get(acopy) _itemsininv (Variables|Default|GetCachedLastItemIndexIterated))))) (not (.bSuccess (Utilities|Casting|CastToBP_GOTAShield (Utilities|Array|Get(acopy) _itemsininv (Variables|Default|GetCachedLastItemIndexIterated))))) (Utilities|IsValid (Utilities|Array|Get(acopy) _itemsininv (Variables|Default|GetCachedLastItemIndexIterated))) (!= (Utilities|Array|Get(acopy) _itemsininv (Variables|Default|GetCachedLastItemIndexIterated)) (Variables|Default|GetPrimaryItem)))
      (return 0)
      (else
        (Math|Integer|IncrementInt (Variables|Default|GetCachedLastItemIndexIterated)))))
  (return 0))

(fn GetPreviousEquipableItem
  (params (StartingInvPoint :type Integer))
  (bind _itemsininv (Variables|Default|GetItemsInInv))
  (bind _output_get (Variables|Default|SetCachedLastItemIndexIterated StartingInvPoint))
  (for (_array_element _array_index) _itemsininv
    (if (Math|Boolean|ANDBoolean (not (.bSuccess (Utilities|Casting|CastToBP_GOTAShield (Utilities|Array|Get(acopy) _itemsininv (+ (Variables|Default|GetCachedLastItemIndexIterated) -1))))) (not (.bSuccess (Utilities|Casting|CastToBP_GOTAArmour (Utilities|Array|Get(acopy) _itemsininv (+ (Variables|Default|GetCachedLastItemIndexIterated) -1))))) (Utilities|IsValid (Utilities|Array|Get(acopy) _itemsininv (+ (Variables|Default|GetCachedLastItemIndexIterated) -1))) (!= (Utilities|Array|Get(acopy) _itemsininv (+ (Variables|Default|GetCachedLastItemIndexIterated) -1)) (Variables|Default|GetPrimaryItem)))
      (return (Utilities|Array|Get(acopy) _itemsininv (+ (Variables|Default|GetCachedLastItemIndexIterated) -1)))
      (else
        (Math|Integer|DecrementInt (Variables|Default|GetCachedLastItemIndexIterated)))))
  (Variables|Default|SetCachedLastItemIndexIterated (- (Utilities|Array|Length _itemsininv) 1))
  (for _array_element_2 _itemsininv
    (if (Math|Boolean|ANDBoolean (not (.bSuccess (Utilities|Casting|CastToBP_GOTAArmour (Utilities|Array|Get(acopy) _itemsininv (Variables|Default|GetCachedLastItemIndexIterated))))) (not (.bSuccess (Utilities|Casting|CastToBP_GOTAShield (Utilities|Array|Get(acopy) _itemsininv (Variables|Default|GetCachedLastItemIndexIterated))))) (Utilities|IsValid (Utilities|Array|Get(acopy) _itemsininv (Variables|Default|GetCachedLastItemIndexIterated))) (!= (Utilities|Array|Get(acopy) _itemsininv (Variables|Default|GetCachedLastItemIndexIterated)) (Variables|Default|GetPrimaryItem)))
      (return 0)
      (else
        (Math|Integer|DecrementInt (Variables|Default|GetCachedLastItemIndexIterated)))))
  (return 0))

(fn OnRepPrimaryItem
  (bind _returnvalue (Components|GetOwner))
  (bind _primaryitem (Variables|Default|GetPrimaryItem))
  (Networking|SwitchHasAuthority
    (:Authority
      _)
    (:Remote
      _))
  (Utilities|FlowControl|Sequence
    (:then_0
      ;[1 1 1] Update it a lot of times just in case
      (bind _ascharacter (Utilities|Casting|CastToCharacter _returnvalue))
      (if (Pawn|IsPlayerControlled _ascharacter)
        (Utilities|Casting|CastToBP_GOTAPCMaxParClass (Pawn|GetController _ascharacter))
        ;;[1 1 1] Becareful or may not empty it ( set it invisible the right pannel)
        (Utilities|IsValid _primaryitem
          (:Is%20Valid
            (CallFunction|ClientDoRDisplayWeap _primaryitem (Variables|/Game/GOTA2/Blueprints/InventoryAndItems/BP_GOTAItemMaxParClassI.BP_GOTAItemMaxParClassI_C|GetDurability _primaryitem)))
          (:Is%20Not%20Valid
            (CallFunction|ClientDoRDisplayWeap)))))
    (:then_1
      (Utilities|Casting|CastToBP_GOTATHItem _primaryitem)
      (bind _asbp_gotachar_max_par_class (Utilities|Casting|CastToBP_GOTACharMaxParClass _returnvalue))
      (Transformation|AttachComponentToComponent (Variables|/Game/GOTA2/Blueprints/Characters/BP_GOTACharMaxParClass.BP_GOTACharMaxParClass_C|GetLeftArmWeapon _asbp_gotachar_max_par_class) (Variables|/Script/Engine.Character|GetMesh _asbp_gotachar_max_par_class) "LeftHandSocketFalx" "SnapToTarget" "SnapToTarget" "KeepRelative" true))))

(fn OnRepSecondaryItem
  (bind _secondaryitem (Variables|Default|GetSecondaryItem))
  ;[1 1 1] Update it a lot of times just in case
  (Networking|SwitchHasAuthority
    (:Authority
      _)
    (:Remote
      _))
  (bind _ascharacter (Utilities|Casting|CastToCharacter (Components|GetOwner)))
  (if (Pawn|IsPlayerControlled _ascharacter)
    (Utilities|Casting|CastToBP_GOTAPCMaxParClass (Pawn|GetController _ascharacter))
    (Utilities|IsValid _secondaryitem
      (:Is%20Valid
        (CallFunction|ClientDoLDisplayWeap _secondaryitem (Variables|/Game/GOTA2/Blueprints/InventoryAndItems/BP_GOTAItemMaxParClassI.BP_GOTAItemMaxParClassI_C|GetDurability _secondaryitem)))
      (:Is%20Not%20Valid
        (CallFunction|ClientDoLDisplayWeap)))
    (bind _asbp_gotashield (Utilities|Casting|CastToBP_GOTAShield _secondaryitem))
    (if (Variables|/Game/GOTA2/Blueprints/InventoryAndItems/BP_GOTAShield.BP_GOTAShield_C|GetbScutumShieldKind _asbp_gotashield)
      (bind _asbp_gotachar_max_par_class (Utilities|Casting|CastToBP_GOTACharMaxParClass _ascharacter))
      (Transformation|AttachComponentToComponent (Variables|/Game/GOTA2/Blueprints/Characters/BP_GOTACharMaxParClass.BP_GOTACharMaxParClass_C|GetLeftArmWeapon _asbp_gotachar_max_par_class) (Variables|/Script/Engine.Character|GetMesh _asbp_gotachar_max_par_class) "LeftHandSocketScutum" "SnapToTarget" "SnapToTarget" "KeepRelative" true))))

(fn SpawnItemfromArchetypeTemplate
  (params (NewArchetype :type BP%20GOTA%20Item%20Max%20Par%20Class%20I%20Class%20Reference) (NewDura :type Integer) (TransformToSpawnAt :type Transform) (SpeificOwner :type Actor%20Object%20Reference))
  (bind _returnvalue (Game|SpawnActorfromClass NewArchetype TransformToSpawnAt "AdjustIfPossibleButAlwaysSpawn" SpeificOwner NewDura "1.000000,1.000000,1.000000" false 0))
  (return _returnvalue))

(fn SpawnRandomItemOfClass
  (params (NewArchetype :type EN_WeaponItemTypeEnum%20Enum :default "NewEnumerator0") (NewDura :type Integer) (TransformToSpawnAt :type Transform) (SpeificOwner :type Actor%20Object%20Reference))
  (bind _onehandedarchetypes (Variables|Default|GetOneHandedArchetypes))
  (bind _speararchetypes (Variables|Default|GetSpearArchetypes))
  (bind _bowarchetypes (Variables|Default|GetBowArchetypes))
  (bind _torsoarmorarchetypes (Variables|Default|GetTorsoArmorArchetypes))
  (bind _quiverarchetypeswip (Variables|Default|GetQuiverArchetypesWIP))
  (bind _foodarchetypes (Variables|Default|GetFoodArchetypes))
  (bind _twohandedarchetypes (Variables|Default|GetTwoHandedArchetypes))
  (bind _legsarmorarchetypes (Variables|Default|GetLegsArmorArchetypes))
  (bind _shieldarchetypesroundshield (Variables|Default|GetShieldArchetypesRoundShield))
  (bind _shieldarchetypesscutum (Variables|Default|GetShieldArchetypesScutum))
  (bind _headarmorarchetypes (Variables|Default|GetHeadArmorArchetypes))
  (switch Utilities|FlowControl|Switch|SwitchonEN_WeaponItemTypeEnum NewArchetype
    (:NewEnumerator0
      (bind _newitem (CallFunction|SpawnItemfromArchetypeTemplate (Utilities|Array|Get(acopy) _onehandedarchetypes (Math|Random|RandomInteger (Utilities|Array|Length _onehandedarchetypes))) NewDura TransformToSpawnAt SpeificOwner))
      (return _newitem))
    (:NewEnumerator3
      (bind _newitem_2 (CallFunction|SpawnItemfromArchetypeTemplate (Utilities|Array|Get(acopy) _speararchetypes (Math|Random|RandomInteger (Utilities|Array|Length _speararchetypes))) NewDura TransformToSpawnAt SpeificOwner))
      (return _newitem_2))
    (:NewEnumerator4
      (bind _newitem_3 (CallFunction|SpawnItemfromArchetypeTemplate (Utilities|Array|Get(acopy) _twohandedarchetypes (Math|Random|RandomInteger (Utilities|Array|Length _twohandedarchetypes))) NewDura TransformToSpawnAt SpeificOwner))
      (return _newitem_3))
    (:NewEnumerator5
      (bind _newitem_4 (CallFunction|SpawnItemfromArchetypeTemplate (Utilities|Array|Get(acopy) _shieldarchetypesroundshield (Math|Random|RandomInteger (Utilities|Array|Length _shieldarchetypesroundshield))) NewDura TransformToSpawnAt SpeificOwner))
      (return _newitem_4))
    (:NewEnumerator6
      (bind _newitem_5 (CallFunction|SpawnItemfromArchetypeTemplate (Utilities|Array|Get(acopy) _shieldarchetypesscutum (Math|Random|RandomInteger (Utilities|Array|Length _shieldarchetypesscutum))) NewDura TransformToSpawnAt SpeificOwner))
      (return _newitem_5))
    (:NewEnumerator8
      (bind _newitem_6 (CallFunction|SpawnItemfromArchetypeTemplate (Utilities|Array|Get(acopy) _foodarchetypes (Math|Random|RandomInteger (Utilities|Array|Length _foodarchetypes))) NewDura TransformToSpawnAt SpeificOwner))
      (return _newitem_6))
    (:NewEnumerator9
      (bind _newitem_7 (CallFunction|SpawnItemfromArchetypeTemplate (Utilities|Array|Get(acopy) _headarmorarchetypes (Math|Random|RandomInteger (Utilities|Array|Length _headarmorarchetypes))) NewDura TransformToSpawnAt SpeificOwner))
      (return _newitem_7))
    (:NewEnumerator10
      (bind _newitem_8 (CallFunction|SpawnItemfromArchetypeTemplate (Utilities|Array|Get(acopy) _torsoarmorarchetypes (Math|Random|RandomInteger (Utilities|Array|Length _torsoarmorarchetypes))) NewDura TransformToSpawnAt SpeificOwner))
      (return _newitem_8))
    (:NewEnumerator11
      (bind _newitem_9 (CallFunction|SpawnItemfromArchetypeTemplate (Utilities|Array|Get(acopy) _legsarmorarchetypes (Math|Random|RandomInteger (Utilities|Array|Length _legsarmorarchetypes))) NewDura TransformToSpawnAt SpeificOwner))
      (return _newitem_9))
    (:NewEnumerator12
      (bind _newitem_10 (CallFunction|SpawnItemfromArchetypeTemplate (Utilities|Array|Get(acopy) _bowarchetypes (Math|Random|RandomInteger (Utilities|Array|Length _bowarchetypes))) NewDura TransformToSpawnAt SpeificOwner))
      (return _newitem_10))
    (:NewEnumerator13
      (bind _newitem_11 (CallFunction|SpawnItemfromArchetypeTemplate (Utilities|Array|Get(acopy) _quiverarchetypeswip (Math|Random|RandomInteger (Utilities|Array|Length _quiverarchetypeswip))) NewDura TransformToSpawnAt SpeificOwner))
      (return _newitem_11))))

(fn IsInventoryFull
  (return (>= (Utilities|Array|Length (Variables|Default|GetItemsInInv)) (Variables|Default|GetInvItemLimit))))

(fn HasQuiver
  (return (Variables|Default|GetQuiverOrBag)))