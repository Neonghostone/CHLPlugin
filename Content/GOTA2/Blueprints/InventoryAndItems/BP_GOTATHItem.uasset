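; Melee weapon item that fills the primary slot, clears the secondary, shows on the character's left-arm mesh and can be thrown.
; Tick runs capped, server-only combo traces during attacks, spins and traces the item in its projectile state, and draws trails.
; Blade traces sweep sockets from their previous positions into damage-or-block handling.
; Throwing hides held meshes and launches the item mesh from the right hand via projectile movement.
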(event EventBeginPlay
  (|CallParentFunction) ; This node is disabled and will not be called.\nDrag off pins to build functionality.
)

(event Collision|EventActorBeginOverlap
  (params (OtherActor :type Actor%20Object%20Reference))
  (|CallParentFunction OtherActor) ; This node is disabled and will not be called.\nDrag off pins to build functionality.
)

(event EventTick
  (params (DeltaSeconds :type Float%20%28single-precision%29))
  (Utilities|FlowControl|Sequence
    (:then_0
      (Networking|SwitchHasAuthority
        (:Authority
          (if (Variables|Default|GetbTracing)
            (if (< (Variables|Default|GetTracesNum) (Variables|Default|GetMaxTraces))
              (if (Class|KismetSystemLibrary|IsTimerActive 0 "TimerBasedCooldownUnleashAttack")
                (CallFunction|DefinitiveComboTrace)
                (Variables|Default|SetTracesNum (+ (Variables|Default|GetTracesNum) 1))))))))
    (:then_1
      (if (Utilities|Enum|Equal(Enum) (Variables|Default|GetEnumItemState) "NewEnumerator8")
        (Transformation|AddLocalRotation (Variables|Default|GetItemStatMesh) "0.000000,15.000000,0.000000" false false)
        (if (> (Math|Vector|VectorLength (Variables|Default|GetLastLocVector)) 0.0)
          (CallFunction|PerformProjectileTrace)
          (else
            (Variables|Default|SetLastLocVector (Transformation|GetActorLocation))))))
    (:then_2
      (CallFunction|DrawTrailCloud))))

(event EventEquip
  (bind _asbp_gotachar_max_par_class (Utilities|Casting|CastToBP_GOTACharMaxParClass (Components|GetOwner)))
  (Default|SetSecondaryItem (Variables|/Game/GOTA2/Blueprints/Characters/BP_GOTACharMaxParClass.BP_GOTACharMaxParClass_C|GetInvReference _asbp_gotachar_max_par_class))
  (Default|SetPrimaryItem (Variables|/Game/GOTA2/Blueprints/Characters/BP_GOTACharMaxParClass.BP_GOTACharMaxParClass_C|GetInvReference _asbp_gotachar_max_par_class) self)
  (Class|SkinnedMeshComponent|SetSkeletalMesh (Variables|/Game/GOTA2/Blueprints/Characters/BP_GOTACharMaxParClass.BP_GOTACharMaxParClass_C|GetRightArmWeapon _asbp_gotachar_max_par_class) 0 true)
  (Variables|/Game/GOTA2/Blueprints/Characters/BP_GOTACharMaxParClass.BP_GOTACharMaxParClass_C|SetRepnoSkeletalMeshRight _asbp_gotachar_max_par_class 0)
  (Utilities|IsValid (Variables|/Game/GOTA2/Blueprints/Characters/BP_GOTACharMaxParClass.BP_GOTACharMaxParClass_C|GetInvReference _asbp_gotachar_max_par_class)
    (:Is%20Valid
      (Variables|/Game/GOTA2/Blueprints/Characters/BP_GOTACharMaxParClass.BP_GOTACharMaxParClass_C|SetRepnoSkeletalMeshLeft _asbp_gotachar_max_par_class (Variables|Default|GetSkeleMeshToEquip))
      (Variables|Default|SetbPicked true)
      (Variables|Default|SetbProtecting false)
      (Variables|Default|SetbMinLoadTime false)
      (Variables|Default|SetbLeftHold false)
      (Variables|Default|SetbPreparedAttack false)
      (Utilities|Array|SetArrayElem :TargetArray (Variables|Default|GetLastLocationsMulti))
      ;[1 1 1] So the blade will work fine
      (CallFunction|ResetforEquip)
      (Transformation|DetachFromComponent (Variables|Default|GetItemStatMesh) "KeepWorld" "KeepWorld" "KeepWorld" true)
      (Variables|Default|SetbStuckOnSurface false)
      (CallFunction|ClearHitActorsAndassingNewLastLocs)
      (Variables|/Game/GOTA2/Blueprints/Characters/BP_GOTACharMaxParClass.BP_GOTACharMaxParClass_C|SetRepnoWeapTypeForAnimBP _asbp_gotachar_max_par_class "NewEnumerator4")
      (Variables|/Game/GOTA2/Blueprints/Characters/BP_GOTACharMaxParClass.BP_GOTACharMaxParClass_C|SetRepnoLeftScale _asbp_gotachar_max_par_class (Variables|Default|GetEquippingScale))
      (Variables|/Game/GOTA2/Blueprints/Characters/BP_GOTACharMaxParClass.BP_GOTACharMaxParClass_C|SetSpecialAttackNum _asbp_gotachar_max_par_class 0))))

(event EventMultiSocketTraceBlade
  (bind _returnvalue (Components|GetOwner))
  (bind _socketsfortracing (Variables|Default|GetSocketsForTracing))
  (bind _lastlocationsmulti (Variables|Default|GetLastLocationsMulti))
  (if (== (Math|Vector|VectorLength (Utilities|Array|Get(acopy) _lastlocationsmulti)) 0.0)
    (for (_ _array_index) _lastlocationsmulti
      (bind _asbp_gotachar_max_par_class (Utilities|Casting|CastToBP_GOTACharMaxParClass _returnvalue))
      (Utilities|Array|SetArrayElem _lastlocationsmulti _array_index (Transformation|GetSocketLocation (Variables|/Game/GOTA2/Blueprints/Characters/BP_GOTACharMaxParClass.BP_GOTACharMaxParClass_C|GetLeftArmWeapon _asbp_gotachar_max_par_class) (Utilities|String|StringToName (Utilities|Array|Get(acopy) _socketsfortracing _array_index)))))
    (else
      (for (_array_element _array_index_2) _socketsfortracing
        (bind _asbp_gotachar_max_par_class_2 (Utilities|Casting|CastToBP_GOTACharMaxParClass _returnvalue))
        (bind _hitresult (CallFunction|CORECollisionTraceStartEndPoint (Utilities|Array|Get(acopy) (Variables|Default|GetLastLocationsMulti) _array_index_2) (Transformation|GetSocketLocation (Variables|/Game/GOTA2/Blueprints/Characters/BP_GOTACharMaxParClass.BP_GOTACharMaxParClass_C|GetLeftArmWeapon _asbp_gotachar_max_par_class_2) (Utilities|String|StringToName _array_element))))
        (CallFunction|ProcessHitResultsDoDamageorBlock _hitresult)
        (Utilities|Array|SetArrayElem _lastlocationsmulti _array_index_2 (Transformation|GetSocketLocation (Variables|/Game/GOTA2/Blueprints/Characters/BP_GOTACharMaxParClass.BP_GOTACharMaxParClass_C|GetLeftArmWeapon _asbp_gotachar_max_par_class_2) (Utilities|String|StringToName _array_element)))))))

(event EventLineTracefromHIlttoTip
  (bind _asbp_gotachar_max_par_class (Utilities|Casting|CastToBP_GOTACharMaxParClass (Components|GetOwner)))
  (CallFunction|CORECollisionTraceStartEndPoint (Transformation|GetSocketLocation (Variables|/Game/GOTA2/Blueprints/Characters/BP_GOTACharMaxParClass.BP_GOTACharMaxParClass_C|GetLeftArmWeapon _asbp_gotachar_max_par_class) (Utilities|String|StringToName (Variables|Default|GetHiltSock))) (Transformation|GetSocketLocation (Variables|/Game/GOTA2/Blueprints/Characters/BP_GOTACharMaxParClass.BP_GOTACharMaxParClass_C|GetLeftArmWeapon _asbp_gotachar_max_par_class) (Utilities|String|StringToName (Variables|Default|GetTipSock)))))

(event EventSpawnAppearProjectileforThrow
  (params (ProjVelo :type Vector :default "0, 0, 0") (LocToSpawn :type Vector :default "0, 0, 0") (FinalPower :type Float%20%28single-precision%29) (ShouldActivateParticles :type Boolean))
  (bind _itemprojectilemodephysics (Variables|Default|GetItemProjectileModePhysics))
  (bind _itemprojectilemodephysics_2 (Variables|Default|GetItemProjectileModePhysics))
  (Utilities|FlowControl|Sequence
    (:then_0
      (bind _asbp_gotachar_max_par_class (Utilities|Casting|CastToBP_GOTACharMaxParClass (Components|GetOwner)))
      ;[1 1 1] Let's null the two just in case
      (Variables|/Game/GOTA2/Blueprints/Characters/BP_GOTACharMaxParClass.BP_GOTACharMaxParClass_C|SetRepnoSkeletalMeshLeft _asbp_gotachar_max_par_class 0)
      (Variables|/Game/GOTA2/Blueprints/Characters/BP_GOTACharMaxParClass.BP_GOTACharMaxParClass_C|SetRepnoSkeletalMeshRight _asbp_gotachar_max_par_class 0)
      (Variables|/Script/Engine.ProjectileMovementComponent|SetProjectileGravityScale _itemprojectilemodephysics_2 1.0)
      (Variables|/Script/Engine.ProjectileMovementComponent|SetInitialSpeed _itemprojectilemodephysics 1e+03)
      (Components|Activation|Deactivate _itemprojectilemodephysics_2)
      (Rendering|SetVisibility (Variables|Default|GetItemStatMesh) true true)
      (Transformation|SetActorLocationAndRotation (Transformation|GetSocketLocation (Variables|/Script/Engine.Character|GetMesh (.AsBP%20GOTAChar%20Max%20Par%20Class (Utilities|Casting|CastToBP_GOTACharMaxParClass (Components|GetOwner)))) "RightHandSocket") (Transformation|GetActorRotation (Components|GetOwner)) false true)
      (Components|Movement|SetUpdatedComponent _itemprojectilemodephysics (Variables|Default|GetItemStatMesh))
      (Utilities|FlowControl|Delay 0.0)
      (Components|Activation|Activate _itemprojectilemodephysics true)
      (bind _output_get (Variables|/Script/Engine.MovementComponent|SetVelocity (Variables|Default|GetItemProjectileModePhysics) (* ProjVelo (* FinalPower (Variables|Default|GetThrowMultiplierPower)))))
      (Collision|SetCollisionEnabled (Variables|Default|GetItemStatMesh) "QueryAndPhysics")
      (Variables|Default|SetbPicked false))))

(event EventUnequip
  (bind _asbp_gotachar_max_par_class (Utilities|Casting|CastToBP_GOTACharMaxParClass (Components|GetOwner)))
  (Default|SetPrimaryItem (Variables|/Game/GOTA2/Blueprints/Characters/BP_GOTACharMaxParClass.BP_GOTACharMaxParClass_C|GetInvReference _asbp_gotachar_max_par_class))
  (Class|SkinnedMeshComponent|SetSkeletalMesh (Variables|/Game/GOTA2/Blueprints/Characters/BP_GOTACharMaxParClass.BP_GOTACharMaxParClass_C|GetRightArmWeapon _asbp_gotachar_max_par_class) 0 true)
  (Variables|/Game/GOTA2/Blueprints/Characters/BP_GOTACharMaxParClass.BP_GOTACharMaxParClass_C|SetRepnoSkeletalMeshRight _asbp_gotachar_max_par_class 0)
  (Utilities|IsValid (Variables|/Game/GOTA2/Blueprints/Characters/BP_GOTACharMaxParClass.BP_GOTACharMaxParClass_C|GetInvReference _asbp_gotachar_max_par_class)
    (:Is%20Valid
      (Variables|/Game/GOTA2/Blueprints/Characters/BP_GOTACharMaxParClass.BP_GOTACharMaxParClass_C|SetRepnoSkeletalMeshLeft _asbp_gotachar_max_par_class 0)
      ;[1 1 1] Not sure why here
      (Variables|Default|SetbPicked true)
      (Variables|Default|SetbProtecting false)
      (Variables|Default|SetbMinLoadTime false)
      (Variables|Default|SetbLeftHold false)
      (Variables|Default|SetbPreparedAttack false)
      (Utilities|Array|SetArrayElem :TargetArray (Variables|Default|GetLastLocationsMulti))
      ;[1 1 1] So the blade will work fine
      (CallFunction|ResetforEquip)
      (Transformation|DetachFromComponent (Variables|Default|GetItemStatMesh) "KeepWorld" "KeepWorld" "KeepWorld" true)
      (Variables|Default|SetbStuckOnSurface false)
      (CallFunction|ClearHitActorsAndassingNewLastLocs)
      (Variables|/Game/GOTA2/Blueprints/Characters/BP_GOTACharMaxParClass.BP_GOTACharMaxParClass_C|SetSpecialAttackNum _asbp_gotachar_max_par_class 0))))

(fn ConstructionScript
  (|CallParentFunction))