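; BP_FoodItem is an edible item that restores the eater's health when HandleGetEaten fires.
; Each bite sets the eater's animation state, briefly stops its movement and, after a delay, damages the food itself.
; A delay-based cooldown blocks rapid bites with a localized red warning to the eater's controller.
; When the bite ends, it resets the animation, plays an eat sound through player controller 0 and calls the OneBite dispatcher.
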(event Custom|HandleGetEaten
  (params (Eater :type BP%20GOTA%20Char%20Max%20Par%20Class%20Object%20Reference))
  (bind _returnvalue (Components|GetOwner))
  (bind _returnvalue_2 (Transformation|GetActorLocation _returnvalue))
  ;[1 1 1] Eat functionality
  (if (Variables|Default|GetbEatingCooldown)
    (bind _asbp_gotapcmax_par_class (Utilities|Casting|CastToBP_GOTAPCMaxParClass (Pawn|GetController Eater)))
    (Default|ClientAddMessage _asbp_gotapcmax_par_class (Utilities|String|ToString(Name) (Utilities|Array|Get(acopy) (Variables|Default|GetDontEatTooFastMulti) (Math|Conversions|ToInteger(Byte) (Variables|/Game/GOTA2/Blueprints/Controllers/BP_GOTAPCMaxParClass.BP_GOTAPCMaxParClass_C|GetPlayerLanguage _asbp_gotapcmax_par_class)))) 2.0 (Math|Color|MakeColor 0 0 255 255))
    (else
      (Variables|/Game/GOTA2/Blueprints/Characters/BP_GOTACharMaxParClass.BP_GOTACharMaxParClass_C|SetReplicatedAnimState Eater "NewEnumerator21")
      (Default|RecoverHealth Eater 50)
      (Default|ServerStopMovementandEnableAgain Eater 1.5)
      (Variables|Default|SetbEatingCooldown true)
      (Utilities|FlowControl|Delay 0.5)
      (Default|ActorTakeDamage self 25 _returnvalue_2 "0, 0, 0" "" "NewEnumerator0" true 25.0 false 0.0 0.0 (Collision|MakeHitResult false false 0.0 0.0 _returnvalue_2 "0, 0, 0" "0,0,1" "0,0,1" 0 0) 0 "0, 0, 0" "NewEnumerator0")
      (Utilities|FlowControl|Delay 1.0)
      (Variables|Default|SetbEatingCooldown false)
      (Variables|/Game/GOTA2/Blueprints/Characters/BP_GOTACharMaxParClass.BP_GOTACharMaxParClass_C|SetReplicatedAnimState Eater "NewEnumerator0")
      (bind _asbp_gotapcmax_par_class_2 (Utilities|Casting|CastToBP_GOTAPCMaxParClass (Game|GetPlayerController 0)))
      (Default|ServerPlaySound _asbp_gotapcmax_par_class_2 (Transformation|GetActorLocation Eater) "/Game/GOTA2/Audio/CU_EatSound.CU_EatSound")
      (Default|CallEventDispatcherOneBite))))

(event EventBeginPlay
  (|CallParentFunction) ; This node is disabled and will not be called.\nDrag off pins to build functionality.
)

(event Collision|EventActorBeginOverlap
  (params (OtherActor :type Actor%20Object%20Reference))
  (|CallParentFunction OtherActor) ; This node is disabled and will not be called.\nDrag off pins to build functionality.
)

(event EventTick
  (params (DeltaSeconds :type Float%20%28single-precision%29))
  (|CallParentFunction DeltaSeconds) ; This node is disabled and will not be called.\nDrag off pins to build functionality.
)

(fn ConstructionScript
  (|CallParentFunction))