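; Torso armour item that puts its skeletal mesh and tunic morph mode on the owning GOTA character.
; Equip registers it as the inventory's torso armour, picks the female or default mesh by character class, marks it picked and copies the owner's team number.
; The mesh goes through a RepNotify variable, while TunicMode is set directly and flagged as not replicated.
; Unequip clears the mesh and TunicMode, leaving the inventory reference set.
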(event EventBeginPlay
  (|CallParentFunction) ; This node is disabled and will not be called.\nDrag off pins to build functionality.
)

(event Collision|EventActorBeginOverlap
  (params (OtherActor :type Actor%20Object%20Reference))
  (|CallParentFunction OtherActor) ; This node is disabled and will not be called.\nDrag off pins to build functionality.
)

(event EventTick
  (params (DeltaSeconds :type Float%20%28single-precision%29))
  (|CallParentFunction DeltaSeconds) ; This node is disabled and will not be called.\nDrag off pins to build functionality.
)

(event EventUnequip
  (bind _asbp_gotachar_max_par_class (Utilities|Casting|CastToBP_GOTACharMaxParClass (Components|GetOwner)))
  (Variables|/Game/GOTA2/Blueprints/Characters/BP_GOTACharMaxParClass.BP_GOTACharMaxParClass_C|SetRepnoSkeletalMeshTorsoArmour _asbp_gotachar_max_par_class 0)
  (Variables|/Game/GOTA2/Blueprints/Characters/BP_GOTACharMaxParClass.BP_GOTACharMaxParClass_C|SetbTunicMode _asbp_gotachar_max_par_class false))

(event EventEquip
  (bind _returnvalue (Components|GetOwner))
  (bind _returnvalue_2 (Components|GetOwner))
  (bind _skelemeshtoequipfemale (Variables|Default|GetSkeleMeshToEquipFemale))
  (bind _skelemeshtoequip (Variables|Default|GetSkeleMeshToEquip))
  (bind _asbp_gotachar_max_par_class (Utilities|Casting|CastToBP_GOTACharMaxParClass _returnvalue))
  (|CallParentFunction)
  (bind _asbp_gotachar_max_par_class_2 (Utilities|Casting|CastToBP_GOTACharMaxParClass _returnvalue_2))
  (Variables|/Game/GOTA2/Blueprints/InventoryAndItems/BP_GOTAInvMaxParClassInclBag.BP_GOTAInvMaxParClassInclBag_C|SetTorsoArmour (Variables|/Game/GOTA2/Blueprints/Characters/BP_GOTACharMaxParClass.BP_GOTACharMaxParClass_C|GetInvReference _asbp_gotachar_max_par_class_2) self)
  (Utilities|FlowControl|Sequence
    (:then_0
      (Utilities|Casting|CastToBP_GOTAGirlMaxParClass _asbp_gotachar_max_par_class_2
        (:then
          (Utilities|IsValid _skelemeshtoequipfemale
            (:Is%20Valid
              (Variables|/Game/GOTA2/Blueprints/Characters/BP_GOTACharMaxParClass.BP_GOTACharMaxParClass_C|SetRepnoSkeletalMeshTorsoArmour _asbp_gotachar_max_par_class_2 _skelemeshtoequipfemale))
            (:Is%20Not%20Valid
              _)))
        (:CastFailed
          (Utilities|IsValid _skelemeshtoequip
            (:Is%20Valid
              (Variables|/Game/GOTA2/Blueprints/Characters/BP_GOTACharMaxParClass.BP_GOTACharMaxParClass_C|SetRepnoSkeletalMeshTorsoArmour _asbp_gotachar_max_par_class_2 _skelemeshtoequip))
            (:Is%20Not%20Valid
              _))))
      (Variables|Default|SetbPicked true)
      ;[1 1 1] This may cause bug, NOT REPLICATED
      (if (Variables|Default|GetNeed%20Tunic%20Morph)
        (Variables|/Game/GOTA2/Blueprints/Characters/BP_GOTACharMaxParClass.BP_GOTACharMaxParClass_C|SetbTunicMode _asbp_gotachar_max_par_class true)
        (else
          (Variables|/Game/GOTA2/Blueprints/Characters/BP_GOTACharMaxParClass.BP_GOTACharMaxParClass_C|SetbTunicMode _asbp_gotachar_max_par_class false))))
    (:then_1
      (bind _asbp_gotachar_max_par_class_3 (Utilities|Casting|CastToBP_GOTACharMaxParClass _returnvalue_2))
      (Variables|Default|SetTeamRepInteger (Variables|/Game/GOTA2/Blueprints/Characters/BP_GOTACharMaxParClass.BP_GOTACharMaxParClass_C|GetTeamNumInt _asbp_gotachar_max_par_class_3)))))

(fn ConstructionScript
  (|CallParentFunction))