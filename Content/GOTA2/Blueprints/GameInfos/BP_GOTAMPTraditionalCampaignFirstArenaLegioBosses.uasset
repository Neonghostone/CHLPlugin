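; Game mode for the multiplayer traditional campaign's first arena Legio bosses match, built on a parent game-info Blueprint.
; While the match has not started, PostLogin runs the parent logic, announces the joining player controller, plays a random peaceful music track and switches that player to UI-only input with the mouse shown.
; HandlePawnDied is deliberately empty, so a pawn's death does not win the match.
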(event EventBeginPlay
  (|CallParentFunction) ; This node is disabled and will not be called.\nDrag off pins to build functionality.
)

(event EventTick
  (params (DeltaSeconds :type Float%20%28single-precision%29))
  (|CallParentFunction DeltaSeconds) ; This node is disabled and will not be called.\nDrag off pins to build functionality.
)

(event EventPostLogin
  (params (NewPlayer :type Player%20Controller%20Object%20Reference))
  (switch Utilities|FlowControl|Switch|SwitchonEN_GameInfoMatchState (Variables|Default|GetGameInfoState)
    (:NewEnumerator0
      (|CallParentFunction NewPlayer)
      (bind _asbp_gotapcmax_par_class (Utilities|Casting|CastToBP_GOTAPCMaxParClass NewPlayer))
      (Default|CallPlayerJoinedtotheGame _asbp_gotapcmax_par_class)
      (Default|SetSongPlayingTrack1 _asbp_gotapcmax_par_class (.OutItem (Utilities|Array|Random (Variables|Default|GetPeacefulMusic))))
      (Input|SetInputModeUIOnly NewPlayer 0 "DoNotLock")
      (Default|ClientShowMouse _asbp_gotapcmax_par_class true))))

(event EventHandlePawnDied
  (params (DiedPawn :type BP%20GOTA%20Char%20Max%20Par%20Class%20Object%20Reference))
  ;[1 1 1] Do not win when pawn dies
)

(fn ConstructionScript
  (|CallParentFunction))