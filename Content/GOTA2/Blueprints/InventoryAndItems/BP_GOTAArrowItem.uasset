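; BP_GOTAArrowItem is an arrow inventory item that can be stored, held, or shot as a projectile.
; Equip adds it to a valid quiver or bag; otherwise it sets the owner's right-hand mesh and can become the primary item unless a shooting weapon holds that slot.
; Fire inputs drive attacks and protecting, deferring to an equipped shield.
; Projectile handlers toggle the ArrowFew particle, disable collision on sticking, and make released arrows non-pickable.
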(event Custom|HandleGetShoRreleased
  (params (LastOwner :type Actor%20Object%20Reference))
  (Actor|SetOwner 0)
  (bind _aspawn (Utilities|Casting|CastToPawn LastOwner))
  (Variables|Default|SetLastOwner _aspawn)
  (Variables|Default|SetbPickable false))

(event EventBeginPlay
  (Audio|Components|Audio|Stop (Variables|Default|GetArrowFew))
  (|CallParentFunction))

(event Collision|EventActorBeginOverlap
  (params (OtherActor :type Actor%20Object%20Reference))
  (|CallParentFunction OtherActor) ; This node is disabled and will not be called.\nDrag off pins to build functionality.
)

(event EventTick
  (params (DeltaSeconds :type Float%20%28single-precision%29))
  (|CallParentFunction DeltaSeconds) ; This node is disabled and will not be called.\nDrag off pins to build functionality.
)

(event EventEquip
  (bind _skelemeshtoequip (Variables|Default|GetSkeleMeshToEquip))
  (bind _asbp_gotachar_max_par_class (Utilities|Casting|CastToBP_GOTACharMaxParClass (Components|GetOwner)))
  (Utilities|IsValid (Variables|/Game/GOTA2/Blueprints/Characters/BP_GOTACharMaxParClass.BP_GOTACharMaxParClass_C|GetInvReference _asbp_gotachar_max_par_class)
    (:Is%20Valid
      (Utilities|IsValid (Variables|/Game/GOTA2/Blueprints/InventoryAndItems/BP_GOTAInvMaxParClassInclBag.BP_GOTAInvMaxParClassInclBag_C|GetQuiverOrBag (Variables|/Game/GOTA2/Blueprints/Characters/BP_GOTACharMaxParClass.BP_GOTACharMaxParClass_C|GetInvReference _asbp_gotachar_max_par_class))
        (:Is%20Valid
          (Default|AddIteminQuiverorBag (Variables|/Game/GOTA2/Blueprints/InventoryAndItems/BP_GOTAInvMaxParClassInclBag.BP_GOTAInvMaxParClassInclBag_C|GetQuiverOrBag (Variables|/Game/GOTA2/Blueprints/Characters/BP_GOTACharMaxParClass.BP_GOTACharMaxParClass_C|GetInvReference _asbp_gotachar_max_par_class)) self))
        (:Is%20Not%20Valid
          (Class|SkinnedMeshComponent|SetSkeletalMesh (Variables|/Game/GOTA2/Blueprints/Characters/BP_GOTACharMaxParClass.BP_GOTACharMaxParClass_C|GetRightArmWeapon _asbp_gotachar_max_par_class) _skelemeshtoequip true)
          (Utilities|IsValid (Variables|/Game/GOTA2/Blueprints/Characters/BP_GOTACharMaxParClass.BP_GOTACharMaxParClass_C|GetInvReference _asbp_gotachar_max_par_class)
            (:Is%20Valid
              (Utilities|Casting|CastToBP_GOTAShootingWeapon (Variables|/Game/GOTA2/Blueprints/InventoryAndItems/BP_GOTAInvMaxParClassInclBag.BP_GOTAInvMaxParClassInclBag_C|GetPrimaryItem (Variables|/Game/GOTA2/Blueprints/Characters/BP_GOTACharMaxParClass.BP_GOTACharMaxParClass_C|GetInvReference _asbp_gotachar_max_par_class))
                (:then
                  _)
                (:CastFailed
                  (Default|SetPrimaryItem (Variables|/Game/GOTA2/Blueprints/Characters/BP_GOTACharMaxParClass.BP_GOTACharMaxParClass_C|GetInvReference _asbp_gotachar_max_par_class) self)))
              (Variables|Default|SetbPicked true)
              (Variables|Default|SetbProtecting false)
              (Variables|Default|SetbMinLoadTime false)
              (Variables|Default|SetbLeftHold false)
              (Variables|Default|SetbPreparedAttack false)
              (Utilities|Array|SetArrayElem :TargetArray (Variables|Default|GetLastLocationsMulti))
              ;[1 1 1] So the blade will work fine
              (CallFunction|ResetforEquip)
              (Transformation|DetachFromComponent (Variables|Default|GetItemStatMesh) "KeepWorld" "KeepWorld" "KeepWorld" true)
              (Variables|Default|SetbStuckOnSurface false)
              (Variables|/Game/GOTA2/Blueprints/Characters/BP_GOTACharMaxParClass.BP_GOTACharMaxParClass_C|SetRepnoSkeletalMeshRight _asbp_gotachar_max_par_class _skelemeshtoequip)
              (Variables|/Game/GOTA2/Blueprints/Characters/BP_GOTACharMaxParClass.BP_GOTACharMaxParClass_C|SetRepnoRightScale _asbp_gotachar_max_par_class (Variables|Default|GetEquippingScale)))))))))

(event EventStartFire
  (params (FireModeNum :type Byte :default 0))
  (bind _asbp_gotachar_max_par_class (Utilities|Casting|CastToBP_GOTACharMaxParClass (Components|GetOwner)))
  (switch Utilities|FlowControl|Switch|SwitchonEN_PawnState (Variables|/Game/GOTA2/Blueprints/Characters/BP_GOTACharMaxParClass.BP_GOTACharMaxParClass_C|GetPawnState _asbp_gotachar_max_par_class)
    (:NewEnumerator0
      (switch Utilities|FlowControl|Switch|SwitchonEN_AnimState (Variables|/Game/GOTA2/Blueprints/Characters/BP_GOTACharMaxParClass.BP_GOTACharMaxParClass_C|GetReplicatedAnimState _asbp_gotachar_max_par_class)
        (:NewEnumerator0
          (bind _asbp_gotachar_max_par_class_2 (Utilities|Casting|CastToBP_GOTACharMaxParClass (Components|GetOwner)))
          (switch int (Math|Conversions|ToInteger(Byte) FireModeNum)
            (:0
              (Variables|Default|SetbLeftHold true)
              (CallFunction|StartAttack FireModeNum))
            (:1
              (Utilities|Casting|CastToBP_GOTAShield (Variables|/Game/GOTA2/Blueprints/InventoryAndItems/BP_GOTAInvMaxParClassInclBag.BP_GOTAInvMaxParClassInclBag_C|GetSecondaryItem (Variables|/Game/GOTA2/Blueprints/Characters/BP_GOTACharMaxParClass.BP_GOTACharMaxParClass_C|GetInvReference _asbp_gotachar_max_par_class_2))
                (:then
                  (if (not (Variables|Default|GetbPreparedAttack))
                    (Default|StartProtecting (Variables|/Game/GOTA2/Blueprints/InventoryAndItems/BP_GOTAInvMaxParClassInclBag.BP_GOTAInvMaxParClassInclBag_C|GetSecondaryItem (Variables|/Game/GOTA2/Blueprints/Characters/BP_GOTACharMaxParClass.BP_GOTACharMaxParClass_C|GetInvReference _asbp_gotachar_max_par_class_2)))))
                (:CastFailed
                  (if (not (Variables|Default|GetbPreparedAttack))
                    (CallFunction|StartProtecting)))))))))))

(event EventStopFIre
  (params (FireModeNum :type Byte :default 0))
  (bind _asbp_gotachar_max_par_class (Utilities|Casting|CastToBP_GOTACharMaxParClass (Components|GetOwner)))
  (switch Utilities|FlowControl|Switch|SwitchonEN_PawnState (Variables|/Game/GOTA2/Blueprints/Characters/BP_GOTACharMaxParClass.BP_GOTACharMaxParClass_C|GetPawnState _asbp_gotachar_max_par_class)
    (:NewEnumerator0
      (switch int (Math|Conversions|ToInteger(Byte) FireModeNum)
        (:0
          (Variables|Default|SetbLeftHold false)
          (if (not (Variables|Default|GetbMinLoadTime))
            (CallFunction|UnleashAttack)))
        (:1
          (bind _asbp_gotashield (Utilities|Casting|CastToBP_GOTAShield (Variables|/Game/GOTA2/Blueprints/InventoryAndItems/BP_GOTAInvMaxParClassInclBag.BP_GOTAInvMaxParClassInclBag_C|GetSecondaryItem (Variables|/Game/GOTA2/Blueprints/Characters/BP_GOTACharMaxParClass.BP_GOTACharMaxParClass_C|GetInvReference _asbp_gotachar_max_par_class)))
            (:then
              (if (not (Variables|Default|GetbPreparedAttack))
                (Default|StopProtecting _asbp_gotashield)))
            (:CastFailed
              (if (not (Variables|Default|GetbPreparedAttack))
                (CallFunction|StartProtecting)))))))))

(event EventProjectileGetStuckonSurface
  (params (SurfaceAct :type Actor%20Object%20Reference) (HitRes :type Hit%20Result%20Structure))
  (Collision|SetCollisionEnabled (Variables|Default|GetItemStatMesh) "NoCollision")
  (|CallParentFunction SurfaceAct HitRes))

(event EventUnequip)

(event EventHandleGetThrownforParticle
  (params (Activate :type Boolean))
  (bind _arrowfew (Variables|Default|GetArrowFew))
  (if Activate
    (Components|Activation|Activate _arrowfew false)
    (else
      (Audio|Components|Audio|Stop _arrowfew)))
  (|CallParentFunction Activate))

(fn ConstructionScript
  (|CallParentFunction))