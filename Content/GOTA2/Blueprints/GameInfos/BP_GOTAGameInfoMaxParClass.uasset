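; Parent game mode for GOTA gladiator matches, running match flow, music, bonuses and broadcasts to player controllers.
; BeginPlay loads or creates option and campaign saves, applies item rules and starts match-clock updates; PostLogin sets up HUD and music.
; HandlePawnDied tallies team deaths to detect a last-team win, then plays victory for every controller regardless of team and server-travels.
; Aggressive music reverts on a refreshable timer; several travel and game-state paths are WIP or deprecated.
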(event Custom|ChangeLaguageForAll
  (params (NewLanguage :type EN_Language%20Enum :default "NewEnumerator0"))
  (Variables|Default|SetServerLanguageTakenEnum NewLanguage)
  (bind _outactors (Actor|GetAllActorsOfClass "/Game/GOTA2/Blueprints/Controllers/BP_GOTAPCMaxParClass.BP_GOTAPCMaxParClass_C"))
  (for _array_element _outactors
    (Default|StartChangeLanguageNow _array_element NewLanguage)
    (Default|ClientAddMessage _array_element (Utilities|String|Append "Game: changing Language to " (Utilities|String|EnumtoString NewLanguage)) 2.0 (Math|Color|MakeColor 255 255 255 255))))

(event Custom|MakeAllPickable
  (params (MakeAllPickable :type Boolean))
  (bind _outactors (Actor|GetAllActorsOfClass "/Game/GOTA2/Blueprints/InventoryAndItems/BP_GOTAItemMaxParClassI.BP_GOTAItemMaxParClassI_C"))
  (for _array_element _outactors
    (Utilities|Casting|CastToBP_GOTADestChunkMaxPar _array_element)
    (Variables|/Game/GOTA2/Blueprints/InventoryAndItems/BP_GOTAItemMaxParClassI.BP_GOTAItemMaxParClassI_C|SetbPickable _array_element MakeAllPickable)))

(event Custom|HandleCommonPawnVictorious
  ;[1 1 1] Handle match end types WIP
  (Variables|Default|SetMatchEndedAlready true))

(event Custom|HandleCommonPawnDefeat
  ;[1 1 1] Handle match end types WIP
  (Variables|Default|SetMatchEndedAlready true))

(event Custom|HandleCommonDraw
  (params (reason :type String))
  ;[1 1 1] Handle match end types WIP
  (if (not (Variables|Default|GetMatchEndedAlready))
    (bind _outactors (Actor|GetAllActorsOfClass "/Game/GOTA2/Blueprints/Controllers/BP_GOTAPCMaxParClass.BP_GOTAPCMaxParClass_C"))
    (for _array_element _outactors
      (Default|ClientPlayDraw _array_element reason))
    (Variables|Default|SetMatchEndedAlready true)
    (Utilities|Time|SetTimerbyEvent (delegate Custom|HandleQuitAfterTimeDraw) (Variables|Default|GetTimeToQuitAfterDraw))))

(event Custom|TurnAllPawnsInmortal
  ;[1 1 1] Miscellenous
  (bind _outactors (Actor|GetAllActorsOfClass "/Game/GOTA2/Blueprints/Characters/BP_GOTACharMaxParClass.BP_GOTACharMaxParClass_C"))
  (for _array_element _outactors
    (Default|ToggleBecomeInmortal _array_element)))

(event Custom|HandleQuitAfterTimeDraw
  ;[1 1 1] Open main menu after some time, in case this is multiplayer should load another level
  (bind _outactors (Actor|GetAllActorsOfClass "/Game/GOTA2/Blueprints/Controllers/BP_GOTAPCMaxParClass.BP_GOTAPCMaxParClass_C"))
  (if (> (Utilities|Array|Length _outactors) 1)
    (CallFunction|PerformServerTravel "Same Level")
    (else
      (Game|OpenLevel(byName) "OfficialMainMenuGladiatorAlone"))))

(event Custom|PerformServerTravel
  (params (levelName :type String))
  ;[1 1 1] DEPRA NOT WORKING
  (Development|ExecuteConsoleCommand "ServerTravel" 0)
  (bind _returnvalue (Game|GetCurrentLevelName true))
  (Game|OpenLevel(byName) (Utilities|String|StringToName _returnvalue) true "listen"))

(event Custom|bHandleVicitoryOrDefat
  (params (WinnerTeam :type Integer))
  (bind _outactors (Actor|GetAllActorsOfClass "/Game/GOTA2/Blueprints/Characters/BP_GOTACharMaxParClass.BP_GOTACharMaxParClass_C"))
  (bind _array_element (Utilities|Array|ForEachLoopwithBreak _outactors)
    (:LoopBody
      (switch Utilities|FlowControl|Switch|SwitchonEN_PawnState (Variables|/Game/GOTA2/Blueprints/Characters/BP_GOTACharMaxParClass.BP_GOTACharMaxParClass_C|GetPawnState _array_element)
        (:NewEnumerator0
          (bind _asbp_gotaaicmax_par_class (Utilities|Casting|CastToBP_GOTAAICMaxParClass (Pawn|GetController _array_element)))
          (Default|GotoState _asbp_gotaaicmax_par_class (Variables|/Game/GOTA2/Blueprints/Controllers/BP_GOTAAICMaxParClass.BP_GOTAAICMaxParClass_C|GetState _asbp_gotaaicmax_par_class) "NewEnumerator5"))))))

(event Custom|HandleServerTravelFromGameInfo
  ;[1 1 1] Victory conditions sometimes the Player controllers won't play the victorious movie ?
  (bind _returnvalue (Game|GetCurrentLevelName true))
  (Development|ExecuteConsoleCommand (Utilities|String|Append "ServerTravel " _returnvalue "?listen") 0))

(event Custom|HandleNewBonification
  (params (NewBoni :type ST%20Bonification%20Structure) (GladiatorToReceiveIt :type BP%20GOTA%20Char%20Max%20Par%20Class%20Object%20Reference))
  (bind (_nameofbonification _entertainmentpointsgettingbydef) (Utilities|Struct|BreakST_Bonification NewBoni))
  (Default|SetNewEntertainment GladiatorToReceiveIt _entertainmentpointsgettingbydef)
  (Default|ServerSideSetLastEntertainmentBoni GladiatorToReceiveIt _nameofbonification)
  (bind _asbp_gotapcmax_par_class (Utilities|Casting|CastToBP_GOTAPCMaxParClass (Pawn|GetController GladiatorToReceiveIt)))
  (Default|ClientHandlePlaybonification _asbp_gotapcmax_par_class NewBoni))

(event Custom|GoToGameState
  (params (GameState :type EN_GameInfoMatchState%20Enum :default "NewEnumerator0"))
  ;[1 1 1] WIP
  (bind _output_get (Variables|Default|SetGameInfoState GameState))
  (switch Utilities|FlowControl|Switch|SwitchonEN_GameInfoMatchState _output_get))

(event Custom|MakeAllThrowable
  (params (bNewThrowable :type Boolean))
  ;[1 1 1] Except Spears and such
  (bind _outactors (Actor|GetAllActorsOfClass "/Game/GOTA2/Blueprints/InventoryAndItems/BP_GOTAItemMaxParClassI.BP_GOTAItemMaxParClassI_C"))
  (for _array_element _outactors
    (Utilities|Casting|CastToBP_GOTABowItem _array_element
      (:CastFailed
        (Utilities|Casting|CastToBP_GOTASpearItem _array_element
          (:CastFailed
            (Variables|/Game/GOTA2/Blueprints/InventoryAndItems/BP_GOTAItemMaxParClassI.BP_GOTAItemMaxParClassI_C|SetbCanBeThrown _array_element bNewThrowable)))))))

(event Custom|PlayerJoinedWIthHUDReady
  (params (PCJoined :type BP%20GOTAPC%20Max%20Par%20Class%20Object%20Reference) (HUDMovieReady :type UW%20Main%20HUD%20Object%20Reference))
  ;[1 1 1] WIP just in case here is needed
  (Development|PrintString (Utilities|String|Append "FROM GmaeiNfo the hud is resteed the playe is" (Utilities|GetDisplayName PCJoined) "Movie is" (Utilities|GetDisplayName HUDMovieReady))))

(event Custom|CountDown321Ofgame
  ;[0.6504 1 0.6169] Countdown
  (Utilities|FlowControl|Delay 3.0)
  (Default|CallGameStartsCountDownEnds))

(event Custom|HandlePawnDied
  (params (DiedPawn :type BP%20GOTA%20Char%20Max%20Par%20Class%20Object%20Reference))
  (bind _returnvalue (Pawn|GetController DiedPawn))
  (bind (_bshouldendgame _winnerteam) (CallFunction|BShouldbeWinnerTEAM))
  (bind _pawnstate (Variables|/Game/GOTA2/Blueprints/Characters/BP_GOTACharMaxParClass.BP_GOTACharMaxParClass_C|GetPawnState DiedPawn))
  (bind _returnvalue_2 (Utilities|Enum|Equal(Enum) _pawnstate "NewEnumerator2"))
  (Utilities|FlowControl|Sequence
    (:then_0
      ;[1 1 1] Seconds to get possessed by spectator
      (Default|GetSpectatorGIven DiedPawn))
    (:then_1
      ;[1 1 1] Player dies, make things happen
      (if (Class|KismetSystemLibrary|IsStandalone)
        (bind _asbp_gotapcmax_par_class (Utilities|Casting|CastToBP_GOTAPCMaxParClass _returnvalue))
        (if _returnvalue_2
          (Default|ClientPlayDefeat _asbp_gotapcmax_par_class)
          (Default|ServerHandleEndGame _asbp_gotapcmax_par_class true)
          (Default|ServerHandleEndGame _asbp_gotapcmax_par_class true))
        (else
          (bind _asbp_gotapcmax_par_class_2 (Utilities|Casting|CastToBP_GOTAPCMaxParClass _returnvalue))
          (if _returnvalue_2
            (Default|ClientPlayDefeat _asbp_gotapcmax_par_class_2)
            (Default|ServerHandleEndGame _asbp_gotapcmax_par_class_2 true)))))
    (:then_2
      ;[1 1 1] Count how many dead glads per team
      (switch int (Variables|/Game/GOTA2/Blueprints/Characters/BP_GOTACharMaxParClass.BP_GOTACharMaxParClass_C|GetTeamNumInt DiedPawn)
        (:0
          (Math|Integer|IncrementInt (Variables|Default|GetTeam0DeadGladsFreeForAll)))
        (:1
          (Math|Integer|IncrementInt (Variables|Default|GetTeam1DeadGlads)))
        (:2
          (Math|Integer|IncrementInt (Variables|Default|GetTeam2DeadGlads)))
        (:3
          (Math|Integer|IncrementInt (Variables|Default|GetTeam3DeadGlads)))
        (:4
          (Math|Integer|IncrementInt (Variables|Default|GetTeam4DeadGlads)))))
    (:then_3
      ;[1 1 1] So we know later who wins assign dead teams
      (CallFunction|BRegisterDeadTeams))
    (:then_4
      ;[1 1 1] Victory conditions sometimes the Player controllers won't play the victorious movie ?
      (if _bshouldendgame
        (bind _outactors (Actor|GetAllActorsOfClass "/Game/GOTA2/Blueprints/Controllers/BP_GOTAPCMaxParClass.BP_GOTAPCMaxParClass_C"))
        (bind _array_element (Utilities|Array|ForEachLoopwithBreak _outactors)
          (:LoopBody
            ;;[1 1 1] Becareful it wins or wins if team is dead
            (if (== _winnerteam (Variables|/Game/GOTA2/Blueprints/Controllers/BP_GOTAPCMaxParClass.BP_GOTAPCMaxParClass_C|GetPlayerTeam _array_element))
              _
              (else
                _))
            (Default|ClientPlayVictorious _array_element)
            ;;[1 1 1] So you can indeed restart later on use game state
            (Default|ServerHandleEndGame _array_element true))
          (:Completed
            (Utilities|FlowControl|Delay 5.0)
            (Development|ExecuteConsoleCommand (Utilities|String|Append "ServerTravel " (stale Custom|HandleServerTravelFromGameInfo _returnvalue) "?listen") 0)))))))

(event Custom|MakeAllthrowableWithBow
  (params (bNewThrowableByBow :type Boolean))
  ;[1 1 1] This is WIP
  (bind _outactors (Actor|GetAllActorsOfClass "/Game/GOTA2/Blueprints/InventoryAndItems/BP_GOTAItemMaxParClassI.BP_GOTAItemMaxParClassI_C"))
  (for _array_element _outactors
    _))

(event Custom|InstanceForAllPlayersDialogueText
  (params (Visiblity :type ESlateVisibility%20Enum :default "Visible") (NewTextVisibility :type String))
  ;[1 1 1] For campaigns and stuff
  (bind _outactors (Actor|GetAllActorsOfClass "/Game/GOTA2/Blueprints/Controllers/BP_GOTAPCMaxParClass.BP_GOTAPCMaxParClass_C"))
  (for _array_element _outactors
    (Default|ClientSetDialTextNewVisibleSetText _array_element Visiblity NewTextVisibility)))

(event Custom|StartPeaceFulTime
  (bind _peacefulmusic (Variables|Default|GetPeacefulMusic))
  (bind _outactors (Actor|GetAllActorsOfClass "/Game/GOTA2/Blueprints/Controllers/BP_GOTAPCMaxParClass.BP_GOTAPCMaxParClass_C"))
  (for _array_element _outactors
    (Variables|/Game/GOTA2/Blueprints/Controllers/BP_GOTAPCMaxParClass.BP_GOTAPCMaxParClass_C|SetSongPlayingTrack1 _array_element (Utilities|Array|Get(acopy) _peacefulmusic (Math|Random|RandomIntegerinRange 0 (- (Utilities|Array|Length _peacefulmusic) 1))))))

(event Custom|StartAgressiveTime
  (bind _agressivemusic (Variables|Default|GetAgressiveMusic))
  (if (Utilities|Time|IsTimerActivebyHandle (Variables|Default|GetPeaceAgainSongTHandle))
    (Utilities|Time|ClearandInvalidateTimerbyHandle (Variables|Default|GetPeaceAgainSongTHandle))
    (bind _returnvalue (Utilities|Time|SetTimerbyEvent (delegate Custom|StartPeaceFulTime) (Variables|Default|GetFloatTimeForPeaceSong)))
    (Variables|Default|SetPeaceAgainSongTHandle _returnvalue)
    (else
      (bind _outactors (Actor|GetAllActorsOfClass "/Game/GOTA2/Blueprints/Controllers/BP_GOTAPCMaxParClass.BP_GOTAPCMaxParClass_C"))
      (for _array_element _outactors
        (Default|SetSongPlayingTrack2 _array_element (Utilities|Array|Get(acopy) _agressivemusic (Math|Random|RandomIntegerinRange 0 (- (Utilities|Array|Length _agressivemusic) 1)))))
      (bind _returnvalue_2 (Utilities|Time|SetTimerbyEvent (delegate Custom|StartPeaceFulTime) (Variables|Default|GetFloatTimeForPeaceSong)))
      (Variables|Default|SetPeaceAgainSongTHandle _returnvalue_2))))

(event Custom|AddMessageForAll
  (params (Message :type String) (Duration :type Float%20%28single-precision%29) (ColorOfMessage :type Color%20Structure))
  ;[0.8111 0.02299 1] Message for all
  (bind _outactors (Actor|GetAllActorsOfClass "/Game/GOTA2/Blueprints/Controllers/BP_GOTAPCMaxParClass.BP_GOTAPCMaxParClass_C"))
  (for _array_element _outactors
    (Default|ClientAddMessage _array_element Message Duration ColorOfMessage)))

(event Custom|UpdateEndTimer
  ;[0 0.837 1] End timer
  (bind _outactors (Actor|GetAllActorsOfClass "/Game/GOTA2/Blueprints/Controllers/BP_GOTAPCMaxParClass.BP_GOTAPCMaxParClass_C"))
  (for _array_element _outactors
    (Default|ClientUpdateNewTime _array_element (Math|Float|Truncate (Utilities|Time|GetTimerRemainingTimebyHandle (Variables|Default|GetMatchEndTHandle))))))

(event EventBeginPlay
  (Utilities|FlowControl|Sequence
    (:then_0
      ;[1 1 1] Load the options if they exist and load the variables that are there, bHasPassed tutorial
      (bind _returnvalue (SaveGame|LoadGamefromSlot "options"))
      (bind _asbp_gotasave_options_max_par (Utilities|Casting|CastToBP_GOTASaveOptionsMaxPar _returnvalue))
      (Utilities|IsValid _asbp_gotasave_options_max_par
        (:Is%20Valid
          (Variables|Default|SetbGMRAMCanThrowNonThrowableItems (Variables|/Game/GOTA2/Blueprints/SaveSystem/BP_GOTASaveOptionsMaxPar.BP_GOTASaveOptionsMaxPar_C|GetbAlllThrowable _asbp_gotasave_options_max_par))
          (Variables|Default|SetbGMRAMCanPickAllItems (Variables|/Game/GOTA2/Blueprints/SaveSystem/BP_GOTASaveOptionsMaxPar.BP_GOTASaveOptionsMaxPar_C|GetbAllPickable _asbp_gotasave_options_max_par))
          (Variables|Default|SetbGMRAMCanShootAllWithBow (Variables|/Game/GOTA2/Blueprints/SaveSystem/BP_GOTASaveOptionsMaxPar.BP_GOTASaveOptionsMaxPar_C|GetbAllBowable _asbp_gotasave_options_max_par))
          (Variables|Default|SetbGMRAMRevive (Variables|/Game/GOTA2/Blueprints/SaveSystem/BP_GOTASaveOptionsMaxPar.BP_GOTASaveOptionsMaxPar_C|GetbReviveFallsFloor _asbp_gotasave_options_max_par))
          (CallFunction|MakeAllThrowable (Variables|Default|GetbGMRAMCanThrowNonThrowableItems))
          (CallFunction|MakeAllPickable (Variables|Default|GetbGMRAMCanPickAllItems))
          (CallFunction|MakeAllthrowablewithBow (Variables|Default|GetbGMRAMCanShootAllWithBow))
          (Utilities|FlowControl|Delay 2.0))))
    (:then_2
      ;[0 0.837 1] End timer
      (bind _returnvalue_2 (Utilities|Time|SetTimerbyEvent (delegate Custom|UpdateEndTimer) 1.0 true))
      (Variables|Default|SetTimeUpdaterTimer _returnvalue_2))
    (:then_3
      ;[0 1.6e-05 1] Save options, not sure why but i set a varaible on it.... Investigate it....
      (bind _returnvalue_3 (SaveGame|LoadGamefromSlot "options"))
      (Utilities|IsValid _returnvalue_3
        (:Is%20Valid
          (bind _asbp_gotasave_options_max_par_2 (Utilities|Casting|CastToBP_GOTASaveOptionsMaxPar _returnvalue_3))
          (Variables|Default|SetServerLanguageTakenEnum (Variables|/Game/GOTA2/Blueprints/SaveSystem/BP_GOTASaveOptionsMaxPar.BP_GOTASaveOptionsMaxPar_C|GetLanguage _asbp_gotasave_options_max_par_2)))
        (:Is%20Not%20Valid
          (bind _returnvalue_4 (SaveGame|CreateSaveGameObject "/Game/GOTA2/Blueprints/SaveSystem/BP_GOTASaveOptionsMaxPar.BP_GOTASaveOptionsMaxPar_C"))
          (SaveGame|SaveGametoSlot _returnvalue_4 "options"))))
    (:then_4
      ;[1 0.4383 0] Save options, campaign, create at the beginning if it does not exist
      (bind _returnvalue_5 (SaveGame|LoadGamefromSlot "campaign"))
      (Utilities|IsValid _returnvalue_5
        (:Is%20Not%20Valid
          (bind _returnvalue_6 (SaveGame|CreateSaveGameObject "/Game/GOTA2/Blueprints/SaveSystem/BP_GOTACampaignSaveSystem.BP_GOTACampaignSaveSystem_C"))
          (SaveGame|SaveGametoSlot _returnvalue_6 "campaign"))))))

(event EventTick
  (params (DeltaSeconds :type Float%20%28single-precision%29))
  (|CallParentFunction DeltaSeconds))

(event EventPostLogin
  (params (NewPlayer :type Player%20Controller%20Object%20Reference))
  (bind _peacefulmusic (Variables|Default|GetPeacefulMusic))
  (bind _asbp_gotapcmax_par_class (Utilities|Casting|CastToBP_GOTAPCMaxParClass NewPlayer))
  (Default|ClientShowtheHUD _asbp_gotapcmax_par_class)
  (Default|CallPlayerJoinedtotheGame _asbp_gotapcmax_par_class)
  (Default|SetSongPlayingTrack1 _asbp_gotapcmax_par_class (Utilities|Array|Get(acopy) _peacefulmusic (Math|Random|RandomIntegerinRange 0 (- (Utilities|Array|Length _peacefulmusic) 1))))
  (Utilities|FlowControl|Delay 1.0)
  (bind _asbp_gotapcmax_par_class_2 (Utilities|Casting|CastToBP_GOTAPCMaxParClass NewPlayer))
  (bind _asbp_gotahudmax_par_class (Utilities|Casting|CastToBP_GOTAHUDMaxParClass (HUD|GetHUD _asbp_gotapcmax_par_class_2)))
  (Default|SetCombatHUDVisible (Variables|/Game/GOTA2/Blueprints/HUD/BP_GOTAHUDMaxParClass.BP_GOTAHUDMaxParClass_C|GetMainHUDMovie _asbp_gotahudmax_par_class) "Visible"))

(fn ConstructionScript)

(fn BAllDead
  (bind _array_element (Utilities|Array|ForEachLoopwithBreak (CallFunction|ReturnAllGaldiators))
    (:LoopBody
      (if (Utilities|Enum|NotEqual(Enum) (Variables|/Game/GOTA2/Blueprints/Characters/BP_GOTACharMaxParClass.BP_GOTACharMaxParClass_C|GetPawnState _array_element) "NewEnumerator2")
        (return false)))
    (:Completed
      (return true))))

(fn ReturnAllGaldiators
  (bind _allglads (LocalVariables|GetAllGlads))
  (bind _outactors (Actor|GetAllActorsOfClass "/Game/GOTA2/Blueprints/Characters/BP_GOTACharMaxParClass.BP_GOTACharMaxParClass_C"))
  (for _array_element _outactors
    (Utilities|Casting|CastToBP_GOTASpectatorMaxParentClass _array_element
      (:CastFailed
        (Utilities|Array|Add _allglads _array_element))))
  (return _allglads))

(fn BAllDeadButOne
  (bind _allgladiators (CallFunction|ReturnAllGaldiators))
  (bind _array_element (Utilities|Array|ForEachLoopwithBreak _allgladiators)
    (:LoopBody
      (if (Utilities|Enum|Equal(Enum) (Variables|/Game/GOTA2/Blueprints/Characters/BP_GOTACharMaxParClass.BP_GOTACharMaxParClass_C|GetPawnState _array_element) "NewEnumerator2")
        (LocalVariables|SetCountDeadPeople (+ (LocalVariables|GetCountDeadPeople) 1))
        (else
          (LocalVariables|SetCachedTheOnylOneLeftAlive _array_element))))
    (:Completed
      (bind _outactors (Actor|GetAllActorsOfClass "/Game/GOTA2/Blueprints/Controllers/BP_GOTAPCMaxParClass.BP_GOTAPCMaxParClass_C"))
      (for _array_element_2 _outactors
        (Default|ClientAddMessage _array_element_2 (Utilities|String|Append (Utilities|Array|Get(acopy) (Variables|Default|GetMultiMessageForAllClientsGladiatorsLeft) (Math|Conversions|ToInteger(Byte) (Variables|/Game/GOTA2/Blueprints/Controllers/BP_GOTAPCMaxParClass.BP_GOTAPCMaxParClass_C|GetPlayerLanguage _array_element_2))) (Utilities|String|ToString(Byte) (LocalVariables|GetCountDeadPeople))) 2.0 (Math|Color|MakeColor 0 255 255 255)))
      (return (== (LocalVariables|GetCountDeadPeople) (Math|Conversions|ToByte(Integer) (- (Utilities|Array|Length _allgladiators) 1))) (LocalVariables|GetCachedTheOnylOneLeftAlive)))))

(fn BThereIsWinnerTeamDEPRA
  (bind _allgladiators (CallFunction|ReturnAllGaldiators))
  (bind _array_element (Utilities|Array|ForEachLoopwithBreak _allgladiators)
    (:LoopBody
      (if (Utilities|Enum|Equal(Enum) (Variables|/Game/GOTA2/Blueprints/Characters/BP_GOTACharMaxParClass.BP_GOTACharMaxParClass_C|GetPawnState _array_element) "NewEnumerator2")
        (LocalVariables|SetCountDeadPeople (+ (LocalVariables|GetCountDeadPeople) 1))
        (else
          (LocalVariables|SetCachedTheOnylOneLeftAlive _array_element))))
    (:Completed
      (bind _outactors (Actor|GetAllActorsOfClass "/Game/GOTA2/Blueprints/Controllers/BP_GOTAPCMaxParClass.BP_GOTAPCMaxParClass_C"))
      (for _array_element_2 _outactors
        (Default|ClientAddMessage _array_element_2 (Utilities|String|Append (Utilities|Array|Get(acopy) (Variables|Default|GetMultiMessageForAllClientsGladiatorsLeft) (Math|Conversions|ToInteger(Byte) (Variables|/Game/GOTA2/Blueprints/Controllers/BP_GOTAPCMaxParClass.BP_GOTAPCMaxParClass_C|GetPlayerLanguage _array_element_2))) (Utilities|String|ToString(Byte) (LocalVariables|GetCountDeadPeople))) 2.0 (Math|Color|MakeColor 0 255 255 255)))
      (return (== (LocalVariables|GetCountDeadPeople) (Math|Conversions|ToByte(Integer) (- (Utilities|Array|Length _allgladiators) 1))) (LocalVariables|GetCachedTheOnylOneLeftAlive)))))

(fn BShouldbeWinnerTEAM
  (bind _t1isdead (Variables|Default|GetT1IsDead))
  (bind _t2isdead (Variables|Default|GetT2IsDead))
  (bind _t3isdead (Variables|Default|GetT3IsDead))
  (bind _t4isdead (Variables|Default|GetT4IsDead))
  (bind _t0isdeadfreeforall (Variables|Default|GetT0IsDeadFreeForAll))
  (Utilities|FlowControl|Sequence
    (:then_0
      (if (Math|Boolean|ANDBoolean _t1isdead _t2isdead _t3isdead _t4isdead (== (- (Variables|Default|GetInitialTeam0GladiatorsFreeForAll) (Variables|Default|GetTeam0DeadGladsFreeForAll)) 1))
        (return true 0)))
    (:then_1
      (if (Math|Boolean|ANDBoolean _t1isdead _t2isdead _t3isdead _t0isdeadfreeforall)
        (return true 4)))
    (:then_2
      (if (Math|Boolean|ANDBoolean _t1isdead _t2isdead _t4isdead _t0isdeadfreeforall)
        (return true 3)))
    (:then_3
      (if (Math|Boolean|ANDBoolean _t1isdead _t3isdead _t4isdead _t0isdeadfreeforall)
        (return true 2)))
    (:then_4
      (if (Math|Boolean|ANDBoolean _t2isdead _t3isdead _t4isdead _t0isdeadfreeforall)
        (return true 4)))
    (:then_5
      (return false 0))))

(fn BRegisterDeadTeams
  (Variables|Default|SetT1IsDead (== (Variables|Default|GetInitialTeam1Gladiators) (Variables|Default|GetTeam1DeadGlads)))
  (Variables|Default|SetT2IsDead (== (Variables|Default|GetInitialTeam2Gladiators) (Variables|Default|GetTeam2DeadGlads)))
  (Variables|Default|SetT3IsDead (== (Variables|Default|GetInitialTeam3Gladiators) (Variables|Default|GetTeam3DeadGlads)))
  (Variables|Default|SetT4IsDead (== (Variables|Default|GetInitialTeam4Gladiators) (Variables|Default|GetTeam4DeadGlads)))
  (Variables|Default|SetT0IsDeadFreeForAll (== (Variables|Default|GetInitialTeam0GladiatorsFreeForAll) (Variables|Default|GetTeam0DeadGladsFreeForAll))))

(fn ReturnCampaignSaveGame
  (bind _returnvalue (SaveGame|LoadGamefromSlot "campaign"))
  (Utilities|IsValid _returnvalue
    (:Is%20Valid
      (bind _asbp_gotacampaign_save_system (Utilities|Casting|CastToBP_GOTACampaignSaveSystem _returnvalue))
      (return _asbp_gotacampaign_save_system))
    (:Is%20Not%20Valid
      (bind _outactors (Actor|GetAllActorsOfClass "/Game/GOTA2/Blueprints/Controllers/BP_GOTAPCMaxParClass.BP_GOTAPCMaxParClass_C"))
      (Default|ClientAddMessage _outactors "ERROR ERROR No Save Game Exists!!!!" 2.0 (Math|Conversions|ToColor(LinearColor) (Math|Color|MakeColor 1.0 0.0 0.0))))))