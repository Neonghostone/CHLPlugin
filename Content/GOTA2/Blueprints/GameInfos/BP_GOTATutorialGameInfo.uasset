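; Game mode Blueprint for the GOTA tutorial, handling player login and combat HUD setup.
; One second after PostLogin, it casts the new player's controller and HUD to the MaxParClass types and sets combat HUD visibility on the main HUD movie.
; The HandleEndMatchbyTimer event is left empty, with no match-end logic attached.
; BeginPlay and Tick are disabled placeholders.
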(event EventBeginPlay
  (|CallParentFunction) ; This node is disabled and will not be called.\nDrag off pins to build functionality.
)

(event EventTick
  (params (DeltaSeconds :type Float%20%28single-precision%29))
  (|CallParentFunction DeltaSeconds) ; This node is disabled and will not be called.\nDrag off pins to build functionality.
)

(event EventHandleEndMatchbyTimer)

(event EventPostLogin
  (params (NewPlayer :type Player%20Controller%20Object%20Reference))
  (Utilities|FlowControl|Delay 1.0)
  (bind _asbp_gotapcmax_par_class (Utilities|Casting|CastToBP_GOTAPCMaxParClass NewPlayer))
  (bind _asbp_gotahudmax_par_class (Utilities|Casting|CastToBP_GOTAHUDMaxParClass (HUD|GetHUD _asbp_gotapcmax_par_class)))
  (Default|SetCombatHUDVisible (Variables|/Game/GOTA2/Blueprints/HUD/BP_GOTAHUDMaxParClass.BP_GOTAHUDMaxParClass_C|GetMainHUDMovie _asbp_gotahudmax_par_class) "Visible"))

(fn ConstructionScript
  (|CallParentFunction))