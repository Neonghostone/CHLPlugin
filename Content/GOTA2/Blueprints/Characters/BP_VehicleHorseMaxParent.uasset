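; Parent Blueprint for a rideable horse that GOTA characters can mount and dismount through server-side possession swaps.
; GetRiden stores the rider, possesses the horse with its controller, snaps it to the mesh's RidingSocket, disables its collision and sets a riding animation state.
; ServerUse detaches the rider, returns possession, restores capsule collision, resets both meshes' rotation and changes the replicated animation state back.
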(event Custom|GetRiden
  (params (Rider :type Character%20Object%20Reference))
  ;[1 0 0.83] Gets called from server
  (bind _asbp_gotachar_max_par_class (Utilities|Casting|CastToBP_GOTACharMaxParClass Rider))
  (Variables|/Game/GOTA2/Blueprints/Characters/BP_GOTACharMaxParClass.BP_GOTACharMaxParClass_C|SetReplicatedAnimState _asbp_gotachar_max_par_class "NewEnumerator45")
  (Variables|Default|Setglobal%20Rider Rider)
  (Pawn|Possess (Pawn|GetController Rider) self)
  (Transformation|AttachComponentToComponent _asbp_gotachar_max_par_class (Variables|Character|GetMesh) "RidingSocket" "SnapToTarget" "SnapToTarget" "KeepWorld" true)
  (Collision|SetCollisionEnabled (Variables|/Script/Engine.Character|GetCapsuleComponent Rider) "NoCollision")
  (Collision|SetCollisionEnabled (Variables|/Script/Engine.Character|GetMesh Rider) "NoCollision"))

(event EventBeginPlay)

(event Collision|EventActorBeginOverlap
  (params (OtherActor :type Actor%20Object%20Reference))
  (|CallParentFunction OtherActor) ; This node is disabled and will not be called.\nDrag off pins to build functionality.
)

(event EventTick
  (params (DeltaSeconds :type Float%20%28single-precision%29))
  (|CallParentFunction DeltaSeconds) ; This node is disabled and will not be called.\nDrag off pins to build functionality.
)

(event EventServerUse
  (bind _global_rider (Variables|Default|Getglobal%20Rider))
  ;[0 1 0.003788] Server ride animal
  (bind _asbp_gotachar_max_par_class (Utilities|Casting|CastToBP_GOTACharMaxParClass _global_rider))
  (Transformation|DetachFromActor _global_rider "KeepWorld" "KeepWorld" "KeepWorld")
  (Pawn|Possess (Pawn|GetController) _global_rider)
  (Collision|SetCollisionEnabled (Variables|/Script/Engine.Character|GetCapsuleComponent _global_rider) "QueryAndPhysics")
  (Transformation|SetRelativeRotation (Variables|Character|GetMesh) "0,-90.000000, 0" false false)
  (Variables|/Game/GOTA2/Blueprints/Characters/BP_GOTACharMaxParClass.BP_GOTACharMaxParClass_C|SetReplicatedAnimState _asbp_gotachar_max_par_class "NewEnumerator0"))

(fn ConstructionScript)