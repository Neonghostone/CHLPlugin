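; BP_GOTAArmourHead is a head armour item that changes the head armour mesh on its owning character.
; Equip picks the female or default mesh by the owner's class, assigns it to RepnoSkeletalMeshHeadArmour, marks itself picked and registers in the inventory's HeadArmour slot.
; Unequip clears only the mesh variable, leaving the inventory slot untouched.
; A material handler ignores its input and applies the default mesh's first material to HeadProtection.
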(event Custom|HandleEquipSetMaterial_1
  (params (InterfaceMaterial :type Material%20Interface%20Object%20Reference))
  (bind _asbp_gotachar_max_par_class (Utilities|Casting|CastToBP_GOTACharMaxParClass (Components|GetOwner)))
  (Rendering|Material|SetMaterial (Variables|/Game/GOTA2/Blueprints/Characters/BP_GOTACharMaxParClass.BP_GOTACharMaxParClass_C|GetHeadProtection _asbp_gotachar_max_par_class) 0 (.materialinterface (Utilities|Array|Get(acopy) (Variables|/Script/Engine.SkeletalMesh|GetMaterials (Variables|Default|GetSkeleMeshToEquip))))))

(event EventBeginPlay
  (Utilities|FlowControl|Sequence
    (:then_0
      (|CallParentFunction))))

(event Collision|EventActorBeginOverlap
  (params (OtherActor :type Actor%20Object%20Reference))
  (|CallParentFunction OtherActor) ; This node is disabled and will not be called.\nDrag off pins to build functionality.
)

(event EventTick
  (params (DeltaSeconds :type Float%20%28single-precision%29))
  (|CallParentFunction DeltaSeconds) ; This node is disabled and will not be called.\nDrag off pins to build functionality.
)

(event EventEquip
  (bind _skelemeshtoequip (Variables|Default|GetSkeleMeshToEquip))
  (bind _skelemeshtoequipfemale (Variables|Default|GetSkeleMeshToEquipFemale))
  (bind _asbp_gotachar_max_par_class (Utilities|Casting|CastToBP_GOTACharMaxParClass (Components|GetOwner)))
  (Utilities|Casting|CastToBP_GOTAGirlMaxParClass _asbp_gotachar_max_par_class
    (:then
      (Utilities|IsValid _skelemeshtoequipfemale
        (:Is%20Valid
          (Variables|/Game/GOTA2/Blueprints/Characters/BP_GOTACharMaxParClass.BP_GOTACharMaxParClass_C|SetRepnoSkeletalMeshHeadArmour _asbp_gotachar_max_par_class _skelemeshtoequipfemale))
        (:Is%20Not%20Valid
          _)))
    (:CastFailed
      (Utilities|IsValid _skelemeshtoequip
        (:Is%20Valid
          (bind _output_get (Variables|/Game/GOTA2/Blueprints/Characters/BP_GOTACharMaxParClass.BP_GOTACharMaxParClass_C|SetRepnoSkeletalMeshHeadArmour _asbp_gotachar_max_par_class _skelemeshtoequip)))
        (:Is%20Not%20Valid
          _))))
  (Variables|Default|SetbPicked true)
  (Variables|/Game/GOTA2/Blueprints/InventoryAndItems/BP_GOTAInvMaxParClassInclBag.BP_GOTAInvMaxParClassInclBag_C|SetHeadArmour (Variables|/Game/GOTA2/Blueprints/Characters/BP_GOTACharMaxParClass.BP_GOTACharMaxParClass_C|GetInvReference _asbp_gotachar_max_par_class) self))

(event EventUnequip
  (bind _asbp_gotachar_max_par_class (Utilities|Casting|CastToBP_GOTACharMaxParClass (Components|GetOwner)))
  (Variables|/Game/GOTA2/Blueprints/Characters/BP_GOTACharMaxParClass.BP_GOTACharMaxParClass_C|SetRepnoSkeletalMeshHeadArmour _asbp_gotachar_max_par_class 0))

(fn ConstructionScript
  (|CallParentFunction))