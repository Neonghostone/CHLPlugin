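; BP_GOTASaveOptionsMaxPar is a save-game object that stores player options: item toggles, revive and gore settings, sound volumes, animation speed fix and language.
; SaveGameAndReturnResultOptions copies its parameters into variables and saves itself to the "options" slot, identically whether or not that slot exists.
; LoadAndReturnTheSlot instead loads or creates a BP_GOTASaveSystemGeneral from the "match" slot.
; StartSavingGame is empty and the debug prints are disconnected.
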(event Custom|StartSavingGame
  (params (NewBots :type Byte) (GameModeSaving :type Game%20Mode%20Object%20Reference)))

(fn LoadandReturntheSlot
  (params (slot :type String))
  ;[1 1 1] Description: Fill all the options and save em from here, Debug mode deactivated as we need Enum
  (bind _returnvalue (SaveGame|DoesSaveGameExist "match"))
  (if _returnvalue
    (bind _returnvalue_2 (SaveGame|LoadGamefromSlot "match"))
    (bind _asbp_gotasave_system_general (Utilities|Casting|CastToBP_GOTASaveSystemGeneral _returnvalue_2))
    (return _asbp_gotasave_system_general)
    (else
      ;[1 1 1] Unnecesary but you never know
      (bind _returnvalue_3 (SaveGame|CreateSaveGameObject "/Game/GOTA2/Blueprints/SaveSystem/BP_GOTASaveSystemGeneral.BP_GOTASaveSystemGeneral_C"))
      (bind _asbp_gotasave_system_general_2 (Utilities|Casting|CastToBP_GOTASaveSystemGeneral _returnvalue_3))
      (return _asbp_gotasave_system_general_2))))

(fn SaveGameandReturnResultOptions
  (params (gameinfo :type Game%20Mode%20Base%20Object%20Reference) (bpThrowable :type Boolean) (bpPickable :type Boolean) (bpBowable :type Boolean) (MasterSoundVolume :type Float%20%28single-precision%29) (MusicSoundVolume :type Float%20%28single-precision%29) (sfxSoundVolume :type Float%20%28single-precision%29) (bbReviveFalls :type Boolean) (AnimSpeedSavedForClient :type Float%20%28single-precision%29) (DefaultLanguage :type EN_Language%20Enum :default "NewEnumerator0") (bpGore :type Boolean))
  (bind _returnvalue (SaveGame|DoesSaveGameExist "options"))
  (if _returnvalue
    ;[1 1 1] All vars to be saved
    (Variables|Default|SetbAllPickable bpPickable)
    (Variables|Default|SetbAlllThrowable bpThrowable)
    (Variables|Default|SetbAllBowable bpBowable)
    (Variables|Default|SetbReviveFallsFloor bbReviveFalls)
    (Variables|Default|SetbGore bpGore)
    (Variables|Default|SetMasterSoundVolume MasterSoundVolume)
    (Variables|Default|SetMusicSoundVolume MusicSoundVolume)
    (Variables|Default|SetsfxSoundVolume sfxSoundVolume)
    (Variables|Default|SetGlobalMeshAnimSpeedFix AnimSpeedSavedForClient)
    (Variables|Default|SetLanguage DefaultLanguage)
    (bind _returnvalue_2 (SaveGame|SaveGametoSlot self "options"))
    (return _returnvalue_2)
    (else
      (Variables|Default|SetbAllPickable bpPickable)
      (Variables|Default|SetbAlllThrowable bpThrowable)
      (Variables|Default|SetbAllBowable bpBowable)
      (Variables|Default|SetbReviveFallsFloor bbReviveFalls)
      (Variables|Default|SetbGore bpGore)
      (Variables|Default|SetMasterSoundVolume MasterSoundVolume)
      (Variables|Default|SetMusicSoundVolume MusicSoundVolume)
      (Variables|Default|SetsfxSoundVolume sfxSoundVolume)
      (Variables|Default|SetGlobalMeshAnimSpeedFix AnimSpeedSavedForClient)
      (Variables|Default|SetLanguage DefaultLanguage)
      (bind _returnvalue_3 (SaveGame|SaveGametoSlot self "options"))
      (return _returnvalue_3))))