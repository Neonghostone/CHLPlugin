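; Base HUD for GOTA that creates the main HUD widget, shows left-side messages and drives a throw power bar.
; Primary and secondary weapon slots show icon and durability, tinted red to green, seeded from inventory on BeginPlay.
; BeginPlay also hides combat widgets under the menu game mode on authority and notifies the PlayerController's server.
; When flagged, DrawHUD caches throw origin and direction from a screen-center trace.
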(event Custom|HandleNewSecondaryWeapon
  (params (ItemMaxParentClass :type BP%20GOTA%20Item%20Max%20Par%20Class%20I%20Object%20Reference) (bewDura :type Integer))
  (bind _returnvalue (Math|Conversions|ToFloat(Integer) bewDura))
  (bind _mainhudmovie (Variables|Default|GetMainHUDMovie))
  (bind _leftsideitemslotnew (Variables|/Game/GOTA2/Blueprints/HUD/UW_MainHUD.UW_MainHUD_C|GetLeftSideItemSlotNew _mainhudmovie))
  ;[1 1 1] New functionality
  (Utilities|IsValid ItemMaxParentClass
    (:Is%20Valid
      (Utilities|IsValid _mainhudmovie
        (:Is%20Valid
          (bind _asw_item (Utilities|Casting|CastToW_Item (Class|PanelWidget|GetChildat (Variables|/Game/fantasy_gui_5/widgets/templates/item/W_Inventory_Item_Slot.W_Inventory_Item_Slot_C|GetContentBorder _leftsideitemslotnew))))
          (Class|Image|SetBrush (Variables|/Game/fantasy_gui_5/widgets/templates/item/W_Item.W_Item_C|Getitem_icon _asw_item) (Variables|/Game/GOTA2/Blueprints/InventoryAndItems/BP_GOTAItemMaxParClassI.BP_GOTAItemMaxParClassI_C|GetInvImage ItemMaxParentClass))
          (Rendering|Components|TextRender|SetText (Variables|/Game/fantasy_gui_5/widgets/templates/item/W_Item.W_Item_C|Getitem_quality _asw_item) (Utilities|Text|ToText(String) (Utilities|String|Append (Utilities|String|ToString(Integer) bewDura) "/" "99")))
          (CallFunction|SetColorOfLeftItemwithNewQuality _returnvalue)
          (Widget|SetVisibility _leftsideitemslotnew "Visible")
          (Appearance|SetColorandOpacity (Variables|/Game/fantasy_gui_5/widgets/templates/item/W_Item.W_Item_C|Getitem_quality _asw_item) (Utilities|Struct|MakeSlateColor (CallFunction|ReturnColorforDura _returnvalue) "UseColor_Specified") :!class /Script/UMG.TextBlock))))
    (:Is%20Not%20Valid
      (Utilities|IsValid _mainhudmovie
        (:Is%20Valid
          (Widget|SetVisibility _leftsideitemslotnew "Hidden"))))))

(event Custom|HandleNewPrimaryWeapon
  (params (ItemMaxParentClass :type BP%20GOTA%20Item%20Max%20Par%20Class%20I%20Object%20Reference) (NewDura :type Integer))
  (bind _mainhudmovie (Variables|Default|GetMainHUDMovie))
  (bind _rightsideitemslotnew (Variables|/Game/GOTA2/Blueprints/HUD/UW_MainHUD.UW_MainHUD_C|GetRightSideItemSlotNew _mainhudmovie))
  ;[1 1 1] New functionality
  (Utilities|IsValid ItemMaxParentClass
    (:Is%20Valid
      (Utilities|IsValid _mainhudmovie
        (:Is%20Valid
          (bind _asw_item (Utilities|Casting|CastToW_Item (Class|PanelWidget|GetChildat (Variables|/Game/fantasy_gui_5/widgets/templates/item/W_Inventory_Item_Slot.W_Inventory_Item_Slot_C|GetContentBorder _rightsideitemslotnew))))
          (Class|Image|SetBrush (Variables|/Game/fantasy_gui_5/widgets/templates/item/W_Item.W_Item_C|Getitem_icon _asw_item) (Variables|/Game/GOTA2/Blueprints/InventoryAndItems/BP_GOTAItemMaxParClassI.BP_GOTAItemMaxParClassI_C|GetInvImage ItemMaxParentClass))
          (Rendering|Components|TextRender|SetText (Variables|/Game/fantasy_gui_5/widgets/templates/item/W_Item.W_Item_C|Getitem_quality _asw_item) (Utilities|Text|ToText(String) (Utilities|String|Append (Utilities|String|ToString(Integer) NewDura) "/" "99")))
          (Widget|SetVisibility _rightsideitemslotnew "Visible")
          (Appearance|SetColorandOpacity (Variables|/Game/fantasy_gui_5/widgets/templates/item/W_Item.W_Item_C|Getitem_quality _asw_item) (Utilities|Struct|MakeSlateColor (CallFunction|ReturnColorforDura (Math|Conversions|ToFloat(Integer) NewDura)) "UseColor_Specified") :!class /Script/UMG.TextBlock))))
    (:Is%20Not%20Valid
      (Utilities|IsValid _mainhudmovie
        (:Is%20Valid
          (Widget|SetVisibility _rightsideitemslotnew "Hidden"))))))

(event Custom|HUDCreatedEventFromClient)

(event Custom|AddLeftSideMessageOnScreen
  (params (NewMessage :type String) (Duration :type Float%20%28single-precision%29) (ColorOfMessage :type Color%20Structure))
  (bind _mainhudmovie (Variables|Default|GetMainHUDMovie))
  ;[1 1 1] Duration still on the works
  (Utilities|IsValid _mainhudmovie
    (:Is%20Valid
      (bind _returnvalue (UserInterface|CreateWidget "/Game/GOTA2/Blueprints/HUD/UW_LeftScreenMessage.UW_LeftScreenMessage_C"))
      (Rendering|Components|TextRender|SetText (Variables|/Game/GOTA2/Blueprints/HUD/UW_LeftScreenMessage.UW_LeftScreenMessage_C|GetMessageText _returnvalue) (Utilities|Text|ToText(String) NewMessage))
      (Widget|Panel|AddChild (Variables|/Game/GOTA2/Blueprints/HUD/UW_MainHUD.UW_MainHUD_C|GetLOGLeftSideSL _mainhudmovie) _returnvalue)
      (Appearance|SetColorandOpacity (Variables|/Game/GOTA2/Blueprints/HUD/UW_LeftScreenMessage.UW_LeftScreenMessage_C|GetMessageText _returnvalue) (Utilities|Struct|MakeSlateColor (Math|Conversions|ToLinearColor(Color) ColorOfMessage)) :!class /Script/UMG.TextBlock))))

(event Custom|StartProgressingBasr
  (params (rate :type Float%20%28single-precision%29))
  (bind _returnvalue (Utilities|Time|SetTimerbyEvent (delegate Custom|ProgressTheBar) rate true))
  (Variables|Default|SetProgressBarLerping _returnvalue))

(event Custom|ProgressTheBar
  (bind _mainhudmovie (Variables|Default|GetMainHUDMovie))
  (bind _throwpower (Variables|/Game/GOTA2/Blueprints/HUD/UW_MainHUD.UW_MainHUD_C|GetThrowPower _mainhudmovie))
  (Progress|SetPercent _throwpower (+ (Variables|/Script/UMG.ProgressBar|GetPercent _throwpower) 0.1)))

(event Custom|SetColorOfLeftItemWithNewQuality
  (params (NewDura :type Float%20%28single-precision%29))
  ;[1 1 1] WIP depra
)

(event Custom|SetColorOfRightItemWithNewQuality
  (params (NewDura :type Float%20%28single-precision%29))
  ;[1 1 1] WIP depra
)

(event Custom|ReturnColorForItemQuality
  (params (NewDura :type Float%20%28single-precision%29))
  ;[1 1 1] WIP depra
)

(event Custom|OnHudMovieCreated
  ;[0 0 1] To have exact timing when things are created
  (bind _asbp_gotapcmax_par_class (Utilities|Casting|CastToBP_GOTAPCMaxParClass (Game|Player|GetOwningPlayerController)))
  (Default|ServeronHUDMovieCreatedfromClient _asbp_gotapcmax_par_class)
  (Development|PrintString "FROM GOTA HUD movie tier2 EVent dispatcher shall work" true true "(R=1.000000,G=0.940055,B=0.000000,A=1.000000)")
  (bind _asbp_gotachar_max_par_class (Utilities|Casting|CastToBP_GOTACharMaxParClass (Pawn|GetControlledPawn (Variables|Default|GetPlayerOwner))))
  ;[1 1 1] Wait for the hud to exist and pc on hud created
  (Utilities|IsValid (Variables|/Game/GOTA2/Blueprints/InventoryAndItems/BP_GOTAInvMaxParClassInclBag.BP_GOTAInvMaxParClassInclBag_C|GetPrimaryItem (Variables|/Game/GOTA2/Blueprints/Characters/BP_GOTACharMaxParClass.BP_GOTACharMaxParClass_C|GetInvReference _asbp_gotachar_max_par_class))
    (:Is%20Not%20Valid
      (Default|UpdateSpecialAttacksLowerLeft (Variables|Default|GetMainHUDMovie) (Variables|/Game/GOTA2/Blueprints/Characters/BP_GOTACharMaxParClass.BP_GOTACharMaxParClass_C|GetMeleeSpecialAttacks _asbp_gotachar_max_par_class)))))

(event Custom|AddWIPMessageHUD
  ;[1 0.8122 0] For not repeating the same nodes over and over
  (bind _asbp_gotapcmax_par_class (Utilities|Casting|CastToBP_GOTAPCMaxParClass (Game|Player|GetOwningPlayerController)))
  (Default|ClientAddMessage _asbp_gotapcmax_par_class "Difficulty on campaign not implemented yet! WIP" 2.0 (Math|Color|MakeColor 0 255 255 255)))

(event EventBeginPlay
  (Utilities|FlowControl|Sequence
    (:then_0
      (bind _returnvalue (UserInterface|CreateWidget "/Game/GOTA2/Blueprints/HUD/UW_MainHUD.UW_MainHUD_C" (Variables|Default|GetPlayerOwner)))
      (Variables|Default|SetMainHUDMovie _returnvalue)
      (UserInterface|Viewport|AddtoViewport _returnvalue 0)
      (bind _asbp_gotachar_max_par_class (Utilities|Casting|CastToBP_GOTACharMaxParClass (Class|HUD|GetOwningPawn)))
      (Utilities|IsValid (Variables|/Game/GOTA2/Blueprints/Characters/BP_GOTACharMaxParClass.BP_GOTACharMaxParClass_C|GetInvReference _asbp_gotachar_max_par_class)
        (:Is%20Valid
          (Utilities|IsValid (Variables|/Game/GOTA2/Blueprints/InventoryAndItems/BP_GOTAInvMaxParClassInclBag.BP_GOTAInvMaxParClassInclBag_C|GetPrimaryItem (Variables|/Game/GOTA2/Blueprints/Characters/BP_GOTACharMaxParClass.BP_GOTACharMaxParClass_C|GetInvReference _asbp_gotachar_max_par_class))
            (:Is%20Valid
              (CallFunction|HandleNewPrimaryWeapon (Variables|/Game/GOTA2/Blueprints/InventoryAndItems/BP_GOTAInvMaxParClassInclBag.BP_GOTAInvMaxParClassInclBag_C|GetPrimaryItem (Variables|/Game/GOTA2/Blueprints/Characters/BP_GOTACharMaxParClass.BP_GOTACharMaxParClass_C|GetInvReference _asbp_gotachar_max_par_class)) (Variables|/Game/GOTA2/Blueprints/InventoryAndItems/BP_GOTAItemMaxParClassI.BP_GOTAItemMaxParClassI_C|GetDurability (Variables|/Game/GOTA2/Blueprints/InventoryAndItems/BP_GOTAInvMaxParClassInclBag.BP_GOTAInvMaxParClassInclBag_C|GetPrimaryItem (Variables|/Game/GOTA2/Blueprints/Characters/BP_GOTACharMaxParClass.BP_GOTACharMaxParClass_C|GetInvReference _asbp_gotachar_max_par_class))))
              (Utilities|IsValid (Variables|/Game/GOTA2/Blueprints/InventoryAndItems/BP_GOTAInvMaxParClassInclBag.BP_GOTAInvMaxParClassInclBag_C|GetSecondaryItem (Variables|/Game/GOTA2/Blueprints/Characters/BP_GOTACharMaxParClass.BP_GOTACharMaxParClass_C|GetInvReference _asbp_gotachar_max_par_class))
                (:Is%20Valid
                  (CallFunction|HandleNewSecondaryWeapon (Variables|/Game/GOTA2/Blueprints/InventoryAndItems/BP_GOTAInvMaxParClassInclBag.BP_GOTAInvMaxParClassInclBag_C|GetSecondaryItem (Variables|/Game/GOTA2/Blueprints/Characters/BP_GOTACharMaxParClass.BP_GOTACharMaxParClass_C|GetInvReference _asbp_gotachar_max_par_class)) (Variables|/Game/GOTA2/Blueprints/InventoryAndItems/BP_GOTAItemMaxParClassI.BP_GOTAItemMaxParClassI_C|GetDurability (Variables|/Game/GOTA2/Blueprints/InventoryAndItems/BP_GOTAInvMaxParClassInclBag.BP_GOTAInvMaxParClassInclBag_C|GetSecondaryItem (Variables|/Game/GOTA2/Blueprints/Characters/BP_GOTACharMaxParClass.BP_GOTACharMaxParClass_C|GetInvReference _asbp_gotachar_max_par_class)))))))))))
    (:then_1
      (Networking|SwitchHasAuthority
        (:Authority
          (Utilities|Casting|CastToBP_GOTAGameInfoMenu (Game|GetGameMode))
          (Widget|SetVisibility (Variables|/Game/GOTA2/Blueprints/HUD/UW_MainHUD.UW_MainHUD_C|GetCrosshair (Variables|Default|GetMainHUDMovie)) "Hidden")
          (Widget|SetVisibility (Variables|/Game/GOTA2/Blueprints/HUD/UW_MainHUD.UW_MainHUD_C|GetLOGLeftSideSL (Variables|Default|GetMainHUDMovie)) "HitTestInvisible"))))
    (:then_2
      ;[0.005664 1 0] start cards game if necessary
      (bind _asbp_gotapcmax_par_class (Utilities|Casting|CastToBP_GOTAPCMaxParClass (Variables|Default|GetPlayerOwner)))
      (Default|ServerAsktheServerforOperationonBeginPlay _asbp_gotapcmax_par_class))))

(event Collision|EventActorBeginOverlap
  (params (OtherActor :type Actor%20Object%20Reference)))

(event EventTick
  (params (DeltaSeconds :type Float%20%28single-precision%29)))

(event EventDrawHUD
  (params (SizeX :type Integer) (SizeY :type Integer))
  (bind (_worldpos _direction) (CallFunction|GetScreenCenterLoctoThrow))
  (if (Variables|Default|GetbShouldUpdatePosAndDir)
    (Variables|Default|SetWorldPosConstant _worldpos)
    (Variables|Default|SetDirectionConstant _direction)))

(fn ConstructionScript)

(fn GetScreenCenterLoctoThrow
  (bind _returnvalue (Viewport|GetViewportSize))
  (bind _playerowner (Variables|Default|GetPlayerOwner))
  (bind _returnvalue_2 (/ (.y _returnvalue) 2.0))
  (bind _returnvalue_3 (/ (.x _returnvalue) 2.0))
  (bind _returnvalue_4 (Pawn|GetControlledPawn _playerowner))
  (bind (_worldposition _worlddirection) (Class|HUD|Deproject _returnvalue_3 _returnvalue_2))
  (bind _returnvalue_5 (Transformation|GetActorLocation _returnvalue_4))
  (Utilities|IsValid _returnvalue_4
    (:Is%20Valid
      (bind _outhit (Collision|LineTraceForObjects _worldposition (+ _returnvalue_5 (* _worlddirection 1e+04)) (Utilities|Array|MakeArray "ObjectTypeQuery3" "ObjectTypeQuery1") false (Utilities|Array|MakeArray _returnvalue_4) "None"))
      (Utilities|IsValid (.HitActor (Collision|BreakHitResult _outhit))
        (:Is%20Valid
          (return _worldposition (Math|Rotator|GetRotationXVector (Math|Conversions|RotationFromXVector (- (.Location (Collision|BreakHitResult _outhit)) _returnvalue_5)))))
        (:Is%20Not%20Valid
          (return _worldposition _worlddirection))))))

(fn ReturnQualityforItem
  (params (ItemToCheck :type BP%20GOTA%20Item%20Max%20Par%20Class%20I%20Object%20Reference))
  (bind _durability (Variables|/Game/GOTA2/Blueprints/InventoryAndItems/BP_GOTAItemMaxParClassI.BP_GOTAItemMaxParClassI_C|GetDurability ItemToCheck))
  ;[1 1 1] There are easier/better ways
  (if (> _durability 50)
    (return (Math|Conversions|ToColor(LinearColor) (Math|Color|MakeColor 0.0 255.0 0.0 255.0)))
    (elif (> _durability 30)
      (return (Math|Conversions|ToColor(LinearColor) (Math|Color|MakeColor 255.0 255.0 0.0 255.0)))
      (else
        (return (Math|Conversions|ToColor(LinearColor) (Math|Color|MakeColor 255.0 0.0 0.0 255.0)))))))

(fn ReturnColorforDura
  (params (Dura :type Float%20%28single-precision%29))
  (bind _returnvalue (/ Dura 1e+02))
  (bind _returnvalue_2 (Math|Float|MakeLiteralFloat 1.0))
  (bind _returnvalue_3 (/ Dura 1e+02))
  (bind _returnvalue_4 (- _returnvalue_2 _returnvalue))
  (bind _returnvalue_5 (Math|Color|MakeColor _returnvalue_4 _returnvalue_3 0.0))
  (bind (_r _g _b _a) (Math|Color|BreakColor _returnvalue_5))
  (return (Utilities|Struct|MakeLinearColor _r _g _b _a)))