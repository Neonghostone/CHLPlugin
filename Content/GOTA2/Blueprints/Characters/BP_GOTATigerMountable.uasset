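; Player-controllable tiger character with melee attacks, dodging and a special attack; despite the name, it overrides riding with an empty event.
; Left-click hold time selects a small attack or leaping big attack, while clicking mid-air triggers a jump attack.
; ReplicatedAnimState gates actions and drives Tick's procedural root motion and authority-only paw and head socket traces.
; Trace hits damage character meshes, or stun the tiger with sparks when blocked by weapons or shields.
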(event Custom|ServerPrepareAttackForTiger
  (Variables|Default|SetReplicatedAnimState "NewEnumerator39")
  (Components|Movement|StopMovementImmediately (Variables|Character|GetCharacterMovement)))

(event Custom|ServerUnleashBigAttackForTiger
  (bind _charactermovement (Variables|Character|GetCharacterMovement))
  (bind _outactors (Actor|GetAllActorsOfClass "/Game/GOTA2/Blueprints/Controllers/BP_GOTAPCMaxParClass.BP_GOTAPCMaxParClass_C"))
  (Default|ClientMulticastPlaySound _outactors (Transformation|GetActorLocation) (Variables|Default|GetTigerJumpAttackSoundBoth))
  (Variables|Default|SetReplicatedAnimState "NewEnumerator40")
  (Variables|/Script/Engine.CharacterMovementComponent|SetMaxWalkSpeed _charactermovement 1.5e+03)
  (Variables|/Script/Engine.CharacterMovementComponent|SetMaxAcceleration _charactermovement 5.12e+03)
  (Utilities|FlowControl|Delay 1.0)
  (CallFunction|BigResetVariablesAfterforAttack))

(event Custom|StartUnpressLeftTiger
  (switch Utilities|FlowControl|Switch|SwitchonEN_PawnState (Variables|Default|GetPawnState)
    (:NewEnumerator0
      (switch Utilities|FlowControl|Switch|SwitchonEN_AnimState (Variables|Default|GetReplicatedAnimState)
        (:NewEnumerator39
          (if (Variables|Default|GetbAttackPreparedMoreThanTime)
            (CallFunction|ServerTriggerNowforClienttheTigerAttack)
            (else
              (CallFunction|ServerUnleashSmallTigerAtttack))))))))

(event Custom|TraceAllBodyPartsTiger
  ;[0.9932 1 0] Desc: Neongho: Add shield and parry detection and cooldown when an shield or parry is hit
  (bind _traceresults (CallFunction|COREBodyCollisionTraceStartEndPoint (Transformation|GetSocketLocation (Variables|Character|GetMesh) "FrontPawRSocketStart") (Transformation|GetSocketLocation (Variables|Character|GetMesh) "FrontPawRSocketEnd")))
  (for _array_element _traceresults
    (CallFunction|ProcessTigerHIts _array_element))
  (bind _traceresults_2 (CallFunction|COREBodyCollisionTraceStartEndPoint (Transformation|GetSocketLocation (Variables|Character|GetMesh) "FrontPawLSocketStart") (Transformation|GetSocketLocation (Variables|Character|GetMesh) "FrontPawLSocketEnd")))
  (for _array_element_2 _traceresults_2
    (CallFunction|ProcessTigerHIts _array_element_2))
  ;;[1 1 1] Trace head
  (bind _traceresults_3 (CallFunction|COREBodyCollisionTraceStartEndPoint (Transformation|GetSocketLocation (Variables|Character|GetMesh) "FaceSocketHeadStart") (Transformation|GetSocketLocation (Variables|Character|GetMesh) "FaceSocketHeadEnd")))
  (for _array_element_3 _traceresults_3
    (CallFunction|ProcessTigerHIts _array_element_3)))

(event Custom|TraceBodyPart
  (params (Socket1 :type String) (Socket2 :type String))
  ;[0.9434 1 0] Trace body part
  (bind _traceresults (CallFunction|COREBodyCollisionTraceStartEndPoint (Transformation|GetSocketLocation (Variables|Character|GetMesh) "FrontPawRSocketStart") (Transformation|GetSocketLocation (Variables|Character|GetMesh) "FrontPawRSocketEnd")))
  (for _array_element _traceresults
    (Class|IGOTATraceInterface|ActorTakeDamage(Message) (.HitActor (Collision|BreakHitResult _array_element)) 1 (.Location (Collision|BreakHitResult _array_element)) (.Normal (Collision|BreakHitResult _array_element)) "" "NewEnumerator7" true 25.0 false 0.0 0.0 _array_element self "0, 0, 0" "NewEnumerator0")))

(event Custom|ProcessTigerHIts
  (params (InputHitResult :type Hit%20Result%20Structure))
  (bind (_bblockinghit _binitialoverlap _time _distance _location _impactpoint _normal _impactnormal _physmat _hitactor _hitcomponent) (Collision|BreakHitResult InputHitResult))
  ;[0.08021 0.01886 0.01455] HitResult
  ;;[1 1 1] Local var
  (Variables|Default|SetbAlreadyBlocked false)
  (Utilities|FlowControl|Sequence
    (:then_0
      (bind _asbp_gotachar_max_par_class (Utilities|Casting|CastToBP_GOTACharMaxParClass _hitactor))
      (bind _asskeletal_mesh_component (Utilities|Casting|CastToSkeletalMeshComponent _hitcomponent))
      (if (and (or (== _asskeletal_mesh_component (Variables|/Game/GOTA2/Blueprints/Characters/BP_GOTACharMaxParClass.BP_GOTACharMaxParClass_C|GetLeftArmWeapon _asbp_gotachar_max_par_class)) (== _asskeletal_mesh_component (Variables|/Game/GOTA2/Blueprints/Characters/BP_GOTACharMaxParClass.BP_GOTACharMaxParClass_C|GetRightArmWeapon _asbp_gotachar_max_par_class))) (Math|Boolean|ORBoolean (Utilities|Enum|Equal(Enum) (Variables|/Game/GOTA2/Blueprints/Characters/BP_GOTACharMaxParClass.BP_GOTACharMaxParClass_C|GetReplicatedAnimState _asbp_gotachar_max_par_class) "NewEnumerator4") (Utilities|Enum|Equal(Enum) (Variables|/Game/GOTA2/Blueprints/Characters/BP_GOTACharMaxParClass.BP_GOTACharMaxParClass_C|GetReplicatedAnimState _asbp_gotachar_max_par_class) "NewEnumerator2") (Utilities|Enum|Equal(Enum) (Variables|/Game/GOTA2/Blueprints/Characters/BP_GOTACharMaxParClass.BP_GOTACharMaxParClass_C|GetReplicatedAnimState _asbp_gotachar_max_par_class) "NewEnumerator3") (Utilities|Enum|Equal(Enum) (Variables|/Game/GOTA2/Blueprints/Characters/BP_GOTACharMaxParClass.BP_GOTACharMaxParClass_C|GetReplicatedAnimState _asbp_gotachar_max_par_class) "NewEnumerator1")))
        (CallFunction|StoptheAttack InputHitResult)
        (Variables|Default|SetbAlreadyBlocked true)))
    (:then_1
      (if (not (Variables|Default|GetbAlreadyBlocked))
        (bind _asbp_gotachar_max_par_class_2 (Utilities|Casting|CastToBP_GOTACharMaxParClass _hitactor))
        (bind _asskeletal_mesh_component_2 (Utilities|Casting|CastToSkeletalMeshComponent _hitcomponent))
        (if (== _asskeletal_mesh_component_2 (Variables|/Script/Engine.Character|GetMesh _asbp_gotachar_max_par_class_2))
          (Default|ActorTakeDamage _asbp_gotachar_max_par_class_2 2 _impactpoint _normal "" "NewEnumerator7" true 25.0 false 0.0 0.0 InputHitResult self "0, 0, 0" "NewEnumerator0"))))))

(event Custom|StopTheAttack
  (params (HitInfo :type Hit%20Result%20Structure))
  (bind (_bblockinghit _binitialoverlap _time _distance _location _impactpoint _normal) (Collision|BreakHitResult HitInfo))
  ;[0.07604 0.07604 0.07604] Prevents From tracing when the tiger is blocked
  (Variables|Default|SetReplicatedAnimState "NewEnumerator0")
  (CallFunction|ServerGetStunned (Math|Random|RandomFloatinRange 1.0 2.0))
  (CallFunction|ForAllPcsSpawnSparks "/Game/GOTA2/Particles/PSN_SparksParry.PSN_SparksParry" _location (Math|Conversions|RotationFromXVector _normal) "1.000000,1.000000,1.000000" "/Game/GOTA2/Particles/FX_Sparks.FX_Sparks")
  (bind _outactors (Actor|GetAllActorsOfClass "/Game/GOTA2/Blueprints/Controllers/BP_GOTAPCMaxParClass.BP_GOTAPCMaxParClass_C"))
  (Default|ServerPlaySound _outactors _location "/Game/GOTA2/Audio/CU_HitRectionArmorHeavyHit.CU_HitRectionArmorHeavyHit"))

(event Custom|StartDodging
  (bind _charactermovement (Variables|Character|GetCharacterMovement))
  ;[0 1 0.204] Dodge and stuff
  (switch Utilities|FlowControl|Switch|SwitchonEN_PawnState (Variables|Default|GetPawnState)
    (:NewEnumerator0
      (switch Utilities|FlowControl|Switch|SwitchonEN_AnimState (Variables|Default|GetReplicatedAnimState)
        (:NewEnumerator0
          (if (not (and (== (Variables|Default|GetDodgeDirX) 0.0) (== (Variables|Default|GetDodgeDirY) 0.0)))
            (Variables|/Script/Engine.CharacterMovementComponent|SetMaxWalkSpeed _charactermovement 1e+03)
            (Variables|/Script/Engine.CharacterMovementComponent|SetMaxAcceleration _charactermovement 4096.0)
            (Variables|Default|SetReplicatedAnimState "NewEnumerator9")
            (CallFunction|ServerAdaptDodgeSpeed)
            (Variables|Default|SetbDodging true)
            (Utilities|FlowControl|Delay 0.75)
            (CallFunction|StopDodgingNow)
            (CallFunction|ServerStopDodging)
            (Variables|Default|SetbDodging false)))))))

(event Custom|BigResetVariablesAfterForAttack
  (Utilities|FlowControl|Sequence
    (:then_0
      (Variables|/Script/Engine.CharacterMovementComponent|SetMaxWalkSpeed (Variables|Character|GetCharacterMovement) 2.5e+02)
      (Character|StopJumping)
      (Variables|/Script/Engine.CharacterMovementComponent|SetMaxAcceleration (Variables|Character|GetCharacterMovement) 1024.0)
      (Variables|Default|SetReplicatedAnimState "NewEnumerator0"))))

(event Custom|StopDodgingNow
  (bind _charactermovement (Variables|Character|GetCharacterMovement))
  ;[0 1 0.204] Dodge and stuff
  (Variables|/Script/Engine.CharacterMovementComponent|SetMaxWalkSpeed _charactermovement 3.5e+02)
  (Variables|/Script/Engine.CharacterMovementComponent|SetMaxAcceleration _charactermovement 1024.0))

(event Custom|ServerStopDodging
  ;[0 1 0.204] Dodge and stuff
  (CallFunction|StopDodgingNow)
  (Variables|Default|SetReplicatedAnimState "NewEnumerator0"))

(event Custom|ServerAdaptDodgeSpeed
  (bind _charactermovement (Variables|Character|GetCharacterMovement))
  ;[0 1 0.204] Dodge and stuff
  (Variables|/Script/Engine.CharacterMovementComponent|SetMaxWalkSpeed _charactermovement 1e+03)
  (Variables|/Script/Engine.CharacterMovementComponent|SetMaxAcceleration _charactermovement 4096.0)
  (Variables|Default|SetReplicatedAnimState "NewEnumerator9"))

(event Custom|ClientTriggerNowTheJumpAttack
  (bind _charactermovement (Variables|Character|GetCharacterMovement))
  (switch Utilities|FlowControl|Switch|SwitchonEN_AnimState (Variables|Default|GetReplicatedAnimState)
    (:NewEnumerator39
      (Utilities|FlowControl|Sequence
        (:then_0
          (Variables|Default|SetShouldkeepAttackingForward true)
          (Utilities|FlowControl|Delay 0.75)
          (Variables|Default|SetShouldkeepAttackingForward false))
        (:then_1
          (CallFunction|ServerUnleashBigAttackforTiger)
          (Variables|Default|SetReplicatedAnimState "NewEnumerator40")
          (CallFunction|ServerStartFire)
          (Variables|/Script/Engine.CharacterMovementComponent|SetMaxWalkSpeed _charactermovement 1.5e+03)
          (Variables|/Script/Engine.CharacterMovementComponent|SetMaxAcceleration _charactermovement 5.12e+03)
          (Utilities|FlowControl|Delay 0.25)
          (Character|Jump))))))

(event Custom|ServerTriggerNowForClientTheTigerAttack
  (bind _charactermovement (Variables|Character|GetCharacterMovement))
  (Variables|/Script/Engine.CharacterMovementComponent|SetMaxWalkSpeed _charactermovement 7.5e+02)
  (Variables|/Script/Engine.CharacterMovementComponent|SetMaxAcceleration _charactermovement 5.12e+04)
  (CallFunction|ClientTriggerNowtheJumpAttack)
  (Variables|Default|SetReplicatedAnimState "NewEnumerator40")
  (Utilities|FlowControl|Delay 2.0))

(event Custom|ServerUnleashSmallTigerAtttack
  (bind _outactors (Actor|GetAllActorsOfClass "/Game/GOTA2/Blueprints/Controllers/BP_GOTAPCMaxParClass.BP_GOTAPCMaxParClass_C"))
  (Default|ClientMulticastPlaySound _outactors (Transformation|GetActorLocation) (Variables|Default|GetTigerSmallAttackSound))
  (Variables|Default|SetReplicatedAnimState "NewEnumerator41")
  (Utilities|FlowControl|Delay 1.0)
  (CallFunction|ResetVariablesforSmallAttack))

(event Custom|StartPressLeftAttackTiger
  (switch Utilities|FlowControl|Switch|SwitchonEN_PawnState (Variables|Default|GetPawnState)
    (:NewEnumerator0
      (switch Utilities|FlowControl|Switch|SwitchonEN_AnimState (Variables|Default|GetReplicatedAnimState)
        (:NewEnumerator0
          (if (AI|Components|NavMovement|IsFalling (Variables|Character|GetCharacterMovement))
            (CallFunction|ServerDotheJumpAttack)
            (else
              (Variables|Default|SetbAttackPreparedMoreThanTime false)
              (Variables|Default|SetReplicatedAnimState "NewEnumerator39")
              (CallFunction|ServerPrepareAttackforTiger)
              (Utilities|FlowControl|Delay (Variables|Default|GetMinTimeForBigAttack))
              (Variables|Default|SetbAttackPreparedMoreThanTime true))))))))

(event Custom|ResetVariablesForSmallAttack
  (Variables|Default|SetReplicatedAnimState "NewEnumerator0"))

(event Custom|ServerDoTheJumpAttack
  (bind _outactors (Actor|GetAllActorsOfClass "/Game/GOTA2/Blueprints/Controllers/BP_GOTAPCMaxParClass.BP_GOTAPCMaxParClass_C"))
  (Default|ClientMulticastPlaySound _outactors (Transformation|GetActorLocation) (Variables|Default|GetTigerJumpAttackSoundBoth))
  (Variables|Default|SetReplicatedAnimState "NewEnumerator42")
  (Utilities|FlowControl|Delay (Variables|Default|GetAttackDuration))
  (Variables|Default|SetReplicatedAnimState "NewEnumerator0"))

(event EventBeginPlay
  (|CallParentFunction) ; This node is disabled and will not be called.\nDrag off pins to build functionality.
)

(event Collision|EventActorBeginOverlap
  (params (OtherActor :type Actor%20Object%20Reference))
  (|CallParentFunction OtherActor) ; This node is disabled and will not be called.\nDrag off pins to build functionality.
)

(event EventTick
  (params (DeltaSeconds :type Float%20%28single-precision%29))
  (bind _returnvalue (Pawn|GetController))
  ;[0 0.6954 1] Tick
  (Utilities|FlowControl|Sequence
    (:then_0
      (Utilities|IsValid _returnvalue
        (:Is%20Valid
          (if (Networking|IsServer)
            (Networking|SwitchHasAuthority
              (:Authority
                (switch Utilities|FlowControl|Switch|SwitchonEN_AnimState (Variables|Default|GetReplicatedAnimState) :!label _label
                  (:NewEnumerator9
                    (if (Variables|Default|GetbDodging) :!label _label_2
                      (CallFunction|ProceduralRootMotionDodgetoASide)))
                  (:NewEnumerator25
                    (goto _label_2))
                  (:NewEnumerator40
                    (if (Variables|Default|GetShouldkeepAttackingForward)
                      (CallFunction|ProceduralRootMotionforAttack)))
                  (:NewEnumerator43
                    (CallFunction|ProceduralRootMotionSpecialAttack)))))
            (elif (Pawn|IsLocalPlayerController _returnvalue)
              (Networking|SwitchHasAuthority
                (:Remote
                  (goto _label))))))))
    (:then_1
      (Networking|SwitchHasAuthority
        (:Authority
          (switch Utilities|FlowControl|Switch|SwitchonEN_AnimState (Variables|Default|GetReplicatedAnimState)
            (:NewEnumerator40
              _)
            (:NewEnumerator41
              _)
            (:NewEnumerator42
              _)
            (:NewEnumerator43
              _))
          (CallFunction|TraceAllBodyPartsTiger))))
    (:then_2
      (|CallParentFunction DeltaSeconds))))

(event EventServerStartFire
  (params (FireModeNum :type Byte :default 0))
  ;[1 1 1] Not used so much as the necessary input from the client for optimiziation
  (switch int (Math|Conversions|ToInteger(Byte) FireModeNum)))

(event EventServerStopFire
  (params (FireModeNum :type Byte :default 0))
  ;[1 1 1] Not used so much as the necessary input from the client for optimiziation
)

(event EventGetRiden
  (params (Rider :type Character%20Object%20Reference))
  ;[0.009375 0 0] Override and stop mounting tigers
)

(event Input|ActionEvents|InputActionLeftMouseClick
  (params (Key :type Key%20Structure :default "None"))
  (:Pressed
    (CallFunction|StartPressLeftAttackTiger))
  (:Released
    (CallFunction|StartUnpressLeftTiger)))

(event Input|ActionEvents|InputActionSpecialAttack
  (params (Key :type Key%20Structure :default "None"))
  ;[1 1 1] Special attacks for tgier
  (:Pressed
    (bind _asbp_gotapcmax_par_class (Utilities|Casting|CastToBP_GOTAPCMaxParClass (Game|GetPlayerController 0)))
    (switch Utilities|FlowControl|Switch|SwitchonEN_AnimState (Variables|Default|GetReplicatedAnimState)
      (:NewEnumerator0
        (switch Utilities|FlowControl|Switch|SwitchonEN_PawnState (Variables|Default|GetPawnState)
          (:NewEnumerator0
            (if (Utilities|Enum|Equal(Enum) (Variables|Default|GetReplicatedAnimState) "NewEnumerator0")
              (CallFunction|ServerPerformSpecialAttack)))))
      (:NewEnumerator4
        (switch Utilities|FlowControl|Switch|SwitchonEN_PawnState (Variables|Default|GetPawnState)
          (:NewEnumerator0
            _)
          (:NewEnumerator7
            _))
        (CallFunction|ServerChangeShieldWheelVariable (+ (Variables|Default|GetShieldWheel) 25))))))

(event Input|ActionEvents|InputActionDodgeSecondaryWithB
  (params (Key :type Key%20Structure :default "None"))
  ;[0 1 0.204] Dodge and stuff
  (:Pressed
    (CallFunction|StartDodging)))

(event Input|ActionEvents|InputActionDodge
  (params (Key :type Key%20Structure :default "None"))
  ;[0 1 0.204] Dodge and stuff
  (:Pressed
    (CallFunction|StartDodging)))

(event Input|AxisEvents|InputAxisMoveRight
  (params (AxisValue :type Float%20%28single-precision%29))
  ;[1 0.1124 0] Forward backwards and left right input
  (if (not (== AxisValue 0.0))
    (Variables|Default|SetDodgeDirY (* AxisValue 1e+02))
    (else
      (Variables|Default|SetDodgeDirY 0.0))))

(event Input|AxisEvents|InputAxisMoveForward
  (params (AxisValue :type Float%20%28single-precision%29))
  ;[1 0.1124 0] Forward backwards and left right input
  (switch Utilities|FlowControl|Switch|SwitchonEN_AnimState (Variables|Default|GetReplicatedAnimState)
    (:NewEnumerator0
      (Pawn|Input|AddMovementInput (Math|Vector|GetForwardVector (Transformation|GetActorRotation)) AxisValue false)
      (if (not (== AxisValue 0.0))
        (Variables|Default|SetDodgeDirX (* AxisValue 1e+02))
        (else
          (Variables|Default|SetDodgeDirX 0.0))))))

(fn ConstructionScript
  (|CallParentFunction))