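; Arena spawner actor that places gladiators and tigers at random points inside its Box at a fixed height, with random yaw, and returns them.
; The random function picks one of four basic types, unless the game mode forces one, with hard-coded weapons.
; The custom function spawns the requested class with a random per-class loadout and team, passing difficulty through unused.
; Its copied game-mode override result goes unused.
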(event EventBeginPlay)

(event Collision|EventActorBeginOverlap
  (params (OtherActor :type Actor%20Object%20Reference)))

(event EventTick
  (params (DeltaSeconds :type Float%20%28single-precision%29)))

(fn ConstructionScript)

(fn SpawnGladiatorandRandomReturnIt
  (bind _returnvalue (Math|Random|RandomFloatinRange -1.8e+02 1.8e+02))
  (bind _self self)
  (bind _box (Variables|Default|GetBox))
  (bind _returnvalue_2 (Transformation|GetActorLocation _self))
  (bind _returnvalue_3 (Math|Rotator|MakeRotator 0.0 0.0 _returnvalue))
  (bind _returnvalue_4 (Components|Box|GetScaledBoxExtent _box))
  (bind _returnvalue_5 (Math|Random|RandomPointinBoundingBox _returnvalue_2 _returnvalue_4))
  (bind (_x _y) (Math|Vector|BreakVector _returnvalue_5))
  (bind _returnvalue_6 (Math|Vector|MakeVector _x _y 3e+02))
  (bind _returnvalue_7 (Math|Transform|MakeTransform _returnvalue_6 _returnvalue_3))
  (bind _asbp_gotaarena_game_info (Utilities|Casting|CastToBP_GOTAArenaGameInfo (Game|GetGameMode))
    (:then
      (if (Variables|/Game/GOTA2/Blueprints/GameInfos/BP_GOTAArenaGameInfo.BP_GOTAArenaGameInfo_C|GetbOverrideSpawnModeAllSameType _asbp_gotaarena_game_info)
        (LocalVariables|SetRandomGladiator (Variables|/Game/GOTA2/Blueprints/GameInfos/BP_GOTAArenaGameInfo.BP_GOTAArenaGameInfo_C|GetOverrideSameTypeType _asbp_gotaarena_game_info))
        (else
          (LocalVariables|SetRandomGladiator (Utilities|Enum|ByteToEnumEN_GladiatorType (Math|Conversions|ToByte(Integer) (Math|Random|RandomInteger 4))) :!label _label))))
    (:CastFailed
      (goto _label)))
  (switch Utilities|FlowControl|Switch|SwitchonEN_GladiatorType (LocalVariables|GetRandomGladiator)
    (:NewEnumerator0
      (bind _returnvalue_8 (Game|SpawnActorfromClass "/Game/GOTA2/Blueprints/Characters/BP_GOTANumeriusOriginaInUsel.BP_GOTANumeriusOriginaInUsel_C" _returnvalue_7 "AdjustIfPossibleButAlwaysSpawn" 0 100 100 (Utilities|Array|MakeArray "/Game/GOTA2/Blueprints/InventoryAndItems/BP_GOTAGladius_A.BP_GOTAGladius_A_C" (select (Math|Random|RandomBool) "/Game/GOTA2/Blueprints/InventoryAndItems/BP_GOTAShield.BP_GOTAShield_C" 0)) 0 0))
      (return _returnvalue_8))
    (:NewEnumerator1
      (bind _returnvalue_9 (Game|SpawnActorfromClass "/Game/GOTA2/Blueprints/Characters/BP_GOTANumeriusOriginaInUsel.BP_GOTANumeriusOriginaInUsel_C" _returnvalue_7 "AdjustIfPossibleButAlwaysSpawn" 0 100 100 (Utilities|Array|MakeArray "/Game/GOTA2/Blueprints/InventoryAndItems/BP_GOTAFalx.BP_GOTAFalx_C") 0 0))
      (return _returnvalue_9))
    (:NewEnumerator2
      (bind _returnvalue_10 (Game|SpawnActorfromClass "/Game/GOTA2/Blueprints/Characters/BP_GOTANumeriusOriginaInUsel.BP_GOTANumeriusOriginaInUsel_C" _returnvalue_7 "AdjustIfPossibleButAlwaysSpawn" 0 100 100 (Utilities|Array|MakeArray "/Game/GOTA2/Blueprints/InventoryAndItems/BP_GOTABowItem.BP_GOTABowItem_C" "/Game/GOTA2/Blueprints/InventoryAndItems/BP_GOTAArrowItem.BP_GOTAArrowItem_C" "/Game/GOTA2/Blueprints/InventoryAndItems/BP_GOTAArrowItem.BP_GOTAArrowItem_C" "/Game/GOTA2/Blueprints/InventoryAndItems/BP_GOTAArrowItem.BP_GOTAArrowItem_C" "/Game/GOTA2/Blueprints/InventoryAndItems/BP_GOTAArrowItem.BP_GOTAArrowItem_C" "/Game/GOTA2/Blueprints/InventoryAndItems/BP_GOTAArrowItem.BP_GOTAArrowItem_C" "/Game/GOTA2/Blueprints/InventoryAndItems/BP_GOTAArrowItem.BP_GOTAArrowItem_C" "/Game/GOTA2/Blueprints/InventoryAndItems/BP_GOTAArrowItem.BP_GOTAArrowItem_C" "/Game/GOTA2/Blueprints/InventoryAndItems/BP_GOTAArrowItem.BP_GOTAArrowItem_C" "/Game/GOTA2/Blueprints/InventoryAndItems/BP_GOTAArrowItem.BP_GOTAArrowItem_C") 0 0))
      (return _returnvalue_10))
    (:NewEnumerator3
      (bind _returnvalue_11 (Game|SpawnActorfromClass "/Game/GOTA2/Blueprints/Characters/BP_GOTANumeriusOriginaInUsel.BP_GOTANumeriusOriginaInUsel_C" _returnvalue_7 "AdjustIfPossibleButAlwaysSpawn" 0 100 100 (Utilities|Array|MakeArray "/Game/GOTA2/Blueprints/InventoryAndItems/BP_GOTASpearItem.BP_GOTASpearItem_C" (select (Math|Random|RandomBool) "/Game/GOTA2/Blueprints/InventoryAndItems/BP_GOTAShield.BP_GOTAShield_C" 0)) 0 0))
      (return _returnvalue_11))))

(fn SpawnGladiatorCustomandReturnIt
  (params (GladDiff :type EN_MatchDifficulty%20Enum :default "NewEnumerator0") (GladClass :type EN_GladiatorType%20Enum :default "NewEnumerator0") (GladiatorTeam :type Integer))
  (bind _returnvalue (Math|Random|RandomFloatinRange -1.8e+02 1.8e+02))
  (bind _self self)
  (bind _box (Variables|Default|GetBox))
  (bind _swordmanrandomitems (Variables|Default|GetSwordManRandomItems))
  (bind _spearmanrandomitems (Variables|Default|GetSpearmanRandomItems))
  (bind _archerinventories (Variables|Default|GetArcherInventories))
  (bind _twohandedinventories (Variables|Default|GetTwoHandedInventories))
  (bind _returnvalue_2 (Transformation|GetActorLocation _self))
  (bind _returnvalue_3 (Math|Rotator|MakeRotator 0.0 0.0 _returnvalue))
  (bind _returnvalue_4 (Components|Box|GetScaledBoxExtent _box))
  (bind _returnvalue_5 (Math|Random|RandomPointinBoundingBox _returnvalue_2 _returnvalue_4))
  (bind (_x _y) (Math|Vector|BreakVector _returnvalue_5))
  (bind _returnvalue_6 (Math|Vector|MakeVector _x _y 3e+02))
  (bind _returnvalue_7 (Math|Transform|MakeTransform _returnvalue_6 _returnvalue_3))
  (bind _asbp_gotaarena_game_info (Utilities|Casting|CastToBP_GOTAArenaGameInfo (Game|GetGameMode))
    (:then
      (if (Variables|/Game/GOTA2/Blueprints/GameInfos/BP_GOTAArenaGameInfo.BP_GOTAArenaGameInfo_C|GetbOverrideSpawnModeAllSameType _asbp_gotaarena_game_info)
        (LocalVariables|SetRandomGladiator (Variables|/Game/GOTA2/Blueprints/GameInfos/BP_GOTAArenaGameInfo.BP_GOTAArenaGameInfo_C|GetOverrideSameTypeType _asbp_gotaarena_game_info))
        (else
          (LocalVariables|SetRandomGladiator (Utilities|Enum|ByteToEnumEN_GladiatorType (Math|Conversions|ToByte(Integer) (Math|Random|RandomInteger 4))) :!label _label))))
    (:CastFailed
      (goto _label)))
  (switch Utilities|FlowControl|Switch|SwitchonEN_GladiatorType GladClass
    (:NewEnumerator0
      (bind _returnvalue_8 (Game|SpawnActorfromClass "/Game/GOTA2/Blueprints/Characters/BP_GOTANumeriusOriginaInUsel.BP_GOTANumeriusOriginaInUsel_C" _returnvalue_7 "AdjustIfPossibleButAlwaysSpawn" 0 100 100 (.items (Utilities|Array|Get(acopy) _swordmanrandomitems (Math|Random|RandomIntegerinRange 0 (- (Utilities|Array|Length _swordmanrandomitems) 1)))) GladiatorTeam 0))
      ;[1 1 1] Not sure why gladiator difficulty
      (return _returnvalue_8 GladDiff))
    (:NewEnumerator1
      (bind _returnvalue_9 (Game|SpawnActorfromClass "/Game/GOTA2/Blueprints/Characters/BP_GOTANumeriusOriginaInUsel.BP_GOTANumeriusOriginaInUsel_C" _returnvalue_7 "AdjustIfPossibleButAlwaysSpawn" 0 100 100 (.items (Utilities|Array|Get(acopy) _twohandedinventories (Math|Random|RandomIntegerinRange 0 (- (Utilities|Array|Length _twohandedinventories) 1)))) GladiatorTeam 0))
      (return _returnvalue_9 GladDiff))
    (:NewEnumerator2
      (bind _returnvalue_10 (Game|SpawnActorfromClass "/Game/GOTA2/Blueprints/Characters/BP_GOTANumeriusOriginaInUsel.BP_GOTANumeriusOriginaInUsel_C" _returnvalue_7 "AdjustIfPossibleButAlwaysSpawn" 0 100 100 (.items (Utilities|Array|Get(acopy) _archerinventories (Math|Random|RandomIntegerinRange 0 (- (Utilities|Array|Length _archerinventories) 1)))) GladiatorTeam 0))
      (return _returnvalue_10 GladDiff))
    (:NewEnumerator3
      (bind _returnvalue_11 (Game|SpawnActorfromClass "/Game/GOTA2/Blueprints/Characters/BP_GOTANumeriusOriginaInUsel.BP_GOTANumeriusOriginaInUsel_C" _returnvalue_7 "AdjustIfPossibleButAlwaysSpawn" 0 100 100 (.items (Utilities|Array|Get(acopy) _spearmanrandomitems (Math|Random|RandomIntegerinRange 0 (- (Utilities|Array|Length _spearmanrandomitems) 1)))) GladiatorTeam 0))
      (return _returnvalue_11 GladDiff))
    (:NewEnumerator4
      (bind _returnvalue_12 (Game|SpawnActorfromClass "/Game/GOTA2/Blueprints/Characters/BP_GOTANumeriusOriginaInUsel.BP_GOTANumeriusOriginaInUsel_C" _returnvalue_7 "AdjustIfPossibleButAlwaysSpawn" 0 100 100 (.items (.OutItem (Utilities|Array|Random (Variables|Default|GetMurmilloRandomItems)))) GladiatorTeam 0))
      (return _returnvalue_12 GladDiff))
    (:NewEnumerator5
      (bind _returnvalue_13 (Game|SpawnActorfromClass "/Game/GOTA2/Blueprints/Characters/BP_GOTANumeriusOriginaInUsel.BP_GOTANumeriusOriginaInUsel_C" _returnvalue_7 "AdjustIfPossibleButAlwaysSpawn" 0 100 100 (.items (.OutItem (Utilities|Array|Random (Variables|Default|GetHoplomachusRandomItems)))) GladiatorTeam 0))
      (return _returnvalue_13 GladDiff))
    (:NewEnumerator6
      (bind _returnvalue_14 (Game|SpawnActorfromClass "/Game/GOTA2/Blueprints/Characters/BP_GOTANumeriusOriginaInUsel.BP_GOTANumeriusOriginaInUsel_C" _returnvalue_7 "AdjustIfPossibleButAlwaysSpawn" 0 100 100 (.items (.OutItem (Utilities|Array|Random (Variables|Default|GetThracianRandomItems)))) GladiatorTeam 0))
      (return _returnvalue_14 GladDiff))
    (:NewEnumerator7
      (bind _returnvalue_15 (Game|SpawnActorfromClass "/Game/GOTA2/Blueprints/Characters/BP_GOTAGirlMaxParClass.BP_GOTAGirlMaxParClass_C" _returnvalue_7 "AdjustIfPossibleButAlwaysSpawn" 0 100 100 (.items (.OutItem (Utilities|Array|Random (Variables|Default|GetGladiatrixRandomItems)))) GladiatorTeam 0))
      (return _returnvalue_15 GladDiff))
    (:NewEnumerator8
      (bind _returnvalue_16 (Game|SpawnActorfromClass "/Game/GOTA2/Blueprints/Characters/BP_GOTANumeriusOriginaInUsel.BP_GOTANumeriusOriginaInUsel_C" _returnvalue_7 "AdjustIfPossibleButAlwaysSpawn" 0 100 100 (.items (.OutItem (Utilities|Array|Random (Variables|Default|GetSecutorRandomItems)))) GladiatorTeam 0))
      (return _returnvalue_16 GladDiff))
    (:NewEnumerator9
      (bind _returnvalue_17 (Game|SpawnActorfromClass "/Game/GOTA2/Blueprints/Characters/BP_GOTANumeriusOriginaInUsel.BP_GOTANumeriusOriginaInUsel_C" _returnvalue_7 "AdjustIfPossibleButAlwaysSpawn" 0 100 100 (.items (.OutItem (Utilities|Array|Random (Variables|Default|GetUnarmedRandomItems)))) GladiatorTeam 0))
      (return _returnvalue_17 GladDiff))
    (:NewEnumerator11
      (bind _returnvalue_18 (Game|SpawnActorfromClass "/Game/GOTA2/Blueprints/Characters/BP_GOTATigerMountable.BP_GOTATigerMountable_C" _returnvalue_7 "AdjustIfPossibleButAlwaysSpawn" 0 100 100 0 GladiatorTeam 0))
      (return _returnvalue_18 GladDiff))))