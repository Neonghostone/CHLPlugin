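; Bow-style shooting weapon that equips to the character's left hand and fires arrows from the quiver or inventory, or other items if the AllBowable option is saved.
; Holding fire loads an arrow and draws the string to build power; release shoots after minimum tension.
; HUD or AI aim goes to a replicated vector whose OnRep spawns the projectile.
; While drawing, the local player's predicted trajectory renders as spline meshes.
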(event Custom|PrepareLoadArrow
  (params (Arrows :type Array%20of%20BP%20GOTA%20Item%20Max%20Par%20Class%20I%20Object%20References))
  (bind _output (Utilities|Array|Get(acopy) Arrows))
  (Utilities|IsValid (Utilities|Array|Get(acopy) Arrows)
    (:Is%20Valid
      (bind _asbp_gotachar_max_par_class (Utilities|Casting|CastToBP_GOTACharMaxParClass (Components|GetOwner)))
      (Variables|/Game/GOTA2/Blueprints/Characters/BP_GOTACharMaxParClass.BP_GOTACharMaxParClass_C|SetReplicatedAnimState _asbp_gotachar_max_par_class "NewEnumerator12")
      (if (and (> (Utilities|Array|Length Arrows) 0) (> (Utilities|Array|Length (CallFunction|ReturnArrowsandOthersonInv)) 0))
        (Variables|Default|SetbArrowLoading (Utilities|Array|MakeArray _output))
        (Default|EquipasArrow _output self)
        (Utilities|FlowControl|Delay (Variables|Default|GetPrepareAllowTime))
        (Variables|Default|SetbArrowItemLoaded (Utilities|Array|MakeArray _output))
        (Utilities|Array|Clear (Variables|Default|GetbArrowLoading))
        (CallFunction|TenseChord)))
    (:Is%20Not%20Valid
      (Development|PrintString "FROM SHootingBOW likeERROR item is not valid" true true "(R=1.000000,G=0.000000,B=0.017776,A=1.000000)" 1e+01))))

(event Custom|ShootArrow
  (params (ArrowsItemDEPRA :type Array%20of%20BP%20GOTA%20Item%20Max%20Par%20Class%20I%20Object%20References))
  (bind _asbp_gotachar_max_par_class (Utilities|Casting|CastToBP_GOTACharMaxParClass (Components|GetOwner)))
  (switch Utilities|FlowControl|Switch|SwitchonEN_PawnState (Variables|/Game/GOTA2/Blueprints/Characters/BP_GOTACharMaxParClass.BP_GOTACharMaxParClass_C|GetPawnState _asbp_gotachar_max_par_class)
    (:NewEnumerator0
      (Variables|/Game/GOTA2/Blueprints/Characters/BP_GOTACharMaxParClass.BP_GOTACharMaxParClass_C|SetReplicatedAnimState _asbp_gotachar_max_par_class "NewEnumerator14"))
    (:NewEnumerator7
      _))
  (CallFunction|ClientGettheAimVector)
  (Default|MultiDestroyAllSplineMeshComponents _asbp_gotachar_max_par_class)
  (CallFunction|ClearAlltheSplineMeshesDestroyArrow))

(event Custom|TenseChord
  (bind _barrowitemloaded (Variables|Default|GetbArrowItemLoaded))
  (bind _output (Utilities|Array|Get(acopy) _barrowitemloaded))
  ;[1 1 1] reset it
  (Variables|Default|SetThrowPowerLatent 0.0)
  (bind _asbp_gotachar_max_par_class (Utilities|Casting|CastToBP_GOTACharMaxParClass (Components|GetOwner)))
  (Variables|/Game/GOTA2/Blueprints/Characters/BP_GOTACharMaxParClass.BP_GOTACharMaxParClass_C|SetReplicatedAnimState _asbp_gotachar_max_par_class "NewEnumerator13")
  (Utilities|IsValid _output
    (:Is%20Valid
      (CallFunction|ClientShowThrowingStuffandProgress false 0.01)
      (CallFunction|BeginAddingPowerOfThrow)
      (Utilities|FlowControl|Delay (Variables|Default|GetMinTension))
      (if (Variables|Default|GetbLeftHold)
        (Variables|Default|SetbMinLoadTime true)
        (else
          (CallFunction|ShootArrow (Utilities|Array|MakeArray _output))
          (Variables|Default|SetbMinLoadTime true))))))

(event Custom|ServerGetClientConstantDirectionVector
  (params (AimVect :type Vector))
  ;[1 1 1] When the repnotify triggers the arrow gets shot and this triggers it
  (Variables|Default|SetRepnoDirectionAimVector AimVect))

(event Custom|ClientGetTheAimVector
  (bind _returnvalue (Components|GetOwner))
  (bind _asbp_gotachar_max_par_class (Utilities|Casting|CastToBP_GOTACharMaxParClass _returnvalue))
  (bind _returnvalue_2 (Transformation|GetActorRotation _asbp_gotachar_max_par_class))
  (bind _returnvalue_3 (Pawn|GetController _asbp_gotachar_max_par_class))
  ;[1 1 1] When the repnotify triggers the arrow gets shot and this triggers it
  (bind _asplayer_controller (Utilities|Casting|CastToPlayerController _returnvalue_3)
    (:then
      (CallFunction|ServerGetClientConstantDirectionVector (Math|Vector|MakeVector (.X (Math|Vector|BreakVector (Variables|/Game/GOTA2/Blueprints/HUD/BP_GOTAHUDMaxParClass.BP_GOTAHUDMaxParClass_C|GetDirectionConstant (.AsBP%20GOTAHUDMax%20Par%20Class (Utilities|Casting|CastToBP_GOTAHUDMaxParClass (HUD|GetHUD _asplayer_controller)))))) (.Y (Math|Vector|BreakVector (Variables|/Game/GOTA2/Blueprints/HUD/BP_GOTAHUDMaxParClass.BP_GOTAHUDMaxParClass_C|GetDirectionConstant (.AsBP%20GOTAHUDMax%20Par%20Class (Utilities|Casting|CastToBP_GOTAHUDMaxParClass (HUD|GetHUD _asplayer_controller)))))) (.Z (Math|Vector|BreakVector (Variables|/Game/GOTA2/Blueprints/HUD/BP_GOTAHUDMaxParClass.BP_GOTAHUDMaxParClass_C|GetDirectionConstant (.AsBP%20GOTAHUDMax%20Par%20Class (Utilities|Casting|CastToBP_GOTAHUDMaxParClass (HUD|GetHUD _asplayer_controller)))))))))
    (:CastFailed
      (bind _asbp_gotaaicmax_par_class (Utilities|Casting|CastToBP_GOTAAICMaxParClass _returnvalue_3))
      (CallFunction|ServerGetClientConstantDirectionVector (Math|Rotator|GetRotationXVector (Math|Rotator|MakeRotator (.roll _returnvalue_2) (Variables|/Game/GOTA2/Blueprints/Controllers/BP_GOTAAICMaxParClass.BP_GOTAAICMaxParClass_C|GetAImPitch _asbp_gotaaicmax_par_class) (.yaw _returnvalue_2)))))))

(event Custom|RepnoShootArrow
  (params (ArrowGettingShotAt :type Vector))
  (bind _returnvalue (Components|GetOwner))
  (bind _barrowitemloaded (Variables|Default|GetbArrowItemLoaded))
  (bind _asbp_gotachar_max_par_class (Utilities|Casting|CastToBP_GOTACharMaxParClass _returnvalue))
  (bind _output (Utilities|Array|Get(acopy) _barrowitemloaded))
  (if (> (Utilities|Array|Length _barrowitemloaded) 0)
    (CallFunction|ClientPausetheThrowBar)
    (Default|SpawnAppearProjectileforThrow _output ArrowGettingShotAt (+ (Transformation|GetActorLocation _asbp_gotachar_max_par_class) (* (Math|Rotator|GetRotationXVector (Transformation|GetActorRotation _asbp_gotachar_max_par_class)) 1.0) "0,0,30.000000") (Variables|Default|GetThrowPowerLatent) false)
    (Utilities|FlowControl|Delay 0.0)
    (Transformation|AddLocalRotation (Variables|/Game/GOTA2/Blueprints/InventoryAndItems/BP_GOTAItemMaxParClassI.BP_GOTAItemMaxParClassI_C|GetItemStatMesh _output) (Variables|/Game/GOTA2/Blueprints/InventoryAndItems/BP_GOTAItemMaxParClassI.BP_GOTAItemMaxParClassI_C|GetOffsetWhenArrowShot _output) false false)
    (Default|HandlleGetRemovedfromInvArroworQuiver _output)
    (Default|UnequipasArrow _output)
    (bind _asbp_gotaarrow_item (Utilities|Casting|CastToBP_GOTAArrowItem _output)
      (:then
        (Default|HandleGetShoRreleased _asbp_gotaarrow_item (Components|GetOwner)))
      (:CastFailed
        _))
    (Utilities|Array|Clear (Variables|Default|GetbArrowItemLoaded))
    (Utilities|FlowControl|Delay 1.0)
    (bind _asbp_gotachar_max_par_class_2 (Utilities|Casting|CastToBP_GOTACharMaxParClass (Components|GetOwner)))
    (Variables|/Game/GOTA2/Blueprints/Characters/BP_GOTACharMaxParClass.BP_GOTACharMaxParClass_C|SetReplicatedAnimState _asbp_gotachar_max_par_class_2 "NewEnumerator0")
    (Variables|Default|SetbMinLoadTime false)
    (Utilities|FlowControl|Delay 0.5)
    (CallFunction|ClientHideandResetProgressBar)
    (Utilities|FlowControl|Delay 3.0)
    (Default|MultiDestroyAllSplineMeshComponents _asbp_gotachar_max_par_class_2)
    (CallFunction|ClearAlltheSplineMeshesDestroyArrow)))

(event EventBeginPlay
  (|CallParentFunction) ; This node is disabled and will not be called.\nDrag off pins to build functionality.
)

(event Collision|EventActorBeginOverlap
  (params (OtherActor :type Actor%20Object%20Reference))
  (|CallParentFunction OtherActor) ; This node is disabled and will not be called.\nDrag off pins to build functionality.
)

(event EventTick
  (params (DeltaSeconds :type Float%20%28single-precision%29))
  (|CallParentFunction DeltaSeconds) ; This node is disabled and will not be called.\nDrag off pins to build functionality.
)

(event EventEquip
  ;[1 1 1] Equips the bow
  (bind _asbp_gotachar_max_par_class (Utilities|Casting|CastToBP_GOTACharMaxParClass (Components|GetOwner)))
  (Default|SetPrimaryItem (Variables|/Game/GOTA2/Blueprints/Characters/BP_GOTACharMaxParClass.BP_GOTACharMaxParClass_C|GetInvReference _asbp_gotachar_max_par_class) self)
  (Class|SkinnedMeshComponent|SetSkeletalMesh (Variables|/Game/GOTA2/Blueprints/Characters/BP_GOTACharMaxParClass.BP_GOTACharMaxParClass_C|GetRightArmWeapon _asbp_gotachar_max_par_class) 0 true)
  (Variables|/Game/GOTA2/Blueprints/Characters/BP_GOTACharMaxParClass.BP_GOTACharMaxParClass_C|SetRepnoSkeletalMeshRight _asbp_gotachar_max_par_class 0)
  (Utilities|IsValid (Variables|/Game/GOTA2/Blueprints/Characters/BP_GOTACharMaxParClass.BP_GOTACharMaxParClass_C|GetInvReference _asbp_gotachar_max_par_class)
    (:Is%20Valid
      (Variables|/Game/GOTA2/Blueprints/Characters/BP_GOTACharMaxParClass.BP_GOTACharMaxParClass_C|SetRepnoSkeletalMeshLeft _asbp_gotachar_max_par_class (Variables|Default|GetSkeleMeshToEquip))
      (Variables|/Game/GOTA2/Blueprints/Characters/BP_GOTACharMaxParClass.BP_GOTACharMaxParClass_C|SetRepnoLeftScale _asbp_gotachar_max_par_class (Variables|Default|GetEquippingScale))
      (Variables|Default|SetbPicked true)
      (Variables|Default|SetbProtecting false)
      (Variables|Default|SetbMinLoadTime false)
      (Variables|Default|SetbLeftHold false)
      (Variables|Default|SetbPreparedAttack false)
      (Utilities|Array|SetArrayElem :TargetArray (Variables|Default|GetLastLocationsMulti))
      ;;[1 1 1] So the blade will work fine
      (CallFunction|ResetforEquip)
      (Transformation|DetachFromComponent (Variables|Default|GetItemStatMesh) "KeepWorld" "KeepWorld" "KeepWorld" true)
      (Variables|Default|SetbStuckOnSurface false))))

(event EventStartFire
  (params (FireModeNum :type Byte :default 0))
  (bind _arrows (CallFunction|ReturnArrowsandOthersonInv))
  (bind _barrowitemloaded (Variables|Default|GetbArrowItemLoaded))
  ;[1 1 1] Start fire and stop fire to trigger the shot
  ;;[1 1 1] Make sure it is ready to attack
  (switch int (Math|Conversions|ToInteger(Byte) FireModeNum)
    (:0
      (bind _asbp_gotachar_max_par_class (Utilities|Casting|CastToBP_GOTACharMaxParClass (Components|GetOwner)))
      (switch Utilities|FlowControl|Switch|SwitchonEN_PawnState (Variables|/Game/GOTA2/Blueprints/Characters/BP_GOTACharMaxParClass.BP_GOTACharMaxParClass_C|GetPawnState _asbp_gotachar_max_par_class)
        (:NewEnumerator0
          (switch Utilities|FlowControl|Switch|SwitchonEN_AnimState (Variables|/Game/GOTA2/Blueprints/Characters/BP_GOTACharMaxParClass.BP_GOTACharMaxParClass_C|GetReplicatedAnimState _asbp_gotachar_max_par_class)
            (:NewEnumerator0
              (if (> (Utilities|Array|Length _arrows) 0)
                (Utilities|IsValid (Utilities|Array|Get(acopy) _barrowitemloaded)
                  (:Is%20Valid
                    ;;[1 1 1] Neongho: To fix a bug
                    (Utilities|Array|Clear _barrowitemloaded))
                  (:Is%20Not%20Valid
                    _))
                (CallFunction|PrepareLoadArrow (Utilities|Array|MakeArray (Utilities|Array|Get(acopy) _arrows)))
                (Variables|Default|SetbLeftHold true)
                (else
                  (bind _asbp_gotachar_max_par_class_2 (Utilities|Casting|CastToBP_GOTACharMaxParClass (Components|GetOwner)))
                  (if (Class|Controller|IsPlayerController (Pawn|GetController _asbp_gotachar_max_par_class_2))
                    (bind _asbp_gotapcmax_par_class (Utilities|Casting|CastToBP_GOTAPCMaxParClass (Pawn|GetController _asbp_gotachar_max_par_class_2)))
                    (Default|ClientAddMessage _asbp_gotapcmax_par_class (Utilities|Array|Get(acopy) (Variables|Default|GetMultiNoMoreArrowsInQuiver)) 2.0 (Math|Color|MakeColor 0 0 255 255))))))))
        (:NewEnumerator7
          (bind _asbp_gotapcmax_par_class_2 (Utilities|Casting|CastToBP_GOTAPCMaxParClass (Pawn|GetController _asbp_gotachar_max_par_class)))
          (Default|ClientAddMessage _asbp_gotapcmax_par_class_2 (Utilities|Array|Get(acopy) (Variables|Default|GetMultiYouCantShootOnFloor) (Math|Conversions|ToInteger(Byte) (Variables|/Game/GOTA2/Blueprints/Controllers/BP_GOTAPCMaxParClass.BP_GOTAPCMaxParClass_C|GetPlayerLanguage _asbp_gotapcmax_par_class_2))) 2.0 (Math|Color|MakeColor 0 0 255 255)))))))

(event EventStopFIre
  (params (FireModeNum :type Byte :default 0))
  ;[1 1 1] Start fire and stop fire to trigger the shot
  (switch int (Math|Conversions|ToInteger(Byte) FireModeNum)
    (:0
      (Variables|Default|SetbLeftHold false)
      (bind _asbp_gotachar_max_par_class (Utilities|Casting|CastToBP_GOTACharMaxParClass (Components|GetOwner)))
      (switch Utilities|FlowControl|Switch|SwitchonEN_PawnState (Variables|/Game/GOTA2/Blueprints/Characters/BP_GOTACharMaxParClass.BP_GOTACharMaxParClass_C|GetPawnState _asbp_gotachar_max_par_class)
        (:NewEnumerator0
          (switch Utilities|FlowControl|Switch|SwitchonEN_AnimState (Variables|/Game/GOTA2/Blueprints/Characters/BP_GOTACharMaxParClass.BP_GOTACharMaxParClass_C|GetReplicatedAnimState _asbp_gotachar_max_par_class)
            (:NewEnumerator13
              (Utilities|IsValid (Utilities|Array|Get(acopy) (Variables|Default|GetbArrowItemLoaded))
                (:Is%20Valid
                  (if (Variables|Default|GetbMinLoadTime)
                    (CallFunction|ShootArrow (CallFunction|ReturnArrowsandOthersonInv))))))))))))

(event EventUnequip
  (bind _asbp_gotachar_max_par_class (Utilities|Casting|CastToBP_GOTACharMaxParClass (Components|GetOwner)))
  (Class|SkinnedMeshComponent|SetSkeletalMesh (Variables|/Game/GOTA2/Blueprints/Characters/BP_GOTACharMaxParClass.BP_GOTACharMaxParClass_C|GetLeftArmWeapon _asbp_gotachar_max_par_class) 0 true)
  (Variables|/Game/GOTA2/Blueprints/InventoryAndItems/BP_GOTAInvMaxParClassInclBag.BP_GOTAInvMaxParClassInclBag_C|SetPrimaryItem (Variables|/Game/GOTA2/Blueprints/Characters/BP_GOTACharMaxParClass.BP_GOTACharMaxParClass_C|GetInvReference _asbp_gotachar_max_par_class) 0)
  (Variables|Default|SetbPicked false))

(event EventFORBOTHRenderTrajectory
  (bind _returnvalue (Components|GetOwner))
  (bind _projectilesplinemeshpointpatharray (Variables|Default|GetProjectileSplineMeshPointPathArray))
  (Utilities|IsValid _returnvalue
    (:Is%20Valid
      (bind _asbp_gotachar_max_par_class (Utilities|Casting|CastToBP_GOTACharMaxParClass _returnvalue))
      (Utilities|IsValid (Variables|/Game/GOTA2/Blueprints/Characters/BP_GOTACharMaxParClass.BP_GOTACharMaxParClass_C|GetInvReference _asbp_gotachar_max_par_class)
        (:Is%20Valid
          (if (== (Variables|/Game/GOTA2/Blueprints/InventoryAndItems/BP_GOTAInvMaxParClassInclBag.BP_GOTAInvMaxParClassInclBag_C|GetPrimaryItem (Variables|/Game/GOTA2/Blueprints/Characters/BP_GOTACharMaxParClass.BP_GOTACharMaxParClass_C|GetInvReference _asbp_gotachar_max_par_class)) self)
            (if (Pawn|IsLocallyControlled _asbp_gotachar_max_par_class)
              (if (Variables|Default|GetbPicked)
                (bind _asbp_gotapcmax_par_class (Utilities|Casting|CastToBP_GOTAPCMaxParClass (Pawn|GetController _asbp_gotachar_max_par_class)))
                (bind _asbp_gotahudmax_par_class (Utilities|Casting|CastToBP_GOTAHUDMaxParClass (HUD|GetHUD _asbp_gotapcmax_par_class)))
                (switch Utilities|FlowControl|Switch|SwitchonEN_PawnState (Variables|/Game/GOTA2/Blueprints/Characters/BP_GOTACharMaxParClass.BP_GOTACharMaxParClass_C|GetPawnState _asbp_gotachar_max_par_class)
                  (:NewEnumerator0
                    (switch Utilities|FlowControl|Switch|SwitchonEN_AnimState (Variables|/Game/GOTA2/Blueprints/Characters/BP_GOTACharMaxParClass.BP_GOTACharMaxParClass_C|GetReplicatedAnimState _asbp_gotachar_max_par_class)
                      (:NewEnumerator6
                        _)
                      (:NewEnumerator13
                        _))
                    (bind (_outhit _outpathpositions) (Class|GameplayStatics|BlueprintPredictProjectilePathbyObjectType (+ (Transformation|GetActorLocation _asbp_gotachar_max_par_class) "0, 0,30.000000") (* (Variables|/Game/GOTA2/Blueprints/HUD/BP_GOTAHUDMaxParClass.BP_GOTAHUDMaxParClass_C|GetDirectionConstant _asbp_gotahudmax_par_class) (* (Variables|Default|GetThrowPowerLatent) (Variables|Default|GetThrowMultiplierPower) 8.0)) true 2e+01 (Utilities|Array|MakeArray "ObjectTypeQuery1" "ObjectTypeQuery3") false (Utilities|Array|MakeArray (Components|GetOwner)) "None" 0.0 15.0 5.0))
                    (CallFunction|ProcessHitandDrawObjective _outhit "0, 0, 0")
                    (Spline|ClearSplinePoints (Variables|/Game/GOTA2/Blueprints/Characters/BP_GOTACharMaxParClass.BP_GOTACharMaxParClass_C|GetTangentCalculatorSpline _asbp_gotachar_max_par_class) true)
                    (for (_array_element _array_index) _outpathpositions
                      (Spline|AddSplinePointatIndex (Variables|/Game/GOTA2/Blueprints/Characters/BP_GOTACharMaxParClass.BP_GOTACharMaxParClass_C|GetTangentCalculatorSpline _asbp_gotachar_max_par_class) _array_element _array_index "World" true))
                    (Spline|SetSplinePointType (Variables|/Game/GOTA2/Blueprints/Characters/BP_GOTACharMaxParClass.BP_GOTACharMaxParClass_C|GetTangentCalculatorSpline _asbp_gotachar_max_par_class) (Utilities|Array|LastIndex _outpathpositions) "Linear" true)
                    (if (>= (Utilities|Array|Length _projectilesplinemeshpointpatharray) (Spline|GetNumberOfSplinePoints (Variables|/Game/GOTA2/Blueprints/Characters/BP_GOTACharMaxParClass.BP_GOTACharMaxParClass_C|GetTangentCalculatorSpline _asbp_gotachar_max_par_class)))
                      (for (_array_element_2 _array_index_2) (Variables|Default|GetProjectileSplineMeshPointPathArray)
                        (if (> (Math|Vector|VectorLength (Utilities|Array|Get(acopy) _outpathpositions (+ _array_index_2 1))) 0.1)
                          (SplineMesh|SetStartandEnd _array_element_2 (Utilities|Array|Get(acopy) _outpathpositions _array_index_2) (Spline|GetTangentatSplinePoint (Variables|/Game/GOTA2/Blueprints/Characters/BP_GOTACharMaxParClass.BP_GOTACharMaxParClass_C|GetTangentCalculatorSpline _asbp_gotachar_max_par_class) _array_index_2 "World") (Utilities|Array|Get(acopy) _outpathpositions (+ _array_index_2 1)) (Spline|GetTangentatSplinePoint (Variables|/Game/GOTA2/Blueprints/Characters/BP_GOTACharMaxParClass.BP_GOTACharMaxParClass_C|GetTangentCalculatorSpline _asbp_gotachar_max_par_class) (+ _array_index_2 1) "World") true :!class /Script/Engine.SplineMeshComponent)
                          (else
                            (SplineMesh|SetStartandEnd _array_element_2 "0, 0, 0" "0, 0, 0" "0, 0, 0" "0, 0, 0" true :!class /Script/Engine.SplineMeshComponent))))
                      (else
                        (bind _index (Utilities|FlowControl|ForLoopwithBreak 0 (- (Spline|GetNumberOfSplinePoints (Variables|/Game/GOTA2/Blueprints/Characters/BP_GOTACharMaxParClass.BP_GOTACharMaxParClass_C|GetTangentCalculatorSpline _asbp_gotachar_max_par_class)) 1))
                          (:LoopBody
                            (bind _returnvalue_2 (AddComponent|AddSplineMeshComponent _asbp_gotachar_max_par_class true))
                            (SplineMesh|SetStartandEnd _returnvalue_2 (Utilities|Array|Get(acopy) _outpathpositions _index) (Spline|GetTangentatSplinePoint (Variables|/Game/GOTA2/Blueprints/Characters/BP_GOTACharMaxParClass.BP_GOTACharMaxParClass_C|GetTangentCalculatorSpline _asbp_gotachar_max_par_class) _index "World") (Utilities|Array|Get(acopy) _outpathpositions (+ _index 1)) (Spline|GetTangentatSplinePoint (Variables|/Game/GOTA2/Blueprints/Characters/BP_GOTACharMaxParClass.BP_GOTACharMaxParClass_C|GetTangentCalculatorSpline _asbp_gotachar_max_par_class) (+ _index 1) "World") true :!class /Script/Engine.SplineMeshComponent)
                            (Utilities|Array|Add _projectilesplinemeshpointpatharray _returnvalue_2)))))))))))))))

(fn ConstructionScript
  (|CallParentFunction))

(fn ReturnArrowsandOthersonInv
  (bind _returnvalue (Components|GetOwner))
  (bind _arrowsininv (LocalVariables|GetArrowsInInv))
  (bind _arrowsininv_2 (LocalVariables|GetArrowsInInv))
  (Utilities|IsValid _returnvalue
    (:Is%20Valid
      (bind _asbp_gotachar_max_par_class (Utilities|Casting|CastToBP_GOTACharMaxParClass _returnvalue))
      (Utilities|IsValid (Variables|/Game/GOTA2/Blueprints/Characters/BP_GOTACharMaxParClass.BP_GOTACharMaxParClass_C|GetInvReference _asbp_gotachar_max_par_class)
        (:Is%20Valid
          (Utilities|IsValid (Default|HasQuiver (Variables|/Game/GOTA2/Blueprints/Characters/BP_GOTACharMaxParClass.BP_GOTACharMaxParClass_C|GetInvReference _asbp_gotachar_max_par_class))
            (:Is%20Valid
              (Utilities|IsValid (.ArrowInQuiver (Default|HasArrowandReturnIt (Default|HasQuiver (Variables|/Game/GOTA2/Blueprints/Characters/BP_GOTACharMaxParClass.BP_GOTACharMaxParClass_C|GetInvReference _asbp_gotachar_max_par_class))))
                (:Is%20Valid
                  (Utilities|Array|Add _arrowsininv_2 (.ArrowInQuiver (Default|HasArrowandReturnIt (Default|HasQuiver (Variables|/Game/GOTA2/Blueprints/Characters/BP_GOTACharMaxParClass.BP_GOTACharMaxParClass_C|GetInvReference _asbp_gotachar_max_par_class)))))
                  ;[1 1 1] Just returns one arrow here not like the other one
                  (return _arrowsininv_2))
                (:Is%20Not%20Valid
                  _)))
            (:Is%20Not%20Valid
              _))
          (for _array_element (Variables|/Game/GOTA2/Blueprints/InventoryAndItems/BP_GOTAInvMaxParClassInclBag.BP_GOTAInvMaxParClassInclBag_C|GetItemsInInv (Variables|/Game/GOTA2/Blueprints/Characters/BP_GOTACharMaxParClass.BP_GOTACharMaxParClass_C|GetInvReference _asbp_gotachar_max_par_class))
            (bind _asbp_gotaarrow_item (Utilities|Casting|CastToBP_GOTAArrowItem _array_element))
            (Utilities|Array|Add _arrowsininv _asbp_gotaarrow_item))
          (for _array_element_2 (Variables|/Game/GOTA2/Blueprints/InventoryAndItems/BP_GOTAInvMaxParClassInclBag.BP_GOTAInvMaxParClassInclBag_C|GetItemsInInv (Variables|/Game/GOTA2/Blueprints/Characters/BP_GOTACharMaxParClass.BP_GOTACharMaxParClass_C|GetInvReference _asbp_gotachar_max_par_class))
            (Utilities|Casting|CastToBP_GOTAShootingWeapon _array_element_2
              (:CastFailed
                (bind _returnvalue_2 (SaveGame|LoadGamefromSlot "options"))
                (bind _asbp_gotasave_options_max_par (Utilities|Casting|CastToBP_GOTASaveOptionsMaxPar _returnvalue_2))
                (if (Variables|/Game/GOTA2/Blueprints/SaveSystem/BP_GOTASaveOptionsMaxPar.BP_GOTASaveOptionsMaxPar_C|GetbAllBowable _asbp_gotasave_options_max_par)
                  (Utilities|Array|Add _arrowsininv _array_element_2)))))
          (return _arrowsininv))))))

(fn OnRepConstantDirectionAimVector
  ;[1 1 1] Everytime this gets replicated arrow is shot
  (CallFunction|RepnoShootArrow (Variables|Default|GetRepnoDirectionAimVector)))