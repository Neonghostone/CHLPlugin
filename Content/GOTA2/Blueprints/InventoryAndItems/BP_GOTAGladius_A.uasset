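; Gladius weapon Blueprint that runs the unleash phase of its owning character's special attacks.
; UnleashSpecialAttack sets the damage type through a server call, drains random special power, then branches on the selected attack: long thrust or 1H roll variants.
; Each branch opens timed tracing windows with a cooldown timer.
; Rolls add a second window only while the matching anim state persists, and completed attacks return the owner to Idle.
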(event EventBeginPlay
  (|CallParentFunction) ; This node is disabled and will not be called.\nDrag off pins to build functionality.
)

(event Collision|EventActorBeginOverlap
  (params (OtherActor :type Actor%20Object%20Reference))
  (|CallParentFunction OtherActor) ; This node is disabled and will not be called.\nDrag off pins to build functionality.
)

(event EventTick
  (params (DeltaSeconds :type Float%20%28single-precision%29))
  (|CallParentFunction DeltaSeconds) ; This node is disabled and will not be called.\nDrag off pins to build functionality.
)

(event EventUnleashSpecialAttack
  (bind _asbp_gotachar_max_par_class (Utilities|Casting|CastToBP_GOTACharMaxParClass (Components|GetOwner)))
  (Variables|Default|SetCachedLatestSpecialAttackNum 0)
  (CallFunction|SHServerSetDamageType "NewEnumerator1")
  (Default|SubtractSpecialPower _asbp_gotachar_max_par_class (Math|Random|RandomIntegerinRange (Math|Conversions|ToInteger(Byte) (Variables|Default|GetSpecialAttackPowerThatLoosesMin)) (Math|Conversions|ToInteger(Byte) (Variables|Default|GetSpecialAttackPowerThatLoosesMax))))
  (switch Utilities|FlowControl|Switch|SwitchonEN_SpecialAttack (.nameofatttackandstate (Utilities|Array|Get(acopy) (Variables|Default|GetSpecialAttacks) (Math|Conversions|ToInteger(Byte) (Variables|/Game/GOTA2/Blueprints/Characters/BP_GOTACharMaxParClass.BP_GOTACharMaxParClass_C|GetSpecialAttackNum _asbp_gotachar_max_par_class))))
    (:NewEnumerator1
      (Variables|Default|SetbTracing true)
      (Utilities|Time|SetTimerbyFunctionName 0 "TimerBasedCooldownUnleashAttack" 0.7)
      (Variables|Default|SetTracesNum 0)
      (Variables|Default|SetMaxTraces 200)
      (Utilities|FlowControl|Delay (.timeunleashing (Utilities|Array|Get(acopy) (Variables|Default|GetSpecialAttacks) (Math|Conversions|ToInteger(Byte) (Variables|/Game/GOTA2/Blueprints/Characters/BP_GOTACharMaxParClass.BP_GOTACharMaxParClass_C|GetSpecialAttackNum _asbp_gotachar_max_par_class)))))
      (bind _asbp_gotachar_max_par_class_2 (Utilities|Casting|CastToBP_GOTACharMaxParClass (Components|GetOwner)))
      (Variables|/Game/GOTA2/Blueprints/Characters/BP_GOTACharMaxParClass.BP_GOTACharMaxParClass_C|SetReplicatedAnimState _asbp_gotachar_max_par_class_2 "NewEnumerator0")
      (Variables|Default|SetbTracing false))
    (:NewEnumerator2
      (Utilities|FlowControl|Delay 0.285714 :!label _label)
      (Variables|Default|SetTracesNum 0)
      (Variables|Default|SetMaxTraces 200)
      (Utilities|FlowControl|Sequence
        (:then_0
          (Variables|Default|SetbTracing true)
          (Utilities|Time|SetTimerbyFunctionName 0 "TimerBasedCooldownUnleashAttack" 0.7)
          (Utilities|FlowControl|Delay 0.75)
          (switch Utilities|FlowControl|Switch|SwitchonEN_AnimState (Variables|/Game/GOTA2/Blueprints/Characters/BP_GOTACharMaxParClass.BP_GOTACharMaxParClass_C|GetReplicatedAnimState _asbp_gotachar_max_par_class)
            (:NewEnumerator23
              _)
            (:NewEnumerator44
              _))
          (Variables|Default|SetTracesNum 0)
          (Variables|Default|SetbTracing true)
          (Utilities|Time|SetTimerbyFunctionName 0 "TimerBasedCooldownUnleashAttack" 0.4)
          (Utilities|FlowControl|Delay 0.4)
          (bind _asbp_gotachar_max_par_class_3 (Utilities|Casting|CastToBP_GOTACharMaxParClass (Components|GetOwner)))
          (Variables|/Game/GOTA2/Blueprints/Characters/BP_GOTACharMaxParClass.BP_GOTACharMaxParClass_C|SetReplicatedAnimState _asbp_gotachar_max_par_class_3 "NewEnumerator0")
          (Variables|Default|SetbTracing false))))
    (:NewEnumerator6
      (Utilities|FlowControl|Delay 0.285714)
      (Variables|Default|SetTracesNum 0)
      (Variables|Default|SetMaxTraces 200)
      (Utilities|FlowControl|Sequence
        (:then_0
          (Variables|Default|SetbTracing true)
          (Utilities|Time|SetTimerbyFunctionName 0 "TimerBasedCooldownUnleashAttack" 0.7)
          (Utilities|FlowControl|Delay 0.75)
          (switch Utilities|FlowControl|Switch|SwitchonEN_AnimState (Variables|/Game/GOTA2/Blueprints/Characters/BP_GOTACharMaxParClass.BP_GOTACharMaxParClass_C|GetReplicatedAnimState _asbp_gotachar_max_par_class)
            (:NewEnumerator28
              (Variables|Default|SetTracesNum 0)
              (Variables|Default|SetbTracing true)
              (Utilities|Time|SetTimerbyFunctionName 0 "TimerBasedCooldownUnleashAttack" 0.4)
              (Utilities|FlowControl|Delay 0.4)
              (bind _asbp_gotachar_max_par_class_4 (Utilities|Casting|CastToBP_GOTACharMaxParClass (Components|GetOwner)))
              (Variables|/Game/GOTA2/Blueprints/Characters/BP_GOTACharMaxParClass.BP_GOTACharMaxParClass_C|SetReplicatedAnimState _asbp_gotachar_max_par_class_4 "NewEnumerator0")
              (Variables|Default|SetbTracing false))))))
    (:NewEnumerator9
      (goto _label))))

(fn ConstructionScript
  (|CallParentFunction))