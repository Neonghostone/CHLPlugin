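; BP_GOTAFalx is a falx weapon Blueprint that implements the Falx Tornado special attack.
; Unleashing it sets the damage type, drains a random amount of special power and spends vigour on the owning character.
; Timed delays then restart weapon tracing for up to five spin hits, each gated on the replicated tornado anim state and followed by a cooldown timer.
; A parallel branch returns the character to Idle after two seconds.
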(event EventBeginPlay
  (|CallParentFunction) ; This node is disabled and will not be called.\nDrag off pins to build functionality.
)

(event Collision|EventActorBeginOverlap
  (params (OtherActor :type Actor%20Object%20Reference))
  (|CallParentFunction OtherActor) ; This node is disabled and will not be called.\nDrag off pins to build functionality.
)

(event EventTick
  (params (DeltaSeconds :type Float%20%28single-precision%29))
  (|CallParentFunction DeltaSeconds) ; This node is disabled and will not be called.\nDrag off pins to build functionality.
)

(event EventUnleashSpecialAttack
  (CallFunction|SHServerSetDamageType "NewEnumerator1")
  (bind _asbp_gotachar_max_par_class (Utilities|Casting|CastToBP_GOTACharMaxParClass (Components|GetOwner)))
  (Default|SubtractSpecialPower _asbp_gotachar_max_par_class (Math|Random|RandomIntegerinRange (Math|Conversions|ToInteger(Byte) (Variables|Default|GetSpecialAttackPowerThatLoosesMin)) (Math|Conversions|ToInteger(Byte) (Variables|Default|GetSpecialAttackPowerThatLoosesMax))))
  (Default|ServerSpendVigour _asbp_gotachar_max_par_class (.necessaryvigenergy (Utilities|Array|Get(acopy) (Variables|Default|GetSpecialAttacks) (Math|Conversions|ToInteger(Byte) (Variables|/Game/GOTA2/Blueprints/Characters/BP_GOTACharMaxParClass.BP_GOTACharMaxParClass_C|GetSpecialAttackNum _asbp_gotachar_max_par_class)))))
  (switch Utilities|FlowControl|Switch|SwitchonEN_SpecialAttack (.nameofatttackandstate (Utilities|Array|Get(acopy) (Variables|Default|GetSpecialAttacks) (Math|Conversions|ToInteger(Byte) (Variables|/Game/GOTA2/Blueprints/Characters/BP_GOTACharMaxParClass.BP_GOTACharMaxParClass_C|GetSpecialAttackNum _asbp_gotachar_max_par_class))))
    (:NewEnumerator3
      (Utilities|FlowControl|Delay 0.285714)
      (Variables|Default|SetTracesNum 0)
      (Utilities|FlowControl|Sequence
        (:then_0
          ;[1 1 1] Fist trace, and stop the whole anim
          ;;[1 1 1] Tracing causes a bug
          (Variables|Default|SetbTracing true)
          (Utilities|Time|SetTimerbyFunctionName 0 "TimerBasedCooldownUnleashAttack" 0.314286)
          (Utilities|FlowControl|Delay 2.0)
          (bind _asbp_gotachar_max_par_class_2 (Utilities|Casting|CastToBP_GOTACharMaxParClass (Components|GetOwner)))
          ;;[1 1 1] This does not cause bug
          (Variables|/Game/GOTA2/Blueprints/Characters/BP_GOTACharMaxParClass.BP_GOTACharMaxParClass_C|SetReplicatedAnimState _asbp_gotachar_max_par_class_2 "NewEnumerator0")
          (Variables|Default|SetbTracing false))
        (:then_1
          (bind _asbp_gotachar_max_par_class_3 (Utilities|Casting|CastToBP_GOTACharMaxParClass (Components|GetOwner)))
          (switch Utilities|FlowControl|Switch|SwitchonEN_AnimState (Variables|/Game/GOTA2/Blueprints/Characters/BP_GOTACharMaxParClass.BP_GOTACharMaxParClass_C|GetReplicatedAnimState _asbp_gotachar_max_par_class_3)
            (:NewEnumerator22
              ;[1 1 1] Seconadry trace
              (Utilities|FlowControl|Delay 0.485714)
              (Variables|Default|SetTracesNum 0)
              (Variables|Default|SetbTracing true)
              (Utilities|Time|SetTimerbyFunctionName 0 "TimerBasedCooldownUnleashAttack" 0.314286)
              (switch Utilities|FlowControl|Switch|SwitchonEN_AnimState (Variables|/Game/GOTA2/Blueprints/Characters/BP_GOTACharMaxParClass.BP_GOTACharMaxParClass_C|GetReplicatedAnimState _asbp_gotachar_max_par_class_3)
                (:NewEnumerator22
                  ;[1 1 1] Third  trace
                  (Utilities|FlowControl|Delay 0.371429)
                  (Variables|Default|SetTracesNum 0)
                  (Variables|Default|SetbTracing true)
                  (Utilities|Time|SetTimerbyFunctionName 0 "TimerBasedCooldownUnleashAttack" 0.314286)
                  (switch Utilities|FlowControl|Switch|SwitchonEN_AnimState (Variables|/Game/GOTA2/Blueprints/Characters/BP_GOTACharMaxParClass.BP_GOTACharMaxParClass_C|GetReplicatedAnimState _asbp_gotachar_max_par_class_3)
                    (:NewEnumerator22
                      ;[1 1 1] Forth trace
                      (Utilities|FlowControl|Delay 0.371429)
                      (Variables|Default|SetTracesNum 0)
                      (Variables|Default|SetbTracing true)
                      (Utilities|Time|SetTimerbyFunctionName 0 "TimerBasedCooldownUnleashAttack" 0.314286)
                      (switch Utilities|FlowControl|Switch|SwitchonEN_AnimState (Variables|/Game/GOTA2/Blueprints/Characters/BP_GOTACharMaxParClass.BP_GOTACharMaxParClass_C|GetReplicatedAnimState _asbp_gotachar_max_par_class_3)
                        (:NewEnumerator22
                          ;[1 1 1] Fifth trace
                          (Utilities|FlowControl|Delay 0.371429)
                          (Variables|Default|SetTracesNum 0)
                          (Variables|Default|SetbTracing true)
                          (Utilities|Time|SetTimerbyFunctionName 0 "TimerBasedCooldownUnleashAttack" 0.314286))))))))))))))

(fn ConstructionScript
  (|CallParentFunction))