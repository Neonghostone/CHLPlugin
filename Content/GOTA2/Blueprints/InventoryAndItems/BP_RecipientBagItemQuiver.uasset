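; Quiver item that a character wears on the QuiverSocket and that holds items such as arrows.
; Equip disables physics, attaches the mesh and registers it as the inventory's QuiverOrBag; Unequip clears that reference and makes it pickable.
; The AttachedToOwner RepNotify handles attaching and detaching the mesh.
; Added items are de-duplicated, reset and detached; a lookup returns an arrow and its index, while the spear lookup is an empty stub.
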(event Custom|AddItemInQuiverOrBag
  (params (NewItem :type BP%20GOTA%20Item%20Max%20Par%20Class%20I%20Object%20Reference))
  (bind _itemsinquiverbag (Variables|Default|GetItemsInQuiverBag))
  ;[1 1 1] Avoid adding twice
  (if (== (Utilities|Array|FindItem _itemsinquiverbag NewItem) -1)
    (Utilities|Array|Add _itemsinquiverbag NewItem)
    (Variables|/Game/GOTA2/Blueprints/InventoryAndItems/BP_GOTAItemMaxParClassI.BP_GOTAItemMaxParClassI_C|SetbPicked NewItem true)
    (Default|ResetforEquip NewItem)
    (Variables|/Game/GOTA2/Blueprints/InventoryAndItems/BP_GOTAItemMaxParClassI.BP_GOTAItemMaxParClassI_C|SetbProtecting NewItem false)
    (Variables|/Game/GOTA2/Blueprints/InventoryAndItems/BP_GOTAItemMaxParClassI.BP_GOTAItemMaxParClassI_C|SetbMinLoadTime NewItem false)
    (Variables|/Game/GOTA2/Blueprints/InventoryAndItems/BP_GOTAItemMaxParClassI.BP_GOTAItemMaxParClassI_C|SetbLeftHold NewItem false)
    (Variables|/Game/GOTA2/Blueprints/InventoryAndItems/BP_GOTAItemMaxParClassI.BP_GOTAItemMaxParClassI_C|SetbPreparedAttack NewItem false)
    (Utilities|Array|SetArrayElem :TargetArray (Variables|/Game/GOTA2/Blueprints/InventoryAndItems/BP_GOTAItemMaxParClassI.BP_GOTAItemMaxParClassI_C|GetLastLocationsMulti NewItem))
    (Transformation|DetachFromComponent (Variables|/Game/GOTA2/Blueprints/InventoryAndItems/BP_GOTAItemMaxParClassI.BP_GOTAItemMaxParClassI_C|GetItemStatMesh NewItem) "KeepWorld" "KeepWorld" "KeepWorld" true)
    (Variables|/Game/GOTA2/Blueprints/InventoryAndItems/BP_GOTAItemMaxParClassI.BP_GOTAItemMaxParClassI_C|SetbStuckOnSurface NewItem false)))

(event Custom|RemoveItemFromBagOrQuiver
  (params (ItemRemoving :type BP%20GOTA%20Item%20Max%20Par%20Class%20I%20Object%20Reference))
  ;[1 1 1] For when we have to remove it from the quiver
  ;;[1 1 1] Becareful redundancy heer
  (Utilities|Array|RemoveItem (Variables|Default|GetItemsInQuiverBag) ItemRemoving))

(event EventBeginPlay
  (|CallParentFunction))

(event Collision|EventActorBeginOverlap
  (params (OtherActor :type Actor%20Object%20Reference))
  (|CallParentFunction OtherActor) ; This node is disabled and will not be called.\nDrag off pins to build functionality.
)

(event EventTick
  (params (DeltaSeconds :type Float%20%28single-precision%29)))

(event EventEquip
  (bind _asbp_gotachar_max_par_class (Utilities|Casting|CastToBP_GOTACharMaxParClass (Components|GetOwner)))
  (Game|Components|ProjectileMovement|StopSimulating (Variables|Default|GetItemProjectileModePhysics) (Collision|MakeHitResult false false 0.0 0.0 "0, 0, 0" "0, 0, 0" "0,0,1" "0,0,1" 0 0))
  (Physics|SetSimulatePhysics (Variables|Default|GetItemStatMesh) false)
  (Transformation|AttachComponentToComponent (Variables|Default|GetItemStatMesh) (Variables|/Script/Engine.Character|GetMesh _asbp_gotachar_max_par_class) "QuiverSocket" "SnapToTarget" "SnapToTarget" "KeepRelative" true)
  (Collision|SetCollisionEnabled (Variables|Default|GetItemStatMesh) "NoCollision")
  (Variables|Default|SetbPickable false)
  (Variables|/Game/GOTA2/Blueprints/InventoryAndItems/BP_GOTAInvMaxParClassInclBag.BP_GOTAInvMaxParClassInclBag_C|SetQuiverOrBag (Variables|/Game/GOTA2/Blueprints/Characters/BP_GOTACharMaxParClass.BP_GOTACharMaxParClass_C|GetInvReference _asbp_gotachar_max_par_class) self)
  (Variables|Default|SetbPicked true)
  (Variables|Default|SetbAttachedToOwner true)
  (Actor|SetOwner (Variables|Default|GetItemsInQuiverBag) _asbp_gotachar_max_par_class))

(event EventUnequip
  (Variables|Default|SetbAttachedToOwner false)
  (Variables|Default|SetbPickable true)
  (bind _asbp_gotachar_max_par_class (Utilities|Casting|CastToBP_GOTACharMaxParClass (Components|GetOwner)))
  (Variables|/Game/GOTA2/Blueprints/InventoryAndItems/BP_GOTAInvMaxParClassInclBag.BP_GOTAInvMaxParClassInclBag_C|SetQuiverOrBag (Variables|/Game/GOTA2/Blueprints/Characters/BP_GOTACharMaxParClass.BP_GOTACharMaxParClass_C|GetInvReference _asbp_gotachar_max_par_class) 0))

(fn ConstructionScript
  (|CallParentFunction))

(fn OnRepBAttachedtoOwner
  (bind _itemstatmesh (Variables|Default|GetItemStatMesh))
  (if (Variables|Default|GetbAttachedToOwner)
    (bind _asbp_gotachar_max_par_class (Utilities|Casting|CastToBP_GOTACharMaxParClass (Components|GetOwner)))
    (Game|Components|ProjectileMovement|StopSimulating (Variables|Default|GetItemProjectileModePhysics) (Collision|MakeHitResult false false 0.0 0.0 "0, 0, 0" "0, 0, 0" "0,0,1" "0,0,1" 0 0))
    (Physics|SetSimulatePhysics _itemstatmesh false)
    (Transformation|AttachComponentToComponent (Variables|Default|GetItemStatMesh) (Variables|/Script/Engine.Character|GetMesh _asbp_gotachar_max_par_class) "QuiverSocket" "SnapToTarget" "SnapToTarget" "KeepRelative" true)
    (Rendering|SetVisibility _itemstatmesh true false)
    (else
      (Transformation|DetachFromComponent (Variables|Default|GetItemStatMesh) "KeepRelative" "KeepRelative" "KeepRelative" true))))

(fn HasArrowandReturnIt
  (for (_array_element _array_index) (Variables|Default|GetItemsInQuiverBag)
    (bind _asbp_gotaarrow_item (Utilities|Casting|CastToBP_GOTAArrowItem _array_element))
    (return _asbp_gotaarrow_item _array_index))
  (return 0 0))

(fn HasSpearandReturnItWIPFORLATER
  (return 0))